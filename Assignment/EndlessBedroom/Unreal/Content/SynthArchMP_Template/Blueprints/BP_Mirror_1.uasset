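; BP_Mirror_1 is a mirror actor that runs its scene capture only while the player is nearby.
; A box collision's begin overlap activates the SceneCaptureComponent2D when player 0's character capsule enters, and end overlap deactivates it when the capsule leaves.
; Gating the capture on proximity avoids rendering it when the player is outside the box.
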(event OnComponentEndOverlap(BoxCollision)
  (params (OverlappedComponent :type Primitive%20Component%20Object%20Reference) (OtherActor :type Actor%20Object%20Reference) (OtherComp :type Primitive%20Component%20Object%20Reference) (OtherBodyIndex :type Integer))
  (bind _returnvalue (Game|GetPlayerCharacter 0))
  (Utilities|IsValid _returnvalue
    (:Is%20Valid
      (if (and (== OtherActor _returnvalue) (== OtherComp (Variables|/Script/Engine.Character|GetCapsuleComponent _returnvalue)))
        (Components|Activation|Deactivate (Variables|Default|GetSceneCaptureComponent2D))))))

(event OnComponentBeginOverlap(BoxCollision)
  (params (OverlappedComponent :type Primitive%20Component%20Object%20Reference) (OtherActor :type Actor%20Object%20Reference) (OtherComp :type Primitive%20Component%20Object%20Reference) (OtherBodyIndex :type Integer) (bFromSweep :type Boolean) (SweepResult :type Hit%20Result%20Structure%20%28by%20ref%29))
  (bind _returnvalue (Game|GetPlayerCharacter 0))
  (Utilities|IsValid _returnvalue
    (:Is%20Valid
      (if (and (== OtherActor _returnvalue) (== OtherComp (Variables|/Script/Engine.Character|GetCapsuleComponent _returnvalue)))
        (Components|Activation|Activate (Variables|Default|GetSceneCaptureComponent2D) false)))))

(event EventBeginPlay)

(event Collision|EventActorBeginOverlap
  (params (OtherActor :type Actor%20Object%20Reference)))

(event EventTick
  (params (DeltaSeconds :type Float%20%28single-precision%29)))

(fn ConstructionScript)
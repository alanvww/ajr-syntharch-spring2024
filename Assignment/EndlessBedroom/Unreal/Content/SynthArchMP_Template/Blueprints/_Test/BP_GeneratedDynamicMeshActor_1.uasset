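; Test generated dynamic mesh actor that builds a beveled box from configurable dimensions, origin and bevel distance using Geometry Script.
; Rebuilding appends the box, bevels its polygroup edges and scales UVs, optionally multiplied by the largest dimension for world-scale tiling.
; The construction script applies the material.
; An event for saving the mesh as a static mesh asset is noted as broken by a Call in Editor bug.
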(event Custom|CreateNewStaticMesh
  ;[1 0.124 0.1638] This doesn't work because of a bug with "Call in Editor"
  (bind _uniqueassetpathandname (Class|GeometryScriptLibraryCreateNewAssetFunctions|CreateUniqueNewAssetPathName :BaseAssetName (Variables|Default|GetBase%20Asset%20Name) :Debug 0)
    (:Success
      (GeometryScript|AssetManagement|CreateNewStaticMeshAssetfromMesh :FromDynamicMesh (Variables|Default|GetTarget%20Mesh) :AssetPathAndName _uniqueassetpathandname :Debug 0))))

(event EventBeginPlay)

(event Collision|EventActorBeginOverlap
  (params (OtherActor :type Actor%20Object%20Reference)))

(event EventTick
  (params (DeltaSeconds :type Float%20%28single-precision%29)))

(event Events|EventOnRebuildGeneratedMesh
  (params (TargetMesh :type Dynamic%20Mesh%20Object%20Reference))
  (bind _dimension_x (Variables|Default|GetDimension%20X))
  (bind _dimension_y (Variables|Default|GetDimension%20Y))
  (bind _dimension_z (Variables|Default|GetDimension%20Z))
  (bind _uv_scale (Variables|Default|GetUV_Scale))
  (bind (_x _y) (Math|Vector2D|BreakVector2D _uv_scale))
  (bind _returnvalue (>= _dimension_x _dimension_y))
  (bind _returnvalue_2 (Math|Float|SelectFloat _dimension_x _dimension_y _returnvalue))
  (bind _returnvalue_3 (>= _returnvalue_2 _dimension_z))
  (bind _returnvalue_4 (Math|Float|SelectFloat _returnvalue_2 _dimension_z _returnvalue_3))
  (bind _returnvalue_5 (/ _returnvalue_4 1e+02))
  (bind _output_get (Variables|Default|SetTarget%20Mesh TargetMesh))
  (bind _returnvalue_6 (Class|GeometryScriptLibraryMeshPrimitiveFunctions|AppendBox :TargetMesh _output_get :PrimitiveOptions (Utilities|Struct|MakeGeometryScriptPrimitiveOptions "PerFace") :DimensionX _dimension_x :DimensionY _dimension_y :DimensionZ _dimension_z :Origin (Variables|Default|GetOrigin) :Debug 0))
  (bind _returnvalue_7 (Class|GeometryScriptLibraryMeshModelingFunctions|ApplyMeshPolygroupBevel _returnvalue_6 (Utilities|Struct|MakeGeometryScriptMeshBevelOptions (Variables|Default|GetBevel%20Distance) false) 0))
  (GeometryScript|UVs|ScaleMeshUVs :TargetMesh _returnvalue_7 :Scale (select (Variables|Default|GetForceWoldScaleUVs?) (Math|Vector2D|MakeVector2D (* _x _returnvalue_5) (* _y _returnvalue_5)) _uv_scale) :Debug 0)
  (DynamicMeshActor|ReleaseAllComputeMeshes))

(fn ConstructionScript
  (Rendering|Material|SetMaterial (Variables|DynamicMeshActor|GetDynamicMeshComponent) 0 (Variables|Default|GetMaterial)))
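; Trigger volume that toggles a World Partition data layer as the player enters or leaves.
; Box collision overlap events check for player 0's capsule, then set the InDataLayer runtime state to Activated on enter and Unloaded on exit, non-recursively, via the DataLayerSubsystem.
; Both events print debug strings, and a runtime state check is left unconnected.
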(event OnComponentBeginOverlap(BoxCollision)
  (params (OverlappedComponent :type Primitive%20Component%20Object%20Reference) (OtherActor :type Actor%20Object%20Reference) (OtherComp :type Primitive%20Component%20Object%20Reference) (OtherBodyIndex :type Integer) (bFromSweep :type Boolean) (SweepResult :type Hit%20Result%20Structure%20%28by%20ref%29))
  (if (== OtherComp (Variables|/Script/Engine.Character|GetCapsuleComponent (Game|GetPlayerCharacter 0)))
    (DataLayers|SetDataLayerRuntimeState (WorldSubsystems|GetDataLayerSubsystem) (Variables|Default|GetIn%20Data%20Layer) "Activated" false :!class /Script/Engine.DataLayerSubsystem)
    (Development|PrintString "Begin")))

(event OnComponentEndOverlap(BoxCollision)
  (params (OverlappedComponent :type Primitive%20Component%20Object%20Reference) (OtherActor :type Actor%20Object%20Reference) (OtherComp :type Primitive%20Component%20Object%20Reference) (OtherBodyIndex :type Integer))
  (if (== (Variables|/Script/Engine.Character|GetCapsuleComponent (Game|GetPlayerCharacter 0)) OtherComp)
    (DataLayers|SetDataLayerRuntimeState (WorldSubsystems|GetDataLayerSubsystem) (Variables|Default|GetIn%20Data%20Layer) "Unloaded" false :!class /Script/Engine.DataLayerSubsystem)
    (Development|PrintString "End")))

(event EventBeginPlay)

(event Collision|EventActorBeginOverlap
  (params (OtherActor :type Actor%20Object%20Reference)))

(event EventTick
  (params (DeltaSeconds :type Float%20%28single-precision%29)))

(fn ConstructionScript)
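; Portable multiplayer media screen that shows movies and downloaded images from players' media lists, with a console readout.
; BP_MediaButton presses from the owning player drive track and player selection, playback, seeking, volume and screen scale.
; Most actions pass through Server-to-Multicast event pairs, swapping movie and image dynamic materials on the screen mesh.
; The server rebroadcasts playback time and state through a delayed Tick, and initialization seeks movies to that time.
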(event Custom|PlayMedia_URL
  (bind _mediaplayer (Variables|Default|GetMediaPlayer))
  ;[0.5574 0.8041 1] Playback
  ;;[1 1 1] Play
  (switch Utilities|FlowControl|Switch|SwitchonENUM_MediaState (Variables|Default|GetMediaState)
    (:NewEnumerator5
      (Media|MediaPlayer|Play _mediaplayer :!class /Script/MediaAssets.MediaPlayer)
      (Variables|Default|SetMediaState "NewEnumerator0"))
    (:NewEnumerator1
      (bind _returnvalue (Class|MediaPlayer|OpenUrl _mediaplayer (.url (Variables|Default|GetCurrentMediaInfo)) :!label _label))
      (if _returnvalue
        (Variables|Default|SetMediaState "NewEnumerator0")
        (else
          (CallFunction|OnMediaOpenedFailed))))
    (:NewEnumerator3
      (goto _label))))

(event Custom|DisplayImage
  (params (URL :type String))
  (bind _screenimagedmi (Variables|Default|GetScreenImageDMI))
  (bind _screenimagedmi_2 (Variables|Default|GetScreenImageDMI))
  ;[0.5574 0.8041 1] Playback
  ;;[1 1 1] Display Image
  (bind _texture (|DownloadImage (.url (Variables|Default|GetCurrentMediaInfo)))
    (:then
      (Rendering|Material|SetMaterial (Variables|Default|GetScreenMesh) 0 "/Game/SynthArchMP_Template/Materials/MI_StreamingIcon_1.MI_StreamingIcon_1"))
    (:OnSuccess
      (Rendering|Material|SetTextureParameterValue _screenimagedmi_2 "Base Texture" _texture)
      (Rendering|Material|SetMaterial (Variables|Default|GetScreenMesh) 0 _screenimagedmi_2))
    (:OnFail
      (Rendering|Material|SetTextureParameterValue _screenimagedmi "Base Texture" "/Game/SynthArchMP_Template/Textures/NoMediaIcon_1.NoMediaIcon_1")
      (Rendering|Material|SetMaterial (Variables|Default|GetScreenMesh) 0 _screenimagedmi))))

(event Custom|Server_PauseMedia
  (params (MediaState :type ENUM_MediaState%20Enum :default "NewEnumerator0"))
  ;[0.5574 0.8041 1] Playback
  ;;[1 1 1] Pause
  (CallFunction|MulticastPauseMedia MediaState))

(event Custom|Multicast_PauseMedia
  (params (MediaState :type ENUM_MediaState%20Enum :default "NewEnumerator0"))
  ;[0.5574 0.8041 1] Playback
  ;;[1 1 1] Pause
  (Variables|Default|SetMediaState MediaState)
  (Sequencer|Player|Pause (Variables|Default|GetMediaPlayer))
  (Variables|Default|SetMediaState "NewEnumerator5"))

(event Custom|Multicast_RestartMedia
  (params (MediaState :type ENUM_MediaState%20Enum :default "NewEnumerator0"))
  ;[0.5574 0.8041 1] Playback
  ;;[1 1 1] Restart
  (Variables|Default|SetMediaState MediaState)
  (Class|MediaPlayer|OpenUrl (Variables|Default|GetMediaPlayer) (Variables|Default|GetMediaURL))
  (Variables|Default|SetMediaState "NewEnumerator0"))

(event Custom|Server_RestartMedia
  (params (MediaState :type ENUM_MediaState%20Enum :default "NewEnumerator0"))
  ;[0.5574 0.8041 1] Playback
  ;;[1 1 1] Restart
  (CallFunction|MulticastRestartMedia MediaState))

(event Custom|Server_StopMedia
  (params (Selection :type ENUM_MediaFormat%20Enum :default "NewEnumerator0"))
  ;[0.5574 0.8041 1] Playback
  ;;[1 1 1] Stop
  (CallFunction|MulticastStopMedia Selection))

(event Custom|Multicast_StopMedia
  (params (Selection :type ENUM_MediaFormat%20Enum :default "NewEnumerator0"))
  ;[0.5574 0.8041 1] Playback
  ;;[1 1 1] Stop
  (switch Utilities|FlowControl|Switch|SwitchonENUM_MediaFormat Selection
    (:NewEnumerator0
      (Rendering|Material|SetMaterial (Variables|Default|GetScreenMesh) 0 (Variables|Default|GetScreenMovieDMI))
      (Media|MediaPlayer|OpenSource (Variables|Default|GetMediaPlayer) "/Game/SynthArchMP_Template/Media/FMS_BlankMovie_PlayIcon.FMS_BlankMovie_PlayIcon")
      (Variables|Default|SetMediaState "NewEnumerator1"))))

(event Custom|Server_SeekMedia
  (params (SeekNext? :type Boolean))
  ;[0.5574 0.8041 1] Playback
  ;;[1 1 1] Seek
  (if (Utilities|Enum|Equal(Enum) (Variables|Default|GetMediaState) "NewEnumerator0")
    (CallFunction|MulticastSeekMedia SeekNext?)))

(event Custom|Multicast_SeekMedia
  (params (SeekNext? :type Boolean))
  (bind _servermediatime (Variables|Default|GetServerMediaTime))
  (bind _seekspanseconds (Variables|Default|GetSeekSpanSeconds))
  (bind (_days _hours _minutes _seconds _milliseconds) (Math|Timespan|BreakTimespan _servermediatime))
  ;[0.5574 0.8041 1] Playback
  ;;[1 1 1] Seek
  (Media|MediaPlayer|Seek (Variables|Default|GetMediaPlayer) (Math|Timespan|MakeTimespan _days _hours _minutes (select SeekNext? (+ _seconds _seekspanseconds) (- _seconds _seekspanseconds)) _milliseconds)))

(event Custom|Server_ScaleScreen
  (params (Up? :type Boolean))
  (bind _output_get (Variables|Default|SetScreenScaleMultiplier (select Up? (+ (Variables|Default|GetScreenScaleMultiplier) (Variables|Default|GetScreenScaleIncrement)) (- (Variables|Default|GetScreenScaleMultiplier) (Variables|Default|GetScreenScaleIncrement)))))
  (Transformation|SetWorldScale3D (Variables|Default|GetScreen_Root) (Math|Vector|MakeVector 1.0 _output_get _output_get)))

(event Custom|OnMediaOpened_Event
  (params (OpenedUrl :type String))
  (bind _mediaplayer (Variables|Default|GetMediaPlayer))
  ;[1 1 1] BeginPlay
  ;;[1 1 1] Initialize OnMedia Event Binding
  ;;;[1 1 1] OnMediaOpen
  (Components|Timeline|SetLooping _mediaplayer (Utilities|Select :Index (Variables|Default|GetMediaState) :NewEnumerator0 (Variables|Default|GetLooping?) :NewEnumerator5 false :NewEnumerator1 true :NewEnumerator4 false :NewEnumerator3 false))
  (Media|MediaPlayer|Play _mediaplayer :!class /Script/MediaAssets.MediaPlayer))

(event Custom|Init_OnMedia_Events
  ;[1 1 1] BeginPlay
  ;;[1 1 1] Initialize OnMedia Event Binding
  (Utilities|FlowControl|Sequence
    (:then_0
      ;;;[1 1 1] OnMediaOpen
      (EventDispatchers|AssignOnMediaOpened (Variables|Default|GetMediaPlayer) (delegate Custom|OnMediaOpened_Event)))
    (:then_1
      ;;;[1 1 1] OnMediaOpen_Failed
      (Media|MediaPlayer|BindEventtoOnMediaOpenFailed (Variables|Default|GetMediaPlayer) (delegate Custom|OnMediaOpened_Failed)))
    (:then_2
      ;;;[1 1 1] OnEndReached
      (EventDispatchers|AssignOnEndReached (Variables|Default|GetMediaPlayer) (delegate Custom|OnEndReached_Event)))
    (:then_3
      ;;;[1 1 1] OnSeekCompleted
      (EventDispatchers|AssignOnSeekCompleted (Variables|Default|GetMediaPlayer) (delegate Custom|OnSeekCompleted_Event_0)))))

(event Custom|OnEndReached_Event
  ;[1 1 1] BeginPlay
  ;;[1 1 1] Initialize OnMedia Event Binding
  ;;;[1 1 1] OnEndReached
  (if (not (Utilities|Enum|Equal(Enum) (Variables|Default|GetMediaState) "NewEnumerator3"))
    (Variables|Default|SetMediaState "NewEnumerator1")))

(event Custom|Server_UpdateMediaState
  (params (MediaIndex :type Integer) (CurrentMediaInfo :type STRUCT%20Media%20Info%20Structure))
  ;[0.5574 0.8041 1] Playback
  ;;[0.2639 0.6697 1] Update Media State on the console
  (CallFunction|MulticastUpdateMediaState MediaIndex CurrentMediaInfo))

(event Custom|Multicast_UpdateMediaState
  (params (MediaIndex :type Integer) (CurrentMediaInfo :type STRUCT%20Media%20Info%20Structure))
  ;[0.5574 0.8041 1] Playback
  ;;[0.2639 0.6697 1] Update Media State on the console
  (Variables|Default|SetMediaIndex MediaIndex)
  (Variables|Default|SetCurrentMediaInfo CurrentMediaInfo)
  (Utilities|FlowControl|Sequence
    (:then_1
      (CallFunction|UpdateConsoleInfo))))

(event Custom|UpdateMediaState
  ;[0.5574 0.8041 1] Playback
  ;;[0.2639 0.6697 1] Update Media State on the console
  (Utilities|FlowControl|Sequence
    (:then_1
      (CallFunction|UpdateConsoleInfo))))

(event Custom|Multicast_SetVolume
  (params (Up? :type Boolean) (VolumeMultiplier :type Float%20%28double-precision%29))
  ;[0.5574 0.8041 1] Playback
  ;;[1 1 1] Set Volume
  (Variables|Default|SetVolumeMultiplier VolumeMultiplier)
  (if Up?
    (if (<= (+ (Variables|Default|GetVolumeMultiplier) (Variables|Default|GetVolumeMultiplierIncrement)) (Variables|Default|GetVolumeMultiplierMax))
      (Variables|Default|SetVolumeMultiplier (+ (Variables|Default|GetVolumeMultiplier) (Variables|Default|GetVolumeMultiplierIncrement)))
      (Audio|Components|Audio|SetVolumeMultiplier (Variables|Default|GetMediaSound) (Variables|Default|GetVolumeMultiplier) :!class /Script/AudioMixer.SynthComponent :!label _label)
      (bind _asbp_umg_text_box_1 (Utilities|Casting|CastToBP_UMG_TextBox_1 (Variables|/Script/Engine.ChildActorComponent|GetChildActor (Variables|Default|GetUMG_Text_VolumeAmount))))
      (Default|UpdateText _asbp_umg_text_box_1 (Utilities|Text|ToText(Float) (Variables|Default|GetVolumeMultiplier) "HalfToEven")))
    (elif (>= (- (Variables|Default|GetVolumeMultiplier) (Variables|Default|GetVolumeMultiplierIncrement)) 0.0)
      (Variables|Default|SetVolumeMultiplier (- (Variables|Default|GetVolumeMultiplier) (Variables|Default|GetVolumeMultiplierIncrement)))
      (goto _label))))

(event Custom|Server_InitMediaState
  (params (MediaIndex :type Integer) (PlayerInfo :type STRUCT%20Player%20Info%20Structure%20%28by%20ref%29))
  ;[1 1 1] BeginPlay
  ;;[1 1 1] Initialize MediaInfo when MediaScreen is spawned
  (CallFunction|MulticastInitMediaState MediaIndex PlayerInfo))

(event Custom|SelectPlayer
  (params (Next? :type Boolean))
  (bind _currentmediainfo (Variables|Default|GetCurrentMediaInfo))
  ;[0.5574 0.8041 1] Playback
  ;;[1 1 1] Select Player
  (CallFunction|ServerStopMedia (.mediaformat (Variables|Default|GetCurrentMediaInfo)))
  (CallFunction|UpdatePlayerIndex Next?)
  (CallFunction|ServerUpdateMediaState 0 (Variables|Default|GetCurrentMediaInfo))
  (switch Utilities|FlowControl|Switch|SwitchonENUM_MediaFormat (.mediaformat _currentmediainfo)
    (:NewEnumerator0
      (CallFunction|ServerStopMedia "NewEnumerator0"))
    (:NewEnumerator1
      (CallFunction|ServerDisplayImage (.url _currentmediainfo)))))

(event Custom|SelectTrack
  (params (Next? :type Boolean))
  ;[0.5574 0.8041 1] Playback
  ;;[1 1 1] Select Track
  (CallFunction|ServerStopMedia (.mediaformat (Variables|Default|GetCurrentMediaInfo)))
  (CallFunction|UpdateMediaIndex Next?)
  (CallFunction|ServerUpdateMediaState (Variables|Default|GetMediaIndex) (Variables|Default|GetCurrentMediaInfo))
  (switch Utilities|FlowControl|Switch|SwitchonENUM_MediaFormat (.mediaformat (Variables|Default|GetCurrentMediaInfo))
    (:NewEnumerator0
      (CallFunction|ServerStopMedia "NewEnumerator0"))
    (:NewEnumerator1
      (CallFunction|ServerDisplayImage))))

(event Custom|Server_DisplayImage
  (params (URL :type String))
  ;[0.5574 0.8041 1] Playback
  ;;[1 1 1] Display Image
  (CallFunction|MulticastDisplayImage))

(event Custom|OnMediaOpened_Failed
  (params (FailedUrl :type String))
  (bind _mediaplayer (Variables|Default|GetMediaPlayer))
  ;[1 1 1] BeginPlay
  ;;[1 1 1] Initialize OnMedia Event Binding
  ;;;[1 1 1] OnMediaOpen_Failed
  (Media|MediaPlayer|OpenSource _mediaplayer "/Game/SynthArchMP_Template/Media/FMS_MissingMovie_PlayIcon.FMS_MissingMovie_PlayIcon")
  (Components|Timeline|SetLooping _mediaplayer true)
  (Media|MediaPlayer|Play _mediaplayer :!class /Script/MediaAssets.MediaPlayer)
  (Variables|Default|SetMediaState "NewEnumerator3"))

(event Custom|Multicast_DisplayImage
  (params (URL :type String))
  (bind _screenimagedmi (Variables|Default|GetScreenImageDMI))
  (bind _screenimagedmi_2 (Variables|Default|GetScreenImageDMI))
  ;[0.5574 0.8041 1] Playback
  ;;[1 1 1] Display Image
  (bind _texture (|DownloadImage (.url (Variables|Default|GetCurrentMediaInfo)))
    (:then
      (Rendering|Material|SetMaterial (Variables|Default|GetScreenMesh) 0 "/Game/SynthArchMP_Template/Materials/MI_StreamingIcon_1.MI_StreamingIcon_1"))
    (:OnSuccess
      (Rendering|Material|SetTextureParameterValue _screenimagedmi_2 "Base Texture" _texture)
      (Rendering|Material|SetMaterial (Variables|Default|GetScreenMesh) 0 _screenimagedmi_2))
    (:OnFail
      (Rendering|Material|SetTextureParameterValue _screenimagedmi "Base Texture" "/Game/SynthArchMP_Template/Textures/NoMediaIcon_1.NoMediaIcon_1")
      (Rendering|Material|SetMaterial (Variables|Default|GetScreenMesh) 0 _screenimagedmi))))

(event Custom|PauseMedia
  ;[0.5574 0.8041 1] Playback
  ;;[1 1 1] Pause
)

(event Custom|InitPlayMedia_URL
  (bind _mediaplayer (Variables|Default|GetMediaPlayer))
  ;[0.5574 0.8041 1] Playback
  ;;[1 1 1] Play
  (Rendering|Material|SetMaterial (Variables|Default|GetScreenMesh) 0 (Variables|Default|GetScreenMovieDMI))
  (bind _returnvalue (Class|MediaPlayer|OpenUrl _mediaplayer (.url (Variables|Default|GetCurrentMediaInfo))))
  (if _returnvalue
    (if (Audio|Components|Audio|IsPlaying _mediaplayer) :!label _label
      (Utilities|FlowControl|Delay 1.0)
      (Media|MediaPlayer|Seek _mediaplayer (Variables|Default|GetServerMediaTime))
      (else
        (Utilities|FlowControl|Delay 0.2)
        (goto _label)))
    (else
      (CallFunction|OnMediaOpenedFailed))))

(event Custom|InitPauseMedia
  (bind _mediaplayer (Variables|Default|GetMediaPlayer))
  ;[0.5574 0.8041 1] Playback
  ;;[1 1 1] Pause
  (Rendering|Material|SetMaterial (Variables|Default|GetScreenMesh) 0 (Variables|Default|GetScreenMovieDMI))
  (bind _returnvalue (Class|MediaPlayer|OpenUrl _mediaplayer (.url (Variables|Default|GetCurrentMediaInfo))))
  (if _returnvalue
    (Utilities|FlowControl|Delay 0.2)
    (Media|MediaPlayer|Seek _mediaplayer (Variables|Default|GetServerMediaTime))
    (else
      (CallFunction|OnMediaOpenedFailed))))

(event Custom|Server_SetVolume
  (params (Up? :type Boolean))
  ;[0.5574 0.8041 1] Playback
  ;;[1 1 1] Set Volume
  (CallFunction|MulticastSetVolume Up? (Variables|Default|GetVolumeMultiplier)))

(event Custom|Multicast_InitMediaState
  (params (MediaIndex :type Integer) (STRUCT_PlayerInfo :type STRUCT%20Player%20Info%20Structure%20%28by%20ref%29))
  ;[1 1 1] BeginPlay
  ;;[1 1 1] Initialize MediaInfo when MediaScreen is spawned
  (Variables|Default|SetCurrentPlayerInfo STRUCT_PlayerInfo)
  (if (> (Utilities|Array|Length (.MediaInfoArray (Utilities|Struct|BreakSTRUCT_PlayerInfo (Variables|Default|GetCurrentPlayerInfo)))) 0)
    (Variables|Default|SetCurrentMediaInfo (Utilities|Array|Get(acopy) (.MediaInfoArray (Utilities|Struct|BreakSTRUCT_PlayerInfo (Variables|Default|GetCurrentPlayerInfo))) (.MediaInfoIndex (Utilities|Struct|BreakSTRUCT_PlayerInfo (Variables|Default|GetCurrentPlayerInfo)))))
    (Variables|Default|SetMediaIndex (.MediaInfoIndex (Utilities|Struct|BreakSTRUCT_PlayerInfo (Variables|Default|GetCurrentPlayerInfo))))
    (switch Utilities|FlowControl|Switch|SwitchonENUM_MediaFormat (.mediaformat (Variables|Default|GetCurrentMediaInfo))
      (:NewEnumerator0
        (switch Utilities|FlowControl|Switch|SwitchonENUM_MediaState (Variables|Default|GetMediaState)
          (:NewEnumerator0
            (CallFunction|InitPlayMediaURL))
          (:NewEnumerator5
            (CallFunction|InitPauseMedia))
          (:NewEnumerator1
            (CallFunction|StopMedia))))
      (:NewEnumerator1
        (CallFunction|DisplayImage)))))

(event Custom|OnSeekCompleted_Event_0
  ;[1 1 1] BeginPlay
  ;;[1 1 1] Initialize OnMedia Event Binding
  ;;;[1 1 1] OnSeekCompleted
  (switch Utilities|FlowControl|Switch|SwitchonENUM_MediaState (Variables|Default|GetMediaState)
    (:NewEnumerator5
      (Sequencer|Player|Pause (Variables|Default|GetMediaPlayer)))))

(event Custom|RefreshPlayer
  ;[0.5574 0.8041 1] Playback
  ;;[1 1 1] Refresh Player
  (CallFunction|ServerStopMedia (.mediaformat (Variables|Default|GetCurrentMediaInfo)))
  (Variables|Default|SetCurrentMediaInfo (Utilities|Array|Get(acopy) (.MediaInfoArray (Utilities|Struct|BreakSTRUCT_PlayerInfo (Utilities|Array|Get(acopy) (Variables|Default|GetPlayer%20Info%20Array) (Variables|Default|GetPlayerIndex))))))
  (CallFunction|ServerUpdateMediaState 0 (Variables|Default|GetCurrentMediaInfo))
  (switch Utilities|FlowControl|Switch|SwitchonENUM_MediaFormat (.mediaformat (Variables|Default|GetCurrentMediaInfo))
    (:NewEnumerator0
      (CallFunction|ServerStopMedia "NewEnumerator0"))
    (:NewEnumerator1
      (CallFunction|ServerDisplayImage (.url (Variables|Default|GetCurrentMediaInfo))))))

(event Custom|StopMedia
  ;[0.5574 0.8041 1] Playback
  ;;[1 1 1] Stop
  (switch Utilities|FlowControl|Switch|SwitchonENUM_MediaFormat (stale Custom|Multicast_StopMedia Selection)
    (:NewEnumerator0
      (Rendering|Material|SetMaterial (Variables|Default|GetScreenMesh) 0 (Variables|Default|GetScreenMovieDMI))
      (Media|MediaPlayer|OpenSource (Variables|Default|GetMediaPlayer) "/Game/SynthArchMP_Template/Media/FMS_BlankMovie_PlayIcon.FMS_BlankMovie_PlayIcon")
      (Variables|Default|SetMediaState "NewEnumerator1"))))

(event Custom|ShowStreamingIcon
  ;[0.5574 0.8041 1] Playback
  ;;[1 1 1] Display Image
  (Rendering|Material|SetMaterial (Variables|Default|GetScreenMesh) 0 "/Game/SynthArchMP_Template/Materials/MI_StreamingIcon_1.MI_StreamingIcon_1"))

(event Custom|Server_SyncMedia
  (params (ServerMediaTime :type Timespan%20Structure) (MediaState :type ENUM_MediaState%20Enum :default "NewEnumerator0"))
  ;[0.3051 1 0.5352] Tick
  ;;[1 1 1] Sync Media
  (CallFunction|MulticastSyncMedia ServerMediaTime MediaState))

(event Custom|Multicast_SyncMedia
  (params (ServerMediaTime :type Timespan%20Structure) (MediaState :type ENUM_MediaState%20Enum :default "NewEnumerator0"))
  ;[0.3051 1 0.5352] Tick
  ;;[1 1 1] Sync Media
  (Variables|Default|SetServerMediaTime ServerMediaTime)
  (Variables|Default|SetMediaState MediaState)
  (CallFunction|UpdateTextInfo MediaState))

(event Custom|Server_PlayMedia_URL
  (params (MediaState :type ENUM_MediaState%20Enum :default "NewEnumerator0"))
  ;[0.5574 0.8041 1] Playback
  ;;[1 1 1] Play
  (CallFunction|MulticastPlayMediaURL MediaState))

(event Custom|Multicast_PlayMedia_URL
  (params (MediaState :type ENUM_MediaState%20Enum :default "NewEnumerator0"))
  (bind _mediaplayer (Variables|Default|GetMediaPlayer))
  ;[0.5574 0.8041 1] Playback
  ;;[1 1 1] Play
  (Variables|Default|SetMediaState MediaState)
  (switch Utilities|FlowControl|Switch|SwitchonENUM_MediaState (Variables|Default|GetMediaState)
    (:NewEnumerator5
      (Media|MediaPlayer|Play _mediaplayer :!class /Script/MediaAssets.MediaPlayer)
      (Variables|Default|SetMediaState "NewEnumerator0"))
    (:NewEnumerator1
      (bind _returnvalue (Class|MediaPlayer|OpenUrl _mediaplayer (.url (Variables|Default|GetCurrentMediaInfo)) :!label _label))
      (if _returnvalue
        (Variables|Default|SetMediaState "NewEnumerator0")
        (else
          (CallFunction|OnMediaOpenedFailed))))
    (:NewEnumerator3
      (goto _label))))

(event Custom|SyncMedia
  ;[0.3051 1 0.5352] Tick
  ;;[1 1 1] Sync Media
  (Utilities|FlowControl|Delay 1.0)
  (Networking|SwitchHasAuthority
    (:Authority
      (if (Networking|IsServer)
        (bind _output_get (Variables|Default|SetServerMediaTime (Class|MediaPlayer|GetTime (Variables|Default|GetMediaPlayer))))
        (CallFunction|ServerSyncMedia _output_get (Variables|Default|GetMediaState))))))

(event EventBeginPlay
  (bind _mediasound (Variables|Default|GetMediaSound))
  ;[1 1 1] BeginPlay
  (bind _asgame_instance_synth_arch_mp (Utilities|Casting|CastToGameInstance_SynthArchMP (Game|GetGameInstance)))
  (Variables|Default|SetGameInstanceRef _asgame_instance_synth_arch_mp)
  (bind _asgame_state_synth_arch_mp (Utilities|Casting|CastToGameState_SynthArchMP (Game|GetGameState)))
  (Variables|Default|SetPlayer%20Info%20Array (Variables|/Game/SynthArchMP_Template/Blueprints/Core/GameState_SynthArchMP.GameState_SynthArchMP_C|GetPlayerInfoArray _asgame_state_synth_arch_mp))
  (Utilities|FlowControl|Sequence
    (:then_0
      (Rendering|SetVisibility (Variables|Default|GetDebugTesxt_Root) (Variables|Default|GetShowDebugText?) true)
      (Media|MediaSoundComponent|SetMediaPlayer _mediasound (Variables|Default|GetMediaPlayer))
      (Audio|Components|Audio|SetVolumeMultiplier _mediasound (Variables|Default|GetVolume%20Multiplier) :!class /Script/AudioMixer.SynthComponent)
      (CallFunction|InitonMediaEvents))
    (:then_1
      (bind _returnvalue (Rendering|Material|CreateDynamicMaterialInstance (Variables|Default|GetScreenMesh) 0 "/Game/SynthArchMP_Template/Media/MI_Media_Movie_1_1.MI_Media_Movie_1_1" "None" :!class /Script/Engine.PrimitiveComponent))
      (bind _output_get (Variables|Default|SetScreenMovieDMI _returnvalue))
      (Rendering|Material|SetTextureParameterValue _output_get "Media Texture" (Variables|Default|GetMediaTexture))
      (Media|MediaPlayer|OpenSource (Variables|Default|GetMediaPlayer) "/Game/SynthArchMP_Template/Media/FMS_BlankMovie_PlayIcon.FMS_BlankMovie_PlayIcon")
      (bind _returnvalue_2 (Rendering|Material|CreateDynamicMaterialInstance (Variables|Default|GetScreenMesh) 0 "/Game/SynthArchMP_Template/Media/MI_Media_Image_1.MI_Media_Image_1" "None" :!class /Script/Engine.PrimitiveComponent))
      (bind _output_get_2 (Variables|Default|SetScreenImageDMI _returnvalue_2))
      (Rendering|Material|SetTextureParameterValue _output_get_2 "Base Texture" "/Game/SynthArchMP_Template/Textures/NoMediaIcon_1.NoMediaIcon_1")
      (Rendering|Material|SetMaterial (Variables|Default|GetScreenMesh) 0 _output_get_2))))

(event EventPushMediaButton
  (params (%20ButtonFunction :type ENUM_MediaButtonFunction%20Enum :default "NewEnumerator15") (OtherActor%20 :type Actor%20Object%20Reference) (FunctionTag%20 :type Name :default "None"))
  (bind _mediastate (Variables|Default|GetMediaState))
  ;[0.5574 0.8041 1] Playback
  ;;[0.2639 0.6697 1] Receive input from BP_MediaButton child BPs
  ;;;[1 1 1] Check if the owning player is pushing the button and we have media to display
  (if (and (Utilities|Enum|Equal(Enum) (Utilities|GetObjectName OtherActor%20) (Utilities|GetObjectName (Variables|Actor|GetInstigator))) (> (Utilities|Array|Length (.MediaInfoArray (Utilities|Struct|BreakSTRUCT_PlayerInfo (Variables|Default|GetCurrentPlayerInfo)))) 0))
    (switch Utilities|FlowControl|Switch|SwitchonENUM_MediaButtonFunction %20ButtonFunction
      (:NewEnumerator15
        (switch name FunctionTag%20
          (:ScaleUp
            (CallFunction|ServerScaleScreen true))
          (:ScaleDown
            (CallFunction|ServerScaleScreen false))))
      (:NewEnumerator1
        (CallFunction|SelectPlayer false))
      (:NewEnumerator0
        (CallFunction|SelectPlayer true))
      (:NewEnumerator3
        (CallFunction|SelectTrack false))
      (:NewEnumerator2
        (CallFunction|SelectTrack true))
      (:NewEnumerator4
        (CallFunction|ServerPlayMediaURL _mediastate))
      (:NewEnumerator5
        (CallFunction|ServerPauseMedia _mediastate))
      (:NewEnumerator6
        (CallFunction|ServerStopMedia (.mediaformat (Variables|Default|GetCurrentMediaInfo))))
      (:NewEnumerator8
        (CallFunction|ServerSeekMedia false))
      (:NewEnumerator7
        (CallFunction|ServerSeekMedia true))
      (:NewEnumerator14
        (CallFunction|ServerRestartMedia _mediastate))
      (:NewEnumerator9
        (CallFunction|ServerSetVolume true))
      (:NewEnumerator10
        (CallFunction|ServerSetVolume false)))))

(event EventTick
  (params (DeltaSeconds :type Float%20%28single-precision%29))
  ;[0.3051 1 0.5352] Tick
  (CallFunction|SyncMedia))

(fn ConstructionScript
  (Rendering|SetVisibility (Variables|Default|GetDebugTesxt_Root) (Variables|Default|GetShowDebugText?) true))

(fn OnRepServerMediaTime)

(fn UpdateConsoleInfo
  (bind _currentplayerinfo (Variables|Default|GetCurrentPlayerInfo))
  (bind _mediainfoarray (Utilities|Struct|BreakSTRUCT_PlayerInfo _currentplayerinfo))
  (Utilities|FlowControl|Sequence
    (:then_1
      (bind _asbp_umg_text_box_1 (Utilities|Casting|CastToBP_UMG_TextBox_1 (Variables|/Script/Engine.ChildActorComponent|GetChildActor (Variables|Default|GetUMG_Text_Track))))
      (Default|UpdateText _asbp_umg_text_box_1 (Utilities|Text|ToText(String) (Utilities|String|Append "TRACK: " (Utilities|String|ToString(Integer) (+ (Variables|Default|GetMediaIndex) 1)) " / " (Utilities|String|ToString(Integer) (Utilities|Array|Length _mediainfoarray))))))
    (:then_2
      (bind _asbp_umg_text_box_1_2 (Utilities|Casting|CastToBP_UMG_TextBox_1 (Variables|/Script/Engine.ChildActorComponent|GetChildActor (Variables|Default|GetUMG_Text_Format))))
      (Default|UpdateText _asbp_umg_text_box_1_2 (Utilities|Text|ToText(String) (Utilities|String|Append "FORMAT: " (Class|KismetStringLibrary|ToUpper (Utilities|String|EnumtoString (.mediaformat (Utilities|Array|Get(acopy) _mediainfoarray (Variables|Default|GetMediaIndex)))))))))))

(fn UpdatePlayerIndex
  (params (Next? :type Boolean))
  (if Next?
    ;[1 1 1] Check the PlayerIndex and advance or loop to beginning
    (if (== (Utilities|Array|Length (Variables|Default|GetPlayer%20Info%20Array)) (+ (Variables|Default|GetPlayerIndex) 1))
      (Variables|Default|SetPlayerIndex 0)
      (else
        (Math|Integer|IncrementInt (Variables|Default|GetPlayerIndex)
          (:%20%20
            _))))
    (else
      ;[1 1 1] Check the PlayerIndex and reverse or loop to beginning
      (if (< (- (Variables|Default|GetPlayerIndex) 1) 0)
        (Variables|Default|SetPlayerIndex (- (Utilities|Array|Length (Variables|Default|GetPlayer%20Info%20Array)) 1))
        (else
          (Math|Integer|DecrementInt (Variables|Default|GetPlayerIndex)
            (:%20%20
              _))))))
  (bind _output_get (Variables|Default|SetCurrentMediaInfo (Utilities|Array|Get(acopy) (.MediaInfoArray (Utilities|Struct|BreakSTRUCT_PlayerInfo (Utilities|Array|Get(acopy) (Variables|Default|GetPlayer%20Info%20Array) (Variables|Default|GetPlayerIndex)))))))
  (return (Variables|Default|GetPlayerIndex) _output_get))

(fn UpdateMediaIndex
  (params (Next? :type Boolean))
  (bind _currentplayerinfo (Variables|Default|GetCurrentPlayerInfo))
  (bind _currentplayerinfo_2 (Variables|Default|GetCurrentPlayerInfo))
  (bind _mediainfoarray (Utilities|Struct|BreakSTRUCT_PlayerInfo _currentplayerinfo))
  (bind _mediainfoarray_2 (Utilities|Struct|BreakSTRUCT_PlayerInfo _currentplayerinfo_2))
  (bind _returnvalue (Utilities|Array|Length _mediainfoarray))
  (bind _returnvalue_2 (Utilities|Array|Length _mediainfoarray_2))
  (if Next?
    ;[1 1 1] Check the PlayerMediaIndex and advance or loop to beginning
    (if (> _returnvalue 0)
      (if (== _returnvalue (+ (Variables|Default|GetMediaIndex) 1))
        (Variables|Default|SetMediaIndex 0)
        (else
          (Math|Integer|IncrementInt (Variables|Default|GetMediaIndex)
            (:%20%20
              _))))
      (bind _output_get (Variables|Default|SetCurrentMediaInfo (Utilities|Array|Get(acopy) (.MediaInfoArray (Utilities|Struct|BreakSTRUCT_PlayerInfo (Variables|Default|GetCurrentPlayerInfo))) (Variables|Default|GetMediaIndex)) :!label _label))
      (Utilities|Struct|SetmembersinSTRUCT_PlayerInfo (Variables|/Game/SynthArchMP_Template/Blueprints/Core/GameInstance_SynthArchMP.GameInstance_SynthArchMP_C|GetPlayerInfo (Variables|Default|GetGameInstanceRef)) (Variables|Default|GetMediaIndex))
      (return (Variables|Default|GetMediaIndex) _output_get))
    (else
      ;[1 1 1] Check the PlayerMediaIndex and reverse or loop to beginning
      (if (> _returnvalue_2 0)
        (if (< (- (Variables|Default|GetMediaIndex) 1) 0)
          (Variables|Default|SetMediaIndex (- _returnvalue_2 1))
          (goto _label)
          (else
            (Math|Integer|DecrementInt (Variables|Default|GetMediaIndex)
              (:%20%20
                (goto _label)))))))))

(fn UpdateTextInfo
  (params (Enumerator :type ENUM_MediaState%20Enum :default "NewEnumerator0"))
  (bind _mediaplayer (Variables|Default|GetMediaPlayer))
  (bind _servermediatime (Variables|Default|GetServerMediaTime))
  (bind _returnvalue (Class|KismetTextLibrary|AsTimespanTimespan _servermediatime))
  (bind _returnvalue_2 (Class|MediaPlayer|GetTime _mediaplayer))
  (bind _returnvalue_3 (Class|KismetTextLibrary|AsTimespanTimespan _returnvalue_2))
  (bind _returnvalue_4 (Utilities|String|ToString(Text) _returnvalue))
  (bind _returnvalue_5 (Utilities|String|ToString(Text) _returnvalue_3))
  (bind _returnvalue_6 (Utilities|String|Append _returnvalue_4 " / " _returnvalue_5))
  (bind _returnvalue_7 (Utilities|Text|ToText(String) _returnvalue_6))
  (Utilities|FlowControl|Sequence
    (:then_0
      (bind _asbp_umg_text_box_1 (Utilities|Casting|CastToBP_UMG_TextBox_1 (Variables|/Script/Engine.ChildActorComponent|GetChildActor (Variables|Default|GetUMG_Text_MediaTime))))
      (Default|UpdateText _asbp_umg_text_box_1 _returnvalue_7))
    (:then_1
      ;[1 1 1] DebugText
      (if (Variables|Default|GetShowDebugText?)
        (Rendering|Components|TextRender|SetText (Variables|Default|GetTextRender_MediaTime) _returnvalue_7)
        (Rendering|Components|TextRender|SetText (Variables|Default|GetTextRender_MediaState) (Utilities|Text|ToText(String) (Utilities|String|Append "MediaState: " (Utilities|String|EnumtoString Enumerator))))
        (Rendering|Components|TextRender|SetText (Variables|Default|GetTextRender_URL) (Utilities|Text|ToText(String) (.url (Variables|Default|GetCurrentMediaInfo))))))))
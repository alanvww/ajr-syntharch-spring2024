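; Multiplayer media player actor that plays a video source with optional sound and keeps playback synchronized between server and clients.
; On BeginPlay it opens the source, then loops as configured and seeks to a start time, showing a placeholder movie if opening fails.
; Play requests multicast through the server and act on media state.
; A delay-throttled Tick multicasts server time, and clients seek when minutes differ or seconds drift three or more.
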(event Custom|Local_PlayMedia_URL
  (bind _mediaplayer (Variables|Default|GetMediaPlayer))
  ;[1 1 1] Play
  (switch Utilities|FlowControl|Switch|SwitchonENUM_MediaState (Variables|Default|GetMediaState)
    (:NewEnumerator5
      (Media|MediaPlayer|Play _mediaplayer :!class /Script/MediaAssets.MediaPlayer))
    (:NewEnumerator1
      (Media|MediaPlayer|OpenSource _mediaplayer (Variables|Default|GetMediaSource)))
    (:NewEnumerator3
      (Class|MediaPlayer|OpenUrl _mediaplayer (Variables|Default|GetMediaURL))))
  (Variables|Default|SetMediaState "NewEnumerator0"))

(event Custom|OnMediaOpened_Event
  (params (OpenedUrl :type String))
  (bind _mediaplayer (Variables|Default|GetMediaPlayer))
  (bind _starttime (Variables|Default|GetStartTime))
  (bind (_hours _minutes _seconds) (Utilities|Struct|BreakTimecode _starttime))
  ;[1 1 1] OnMedia Event Binding
  ;;[1 1 1] OnMediaOpen
  (Components|Timeline|SetLooping _mediaplayer (Variables|Default|GetLooping?))
  (Media|MediaPlayer|Play _mediaplayer :!class /Script/MediaAssets.MediaPlayer)
  (Media|MediaPlayer|Seek _mediaplayer (Math|Timespan|MakeTimespan 0 0 _minutes _seconds)))

(event Custom|Init_OnMedia_Events
  ;[1 1 1] OnMedia Event Binding
  (Utilities|FlowControl|Sequence
    (:then_0
      ;;[1 1 1] OnMediaOpen
      (EventDispatchers|AssignOnMediaOpened (Variables|Default|GetMediaPlayer) (delegate Custom|OnMediaOpened_Event)))
    (:then_1
      ;;[1 1 1] OnMediaOpen_Failed
      (Media|MediaPlayer|BindEventtoOnMediaOpenFailed (Variables|Default|GetMediaPlayer) (delegate Custom|OnMediaOpened_Failed)))
    (:then_2
      ;;[1 1 1] OnEndReached
      (EventDispatchers|AssignOnEndReached (Variables|Default|GetMediaPlayer) (delegate Custom|OnEndReached_Event)))))

(event Custom|OnEndReached_Event
  ;[1 1 1] OnMedia Event Binding
  ;;[1 1 1] OnEndReached
  (Variables|Default|SetMediaState "NewEnumerator1"))

(event Custom|OnMediaOpened_Failed
  (params (FailedUrl :type String))
  (bind _mediaplayer (Variables|Default|GetMediaPlayer))
  ;[1 1 1] OnMedia Event Binding
  ;;[1 1 1] OnMediaOpen_Failed
  (Media|MediaPlayer|OpenSource _mediaplayer "/Game/SynthArchMP_Template/Media/FMS_MissingMovie_PlayIcon.FMS_MissingMovie_PlayIcon")
  (Components|Timeline|SetLooping _mediaplayer true)
  (Media|MediaPlayer|Play _mediaplayer :!class /Script/MediaAssets.MediaPlayer))

(event Custom|Server_SyncMedia
  (params (ServerMediaTime :type Timespan%20Structure) (MediaState :type ENUM_MediaState%20Enum :default "NewEnumerator0"))
  ;[1 1 1] Sync Media
  (CallFunction|MulticastSyncMedia ServerMediaTime MediaState))

(event Custom|Multicast_SyncMedia
  (params (ServerMediaTime :type Timespan%20Structure) (MediaState :type ENUM_MediaState%20Enum :default "NewEnumerator0"))
  ;[1 1 1] Sync Media
  (Variables|Default|SetServerMediaTime ServerMediaTime)
  (Utilities|FlowControl|Sequence
    (:then_0
      (CallFunction|CheckClientSync))
    (:then_1
      (Rendering|Components|TextRender|SetText (Variables|Default|GetTextRender_MediaTime) (Utilities|Text|ToText(String) (Utilities|String|Append (Utilities|String|ToString(Text) (Class|KismetTextLibrary|AsTimespanTimespan (Variables|Default|GetServerMediaTime))) " / " (Utilities|String|ToString(Text) (Class|KismetTextLibrary|AsTimespanTimespan (Class|MediaPlayer|GetTime (Variables|Default|GetMediaPlayer))))))))))

(event Custom|Server_PlayMedia_URL
  (params (MediaState :type ENUM_MediaState%20Enum :default "NewEnumerator0"))
  ;[1 1 1] Play
  (CallFunction|MulticastPlayMediaURL MediaState))

(event Custom|Multicast_PlayMedia_URL
  (params (MediaState :type ENUM_MediaState%20Enum :default "NewEnumerator0"))
  (bind _mediaplayer (Variables|Default|GetMediaPlayer))
  ;[1 1 1] Play
  (Variables|Default|SetMediaState MediaState)
  (switch Utilities|FlowControl|Switch|SwitchonENUM_MediaState (Variables|Default|GetMediaState)
    (:NewEnumerator5
      (Media|MediaPlayer|Play _mediaplayer :!class /Script/MediaAssets.MediaPlayer))
    (:NewEnumerator1
      (Media|MediaPlayer|OpenSource _mediaplayer (Variables|Default|GetMediaSource)))
    (:NewEnumerator3
      (Class|MediaPlayer|OpenUrl _mediaplayer (Variables|Default|GetMediaURL))))
  (Variables|Default|SetMediaState "NewEnumerator0"))

(event Custom|SyncMedia
  ;[1 1 1] Sync Media
  (Utilities|FlowControl|Delay 1.0)
  (Networking|SwitchHasAuthority
    (:Authority
      (if (Networking|IsServer)
        (bind _output_get (Variables|Default|SetServerMediaTime (Class|MediaPlayer|GetTime (Variables|Default|GetMediaPlayer))))
        (CallFunction|ServerSyncMedia _output_get (Variables|Default|GetMediaState))))))

(event EventBeginPlay
  (bind _mediasound (Variables|Default|GetMediaSound))
  ;[1 1 1] BeginPlay
  (Utilities|FlowControl|Sequence
    (:then_0
      (if (Variables|Default|GetEnableSound?)
        (Media|MediaSoundComponent|SetMediaPlayer _mediasound (Variables|Default|GetMediaPlayer))
        (Audio|Components|Audio|SetVolumeMultiplier _mediasound (Variables|Default|GetVolume%20Multiplier) :!class /Script/AudioMixer.SynthComponent)))
    (:then_1
      (CallFunction|InitonMediaEvents)
      (Utilities|FlowControl|Delay 0.2)
      (Media|MediaPlayer|OpenSource (Variables|Default|GetMediaPlayer) (Variables|Default|GetMediaSource)))))

(event EventTick
  (params (DeltaSeconds :type Float%20%28single-precision%29))
  ;[0.3051 1 0.5352] Tick
  (CallFunction|SyncMedia))

(fn ConstructionScript)

(fn OnRepServerMediaTime)

(fn CheckClientSync
  (bind _servermediatime (Variables|Default|GetServerMediaTime))
  (bind _mediaplayer (Variables|Default|GetMediaPlayer))
  (bind _returnvalue (Class|MediaPlayer|GetTime _mediaplayer))
  (Networking|SwitchHasAuthority
    (:Remote
      (if (== (Math|Timespan|GetMinutes _servermediatime) (Math|Timespan|GetMinutes _returnvalue))
        (if (not (< (Math|Integer|Absolute(Integer) (- (Math|Timespan|GetSeconds _servermediatime) (Math|Timespan|GetSeconds _returnvalue))) 3))
          (Media|MediaPlayer|Seek (Variables|Default|GetMediaPlayer) (Variables|Default|GetServerMediaTime) :!label _label))
        (else
          (goto _label))))))
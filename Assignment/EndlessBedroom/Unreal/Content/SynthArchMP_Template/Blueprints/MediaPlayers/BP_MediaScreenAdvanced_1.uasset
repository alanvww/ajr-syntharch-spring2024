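; Networked media screen that shows each player's list of movies and images from URLs, with console text for user, track, format, time and volume.
; Media button inputs change player, track, playback, seek and volume through Server events that multicast to clients.
; GameState dispatchers refresh the player list and revised media.
; The server broadcasts playback time every second while playing, which initialization uses to seek an already running movie.
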(event Custom|PlayMedia_URL
  (bind _mediaplayer (Variables|Default|GetMediaPlayer))
  ;[0.5574 0.8041 1] Playback
  ;;[1 1 1] Play
  (switch Utilities|FlowControl|Switch|SwitchonENUM_MediaState (Variables|Default|GetMediaState)
    (:NewEnumerator5
      (Media|MediaPlayer|Play _mediaplayer :!class /Script/MediaAssets.MediaPlayer)
      (Variables|Default|SetMediaState "NewEnumerator0"))
    (:NewEnumerator1
      (bind _returnvalue (Class|MediaPlayer|OpenUrl _mediaplayer (.url (Variables|Default|GetCurrentMediaInfo)) :!label _label))
      (if _returnvalue
        (Variables|Default|SetMediaState "NewEnumerator0")
        (else
          (CallFunction|OnMediaOpenedFailed))))
    (:NewEnumerator3
      (goto _label))))

(event Custom|DisplayImage
  (bind _screenimagedmi (Variables|Default|GetScreenImageDMI))
  (bind _screenimagedmi_2 (Variables|Default|GetScreenImageDMI))
  ;[0.5574 0.8041 1] Playback
  ;;[1 1 1] Display Image
  (bind _texture (|DownloadImage (.url (Variables|Default|GetCurrentMediaInfo)))
    (:OnSuccess
      (Rendering|Material|SetTextureParameterValue _screenimagedmi "Base Texture" _texture)
      (Rendering|Material|SetMaterial (Variables|Default|GetScreenMesh) 0 _screenimagedmi))
    (:OnFail
      (Rendering|Material|SetTextureParameterValue _screenimagedmi_2 "Base Texture" "/Game/SynthArchMP_Template/Textures/NoMediaIcon_1.NoMediaIcon_1")
      (Rendering|Material|SetMaterial (Variables|Default|GetScreenMesh) 0 _screenimagedmi_2))))

(event Custom|Server_PauseMedia
  (params (MediaState :type ENUM_MediaState%20Enum :default "NewEnumerator0"))
  ;[0.5574 0.8041 1] Playback
  ;;[1 1 1] Pause
  (CallFunction|MulticastPauseMedia MediaState))

(event Custom|Multicast_PauseMedia
  (params (MediaState :type ENUM_MediaState%20Enum :default "NewEnumerator0"))
  ;[0.5574 0.8041 1] Playback
  ;;[1 1 1] Pause
  (Variables|Default|SetMediaState MediaState)
  (Sequencer|Player|Pause (Variables|Default|GetMediaPlayer))
  (Variables|Default|SetMediaState "NewEnumerator5"))

(event Custom|Multicast_RestartMedia
  (params (MediaState :type ENUM_MediaState%20Enum :default "NewEnumerator0"))
  ;[0.5574 0.8041 1] Playback
  ;;[1 1 1] Restart
  (Variables|Default|SetMediaState MediaState)
  (Class|MediaPlayer|OpenUrl (Variables|Default|GetMediaPlayer) (.url (Variables|Default|GetCurrentMediaInfo)))
  (Variables|Default|SetMediaState "NewEnumerator0"))

(event Custom|Server_RestartMedia
  (params (MediaState :type ENUM_MediaState%20Enum :default "NewEnumerator0"))
  ;[0.5574 0.8041 1] Playback
  ;;[1 1 1] Restart
  (CallFunction|MulticastRestartMedia MediaState))

(event Custom|Server_StopMedia
  (params (Selection :type ENUM_MediaFormat%20Enum :default "NewEnumerator0"))
  ;[0.5574 0.8041 1] Playback
  ;;[1 1 1] Stop
  (CallFunction|MulticastStopMedia Selection))

(event Custom|Multicast_StopMedia
  (params (Selection :type ENUM_MediaFormat%20Enum :default "NewEnumerator0"))
  (bind _screenmoviedmi (Variables|Default|GetScreenMovieDMI))
  ;[0.5574 0.8041 1] Playback
  ;;[1 1 1] Stop
  (Variables|Default|SetMediaState "NewEnumerator1")
  (switch Utilities|FlowControl|Switch|SwitchonENUM_MediaFormat Selection
    (:NewEnumerator0
      (Rendering|Material|SetTextureParameterValue _screenmoviedmi "Media Texture" (Variables|Default|GetMediaTexture))
      (Rendering|Material|SetMaterial (Variables|Default|GetScreenMesh) 0 _screenmoviedmi)
      (Media|MediaPlayer|OpenSource (Variables|Default|GetMediaPlayer) "/Game/SynthArchMP_Template/Media/FMS_BlankMovie_PlayIcon.FMS_BlankMovie_PlayIcon"))))

(event Custom|Server_SeekMedia
  (params (SeekNext? :type Boolean))
  ;[0.5574 0.8041 1] Playback
  ;;[1 1 1] Seek
  (if (Utilities|Enum|Equal(Enum) (Variables|Default|GetMediaState) "NewEnumerator0")
    (CallFunction|MulticastSeekMedia SeekNext?)))

(event Custom|Multicast_SeekMedia
  (params (SeekNext? :type Boolean))
  (bind _servermediatime (Variables|Default|GetServerMediaTime))
  (bind _seekspanseconds (Variables|Default|GetSeekSpanSeconds))
  (bind (_days _hours _minutes _seconds _milliseconds) (Math|Timespan|BreakTimespan _servermediatime))
  ;[0.5574 0.8041 1] Playback
  ;;[1 1 1] Seek
  (Media|MediaPlayer|Seek (Variables|Default|GetMediaPlayer) (Math|Timespan|MakeTimespan _days _hours _minutes (select SeekNext? (+ _seconds _seekspanseconds) (- _seconds _seekspanseconds)) _milliseconds)))

(event Custom|Server_InitMediaState
  (bind _player_info_array (Variables|Default|GetPlayer%20Info%20Array))
  ;[1 1 1] BeginPlay
  ;;[1 1 1] Initialize MediaInfo when Player is spawned
  (if (== (Utilities|Array|Length _player_info_array) 1)
    (Variables|Default|SetCurrentPlayerInfo (Utilities|Array|Get(acopy) _player_info_array))
    (Variables|Default|SetMediaIndex 0))
  (CallFunction|MulticastInitMediaState (Variables|Default|GetPlayerIndex) (Variables|Default|GetMediaIndex)))

(event Custom|Multicast_InitMediaState
  (params (PlayerIndex :type Integer) (MediaIndex :type Integer))
  ;[1 1 1] BeginPlay
  ;;[1 1 1] Initialize MediaInfo when Player is spawned
  (Utilities|FlowControl|DoOnce false
    (:Completed
      (Variables|Default|SetPlayerIndex PlayerIndex)
      (Variables|Default|SetCurrentPlayerInfo (Utilities|Array|Get(acopy) (Variables|Default|GetPlayer%20Info%20Array) (Variables|Default|GetPlayerIndex)))
      (Variables|Default|SetMediaIndex MediaIndex)
      (Variables|Default|SetCurrentMediaInfo (select (Utilities|Array|IsValidIndex (.MediaInfoArray (Utilities|Struct|BreakSTRUCT_PlayerInfo (Variables|Default|GetCurrentPlayerInfo))) (Variables|Default|GetMediaIndex)) (Utilities|Array|Get(acopy) (.MediaInfoArray (Utilities|Struct|BreakSTRUCT_PlayerInfo (Variables|Default|GetCurrentPlayerInfo))) (Variables|Default|GetMediaIndex)) (Variables|Default|GetCurrentMediaInfo)))
      (CallFunction|UpdateMediaConsoleInfo)
      (switch Utilities|FlowControl|Switch|SwitchonENUM_MediaFormat (.mediaformat (Variables|Default|GetCurrentMediaInfo))
        (:NewEnumerator0
          (switch Utilities|FlowControl|Switch|SwitchonENUM_MediaState (Variables|Default|GetMediaState)
            (:NewEnumerator0
              (CallFunction|InitPlayMediaURL))
            (:NewEnumerator5
              (CallFunction|InitPauseMedia))
            (:NewEnumerator1
              (CallFunction|StopMedia))))
        (:NewEnumerator1
          (CallFunction|DisplayImage))))))

(event Custom|OnMediaOpened_Event
  (params (OpenedUrl :type String))
  (bind _mediaplayer (Variables|Default|GetMediaPlayer))
  ;[1 1 1] BeginPlay
  ;;[1 1 1] Initialize OnMedia Event Bindings
  ;;;[1 1 1] OnMediaOpen
  (Media|MediaPlayer|Play _mediaplayer :!class /Script/MediaAssets.MediaPlayer)
  (Utilities|FlowControl|Delay 0.2)
  (Components|Timeline|SetLooping _mediaplayer (Utilities|Select :Index (Variables|Default|GetMediaState) :NewEnumerator0 (Variables|Default|GetLooping?) :NewEnumerator5 false :NewEnumerator1 true :NewEnumerator4 false :NewEnumerator3 false))
  (switch Utilities|FlowControl|Switch|SwitchonENUM_MediaState (Variables|Default|GetMediaState)
    (:NewEnumerator5
      _)
    (:NewEnumerator1
      _))
  (Sequencer|Player|Pause _mediaplayer))

(event Custom|Init_OnMedia_Events
  ;[1 1 1] BeginPlay
  ;;[1 1 1] Initialize OnMedia Event Bindings
  (Utilities|FlowControl|Sequence
    (:then_0
      ;;;[1 1 1] OnMediaOpen
      (EventDispatchers|AssignOnMediaOpened (Variables|Default|GetMediaPlayer) (delegate Custom|OnMediaOpened_Event)))
    (:then_1
      ;;;[1 1 1] OnMediaOpen_Failed
      (Media|MediaPlayer|BindEventtoOnMediaOpenFailed (Variables|Default|GetMediaPlayer) (delegate Custom|OnMediaOpened_Failed)))
    (:then_2
      ;;;[1 1 1] OnEndReached
      (EventDispatchers|AssignOnEndReached (Variables|Default|GetMediaPlayer) (delegate Custom|OnEndReached_Event)))
    (:then_3
      ;;;[1 1 1] OnSeekCompleted
      (EventDispatchers|AssignOnSeekCompleted (Variables|Default|GetMediaPlayer) (delegate Custom|OnSeekCompleted_Event_0)))))

(event Custom|OnEndReached_Event
  ;[1 1 1] BeginPlay
  ;;[1 1 1] Initialize OnMedia Event Bindings
  ;;;[1 1 1] OnEndReached
  (if (not (Utilities|Enum|Equal(Enum) (Variables|Default|GetMediaState) "NewEnumerator3"))
    (Variables|Default|SetMediaState "NewEnumerator1")))

(event Custom|Server_UpdateMediaState
  (params (PlayerIndex :type Integer) (MediaIndex :type Integer) (CurrentMediaInfo :type STRUCT%20Media%20Info%20Structure))
  ;[0.5574 0.8041 1] Playback
  ;;[0.2639 0.6697 1] Update Media State on the console
  (CallFunction|MulticastUpdateMediaState PlayerIndex MediaIndex CurrentMediaInfo))

(event Custom|Multicast_UpdateMediaState
  (params (PlayerIndex :type Integer) (MediaIndex :type Integer) (CurrentMediaInfo :type STRUCT%20Media%20Info%20Structure))
  ;[0.5574 0.8041 1] Playback
  ;;[0.2639 0.6697 1] Update Media State on the console
  (Variables|Default|SetPlayerIndex PlayerIndex)
  (Variables|Default|SetCurrentPlayerInfo (Utilities|Array|Get(acopy) (Variables|Default|GetPlayer%20Info%20Array) (Variables|Default|GetPlayerIndex)))
  (Variables|Default|SetMediaIndex MediaIndex)
  (Variables|Default|SetCurrentMediaInfo CurrentMediaInfo)
  (Utilities|FlowControl|Sequence
    (:then_0
      (CallFunction|UpdateMediaConsoleInfo))))

(event Custom|UpdateMediaState
  ;[0.5574 0.8041 1] Playback
  ;;[0.2639 0.6697 1] Update Media State on the console
  (Utilities|FlowControl|Sequence
    (:then_0
      (CallFunction|UpdateMediaConsoleInfo))))

(event Custom|Multicast_SetVolume
  (params (Up? :type Boolean) (VolumeMultiplier :type Float%20%28double-precision%29))
  ;[0.5574 0.8041 1] Playback
  ;;[1 1 1] Set Volume
  (Variables|Default|SetVolumeMultiplier VolumeMultiplier)
  (if Up?
    (if (<= (+ (Variables|Default|GetVolumeMultiplier) (Variables|Default|GetVolumeMultiplierIncrement)) (Variables|Default|GetVolumeMultiplierMax))
      (Variables|Default|SetVolumeMultiplier (+ (Variables|Default|GetVolumeMultiplier) (Variables|Default|GetVolumeMultiplierIncrement)))
      (Audio|Components|Audio|SetVolumeMultiplier (Variables|Default|GetMediaSound) (Variables|Default|GetVolumeMultiplier) :!class /Script/AudioMixer.SynthComponent :!label _label)
      (bind _asbp_umg_text_box_1 (Utilities|Casting|CastToBP_UMG_TextBox_1 (Variables|/Script/Engine.ChildActorComponent|GetChildActor (Variables|Default|GetUMG_Text_VolumeAmount))))
      (Default|UpdateText _asbp_umg_text_box_1 (Utilities|Text|ToText(Float) (Variables|Default|GetVolumeMultiplier) "HalfToEven"))
      (Rendering|Components|TextRender|SetText (Variables|Default|GetTextRender_VolumeAmount) (Utilities|Text|ToText(Float) (Variables|Default|GetVolumeMultiplier) "HalfToEven")))
    (elif (>= (- (Variables|Default|GetVolumeMultiplier) (Variables|Default|GetVolumeMultiplierIncrement)) 0.0)
      (Variables|Default|SetVolumeMultiplier (- (Variables|Default|GetVolumeMultiplier) (Variables|Default|GetVolumeMultiplierIncrement)))
      (goto _label))))

(event Custom|SelectPlayer
  (params (Next? :type Boolean))
  (bind _currentmediainfo (Variables|Default|GetCurrentMediaInfo))
  ;[0.5574 0.8041 1] Playback
  ;;[1 1 1] Select Player
  (CallFunction|ServerStopMedia (.mediaformat (Variables|Default|GetCurrentMediaInfo)))
  (CallFunction|UpdatePlayerIndex Next?)
  (CallFunction|ServerUpdateMediaState (Variables|Default|GetPlayerIndex) 0 (Variables|Default|GetCurrentMediaInfo))
  (switch Utilities|FlowControl|Switch|SwitchonENUM_MediaFormat (.mediaformat _currentmediainfo)
    (:NewEnumerator0
      (CallFunction|ServerStopMedia "NewEnumerator0"))
    (:NewEnumerator1
      (CallFunction|ServerDisplayImage (.url _currentmediainfo)))))

(event Custom|SelectTrack
  (params (Next? :type Boolean))
  ;[0.5574 0.8041 1] Playback
  ;;[1 1 1] Select Track
  (CallFunction|ServerStopMedia (.mediaformat (Variables|Default|GetCurrentMediaInfo)))
  (CallFunction|UpdateMediaIndex Next?)
  (CallFunction|ServerUpdateMediaState (Variables|Default|GetPlayerIndex) (Variables|Default|GetMediaIndex) (Variables|Default|GetCurrentMediaInfo))
  (switch Utilities|FlowControl|Switch|SwitchonENUM_MediaFormat (.mediaformat (Variables|Default|GetCurrentMediaInfo))
    (:NewEnumerator0
      (CallFunction|ServerStopMedia "NewEnumerator0"))
    (:NewEnumerator1
      (CallFunction|ServerDisplayImage))))

(event Custom|Server_DisplayImage
  (params (URL :type String))
  ;[0.5574 0.8041 1] Playback
  ;;[1 1 1] Display Image
  (CallFunction|MulticastDisplayImage))

(event Custom|OnMediaOpened_Failed
  (params (FailedUrl :type String))
  (bind _mediaplayer (Variables|Default|GetMediaPlayer))
  ;[1 1 1] BeginPlay
  ;;[1 1 1] Initialize OnMedia Event Bindings
  ;;;[1 1 1] OnMediaOpen_Failed
  (Media|MediaPlayer|OpenSource _mediaplayer "/Game/SynthArchMP_Template/Media/FMS_MissingMovie_PlayIcon.FMS_MissingMovie_PlayIcon")
  (Components|Timeline|SetLooping _mediaplayer true)
  (Media|MediaPlayer|Play _mediaplayer :!class /Script/MediaAssets.MediaPlayer)
  (Utilities|FlowControl|Delay 0.2)
  (Sequencer|Player|Pause _mediaplayer)
  (Variables|Default|SetMediaState "NewEnumerator3"))

(event Custom|Multicast_DisplayImage
  (params (URL :type String))
  (bind _screenimagedmi (Variables|Default|GetScreenImageDMI))
  (bind _screenimagedmi_2 (Variables|Default|GetScreenImageDMI))
  ;[0.5574 0.8041 1] Playback
  ;;[1 1 1] Display Image
  (bind _texture (|DownloadImage (.url (Variables|Default|GetCurrentMediaInfo)))
    (:OnSuccess
      (Rendering|Material|SetTextureParameterValue _screenimagedmi "Base Texture" _texture)
      (Rendering|Material|SetMaterial (Variables|Default|GetScreenMesh) 0 _screenimagedmi))
    (:OnFail
      (Rendering|Material|SetTextureParameterValue _screenimagedmi_2 "Base Texture" "/Game/SynthArchMP_Template/Textures/NoMediaIcon_1.NoMediaIcon_1")
      (Rendering|Material|SetMaterial (Variables|Default|GetScreenMesh) 0 _screenimagedmi_2))))

(event Custom|PauseMedia
  ;[0.5574 0.8041 1] Playback
  ;;[1 1 1] Pause
)

(event Custom|InitPlayMedia_URL
  (bind _mediaplayer (Variables|Default|GetMediaPlayer))
  ;[0.5574 0.8041 1] Playback
  ;;[1 1 1] Play
  (Rendering|Material|SetMaterial (Variables|Default|GetScreenMesh) 0 (Variables|Default|GetScreenMovieDMI))
  (bind _returnvalue (Class|MediaPlayer|OpenUrl _mediaplayer (.url (Variables|Default|GetCurrentMediaInfo))))
  (if _returnvalue
    (if (Audio|Components|Audio|IsPlaying _mediaplayer) :!label _label ; Make sure the media is playing \nbefore attempting a Seek
      (Utilities|FlowControl|Delay 1.0)
      (Media|MediaPlayer|Seek _mediaplayer (Variables|Default|GetServerMediaTime))
      (else
        (Utilities|FlowControl|Delay 0.2)
        (goto _label)))
    (else
      (CallFunction|OnMediaOpenedFailed))))

(event Custom|InitPauseMedia
  (bind _mediaplayer (Variables|Default|GetMediaPlayer))
  ;[0.5574 0.8041 1] Playback
  ;;[1 1 1] Pause
  (Rendering|Material|SetMaterial (Variables|Default|GetScreenMesh) 0 (Variables|Default|GetScreenMovieDMI))
  (bind _returnvalue (Class|MediaPlayer|OpenUrl _mediaplayer (.url (Variables|Default|GetCurrentMediaInfo))))
  (if _returnvalue
    (Utilities|FlowControl|Delay 0.2)
    (Media|MediaPlayer|Seek _mediaplayer (Variables|Default|GetServerMediaTime))
    (else
      (CallFunction|OnMediaOpenedFailed))))

(event Custom|Server_SetVolume
  (params (Up? :type Boolean))
  ;[0.5574 0.8041 1] Playback
  ;;[1 1 1] Set Volume
  (CallFunction|MulticastSetVolume Up? (Variables|Default|GetVolumeMultiplier)))

(event Custom|OnSeekCompleted_Event_0
  ;[1 1 1] BeginPlay
  ;;[1 1 1] Initialize OnMedia Event Bindings
  ;;;[1 1 1] OnSeekCompleted
  (Development|PrintString "OnSeekCompleted!!!!!" true true "(R=1.000000,G=0.134413,B=0.706118,A=1.000000)" 5.0)
  (switch Utilities|FlowControl|Switch|SwitchonENUM_MediaState (Variables|Default|GetMediaState)
    (:NewEnumerator5
      (Sequencer|Player|Pause (Variables|Default|GetMediaPlayer)))))

(event Custom|PlayerMediaRevised
  (params (PlayerStateName :type String))
  ;[1 1 1] BeginPlay
  ;;[1 1 1] Player event dispatchers
  ;;;[1 1 1] "Player Media Revised" event dispatcher. Called whenever a player revises their media script. We only refresh the screen when they are the current player.
  (Variables|Default|SetPlayer%20Info%20Array (Variables|/Game/SynthArchMP_Template/Blueprints/Core/GameState_SynthArchMP.GameState_SynthArchMP_C|GetPlayerInfoArray (stale EventBeginPlay _asgame_state_synth_arch_mp)))
  (if (Utilities|Enum|Equal(Enum) (.PlayerStateName (Utilities|Struct|BreakSTRUCT_PlayerInfo (Variables|Default|GetCurrentPlayerInfo))) PlayerStateName)
    (CallFunction|RefreshPlayer)))

(event Custom|RefreshPlayer
  ;[0.5574 0.8041 1] Playback
  ;;[1 1 1] Refresh Player
  (CallFunction|ServerStopMedia (.mediaformat (Variables|Default|GetCurrentMediaInfo)))
  (Variables|Default|SetCurrentMediaInfo (Utilities|Array|Get(acopy) (.MediaInfoArray (Utilities|Struct|BreakSTRUCT_PlayerInfo (Utilities|Array|Get(acopy) (Variables|Default|GetPlayer%20Info%20Array) (Variables|Default|GetPlayerIndex))))))
  (CallFunction|ServerUpdateMediaState (Variables|Default|GetPlayerIndex) 0 (Variables|Default|GetCurrentMediaInfo))
  (switch Utilities|FlowControl|Switch|SwitchonENUM_MediaFormat (.mediaformat (Variables|Default|GetCurrentMediaInfo))
    (:NewEnumerator0
      (CallFunction|ServerStopMedia "NewEnumerator0"))
    (:NewEnumerator1
      (CallFunction|ServerDisplayImage (.url (Variables|Default|GetCurrentMediaInfo))))))

(event Custom|StopMedia
  (bind _screenmoviedmi (Variables|Default|GetScreenMovieDMI))
  ;[0.5574 0.8041 1] Playback
  ;;[1 1 1] Stop
  (Variables|Default|SetMediaState "NewEnumerator1")
  (switch Utilities|FlowControl|Switch|SwitchonENUM_MediaFormat (stale Custom|Multicast_StopMedia Selection)
    (:NewEnumerator0
      (Rendering|Material|SetTextureParameterValue _screenmoviedmi "Media Texture" (Variables|Default|GetMediaTexture))
      (Rendering|Material|SetMaterial (Variables|Default|GetScreenMesh) 0 _screenmoviedmi)
      (Media|MediaPlayer|OpenSource (Variables|Default|GetMediaPlayer) "/Game/SynthArchMP_Template/Media/FMS_BlankMovie_PlayIcon.FMS_BlankMovie_PlayIcon"))))

(event Custom|PlayerInfoAdded
  ;[1 1 1] BeginPlay
  ;;[1 1 1] Player event dispatchers
  ;;;[1 1 1] "Player Info Added" event dispatcher. Updates the PlayerInfoArray whenever a player joins the game.
  (bind _output_get (Variables|Default|SetPlayer%20Info%20Array (Variables|/Game/SynthArchMP_Template/Blueprints/Core/GameState_SynthArchMP.GameState_SynthArchMP_C|GetPlayerInfoArray (stale EventBeginPlay _asgame_state_synth_arch_mp))))
  (if (> (Utilities|Array|Length _output_get) 0)
    (Utilities|FlowControl|Delay 0.2)
    (CallFunction|ServerInitMediaState)))

(event Custom|Server_SyncMedia
  (params (ServerMediaTime :type Timespan%20Structure) (MediaState :type ENUM_MediaState%20Enum :default "NewEnumerator0"))
  ;[0.3051 1 0.5352] Tick
  ;;[1 1 1] Sync Media
  (CallFunction|MulticastSyncMedia ServerMediaTime MediaState))

(event Custom|Multicast_SyncMedia
  (params (ServerMediaTime :type Timespan%20Structure) (MediaState :type ENUM_MediaState%20Enum :default "NewEnumerator0"))
  ;[0.3051 1 0.5352] Tick
  ;;[1 1 1] Sync Media
  (Variables|Default|SetServerMediaTime ServerMediaTime)
  (Variables|Default|SetMediaState MediaState)
  (CallFunction|UpdateTextInfo MediaState))

(event Custom|Server_PlayMedia_URL
  (params (MediaState :type ENUM_MediaState%20Enum :default "NewEnumerator0"))
  ;[0.5574 0.8041 1] Playback
  ;;[1 1 1] Play
  (CallFunction|MulticastPlayMediaURL MediaState))

(event Custom|Multicast_PlayMedia_URL
  (params (MediaState :type ENUM_MediaState%20Enum :default "NewEnumerator0"))
  (bind _mediaplayer (Variables|Default|GetMediaPlayer))
  ;[0.5574 0.8041 1] Playback
  ;;[1 1 1] Play
  (Variables|Default|SetMediaState MediaState)
  (switch Utilities|FlowControl|Switch|SwitchonENUM_MediaState (Variables|Default|GetMediaState)
    (:NewEnumerator5
      (Media|MediaPlayer|Play _mediaplayer :!class /Script/MediaAssets.MediaPlayer)
      (Variables|Default|SetMediaState "NewEnumerator0"))
    (:NewEnumerator1
      (bind _returnvalue (Class|MediaPlayer|OpenUrl _mediaplayer (.url (Variables|Default|GetCurrentMediaInfo)) :!label _label))
      (if _returnvalue
        (Variables|Default|SetMediaState "NewEnumerator0")
        (else
          (CallFunction|OnMediaOpenedFailed))))
    (:NewEnumerator3
      (goto _label))))

(event Custom|SyncMedia
  ;[0.3051 1 0.5352] Tick
  ;;[1 1 1] Sync Media
  (Utilities|FlowControl|Delay 1.0)
  (Networking|SwitchHasAuthority
    (:Authority
      (if (and (Networking|IsServer) (Utilities|Enum|Equal(Enum) (Variables|Default|GetMediaState) "NewEnumerator0"))
        (bind _output_get (Variables|Default|SetServerMediaTime (Class|MediaPlayer|GetTime (Variables|Default|GetMediaPlayer))))
        (CallFunction|ServerSyncMedia _output_get (Variables|Default|GetMediaState))))))

(event EventBeginPlay
  (bind _mediasound (Variables|Default|GetMediaSound))
  ;[1 1 1] BeginPlay
  (bind _asgame_instance_synth_arch_mp (Utilities|Casting|CastToGameInstance_SynthArchMP (Game|GetGameInstance)))
  (Variables|Default|SetGameInstanceRef _asgame_instance_synth_arch_mp)
  (Utilities|FlowControl|Sequence
    (:then_0
      (Rendering|SetVisibility (Variables|Default|GetDebugTesxt_Root) (Variables|Default|GetShowDebugText?) true)
      (Media|MediaSoundComponent|SetMediaPlayer _mediasound (Variables|Default|GetMediaPlayer))
      (Audio|Components|Audio|SetVolumeMultiplier _mediasound (Variables|Default|GetVolume%20Multiplier) :!class /Script/AudioMixer.SynthComponent)
      (CallFunction|InitonMediaEvents))
    (:then_1
      ;;[1 1 1] Init the "movie" dynamic texture. Open and pause the default movie source (so we avoid seeing the white blank screen on the first play).
      (bind _returnvalue (Rendering|Material|CreateDynamicMaterialInstance (Variables|Default|GetScreenMesh) 0 "/Game/SynthArchMP_Template/Media/MI_Media_Movie_1_1.MI_Media_Movie_1_1" "None" :!class /Script/Engine.PrimitiveComponent))
      (bind _output_get (Variables|Default|SetScreenMovieDMI _returnvalue))
      (Rendering|Material|SetTextureParameterValue _output_get "Media Texture" (Variables|Default|GetMediaTexture))
      (Media|MediaPlayer|OpenSource (Variables|Default|GetMediaPlayer) "/Game/SynthArchMP_Template/Media/FMS_BlankMovie_PlayIcon.FMS_BlankMovie_PlayIcon")
      ;;[1 1 1] Init the "image" dynamic texture.
      (bind _returnvalue_2 (Rendering|Material|CreateDynamicMaterialInstance (Variables|Default|GetScreenMesh) 0 "/Game/SynthArchMP_Template/Media/MI_Media_Image_1.MI_Media_Image_1" "None" :!class /Script/Engine.PrimitiveComponent))
      (bind _output_get_2 (Variables|Default|SetScreenImageDMI _returnvalue_2))
      (Rendering|Material|SetTextureParameterValue _output_get_2 "Base Texture" "/Game/SynthArchMP_Template/Textures/NoMediaIcon_1.NoMediaIcon_1"))
    (:then_2
      ;;[1 1 1] Player event dispatchers
      (bind _asgame_state_synth_arch_mp (Utilities|Casting|CastToGameState_SynthArchMP (Game|GetGameState))
        (:then
          (EventDispatchers|BindEventtoPlayerInfoAdded _asgame_state_synth_arch_mp (delegate Custom|PlayerInfoAdded))
          (EventDispatchers|BindEventtoPlayerMediaRevised _asgame_state_synth_arch_mp (delegate Custom|PlayerMediaRevised)))
        (:CastFailed
          (Development|PrintString "GameState Cast Failed!!!!!!!!!!!!!!!!!!!!!!!!!!!!" true true "(R=1.000000,G=0.528119,B=0.081323,A=1.000000)" 1e+01))))))

(event EventPushMediaButton
  (params (%20ButtonFunction :type ENUM_MediaButtonFunction%20Enum :default "NewEnumerator15") (OtherActor%20 :type Actor%20Object%20Reference) (FunctionTag%20 :type Name :default "None"))
  (bind _mediastate (Variables|Default|GetMediaState))
  ;[0.5574 0.8041 1] Playback
  ;;[0.2639 0.6697 1] Receive input from BP_MediaButton child BPs
  (if (> (Utilities|Array|Length (Variables|Default|GetPlayer%20Info%20Array)) 0)
    (switch Utilities|FlowControl|Switch|SwitchonENUM_MediaButtonFunction %20ButtonFunction
      (:NewEnumerator1
        (CallFunction|SelectPlayer false))
      (:NewEnumerator0
        (CallFunction|SelectPlayer true))
      (:NewEnumerator3
        (CallFunction|SelectTrack false))
      (:NewEnumerator2
        (CallFunction|SelectTrack true))
      (:NewEnumerator4
        (CallFunction|ServerPlayMediaURL _mediastate))
      (:NewEnumerator5
        (CallFunction|ServerPauseMedia _mediastate))
      (:NewEnumerator6
        (CallFunction|ServerStopMedia (.mediaformat (Variables|Default|GetCurrentMediaInfo))))
      (:NewEnumerator8
        (CallFunction|ServerSeekMedia false))
      (:NewEnumerator7
        (CallFunction|ServerSeekMedia true))
      (:NewEnumerator14
        (CallFunction|ServerRestartMedia _mediastate))
      (:NewEnumerator9
        (CallFunction|ServerSetVolume true))
      (:NewEnumerator10
        (CallFunction|ServerSetVolume false)))))

(event EventTick
  (params (DeltaSeconds :type Float%20%28single-precision%29))
  ;[0.3051 1 0.5352] Tick
  (CallFunction|SyncMedia))

(fn ConstructionScript
  (Rendering|SetVisibility (Variables|Default|GetDebugTesxt_Root) (Variables|Default|GetShowDebugText?) true))

(fn OnRepServerMediaTime)

(fn UpdateMediaConsoleInfo
  (bind _currentplayerinfo (Variables|Default|GetCurrentPlayerInfo))
  (bind _playerindex (Variables|Default|GetPlayerIndex))
  (bind _currentplayerinfo_2 (Variables|Default|GetCurrentPlayerInfo))
  (bind _mediaindex (Variables|Default|GetMediaIndex))
  (bind _currentplayerinfo_3 (Variables|Default|GetCurrentPlayerInfo))
  (bind _mediaindex_2 (Variables|Default|GetMediaIndex))
  (bind _playername (Utilities|Struct|BreakSTRUCT_PlayerInfo _currentplayerinfo_2))
  (bind _mediainfoarray (Utilities|Struct|BreakSTRUCT_PlayerInfo _currentplayerinfo))
  (bind _mediainfoarray_2 (Utilities|Struct|BreakSTRUCT_PlayerInfo _currentplayerinfo_3))
  (bind _returnvalue (Utilities|String|ToString(Integer) _playerindex))
  (bind _returnvalue_2 (+ _mediaindex_2 1))
  (bind _returnvalue_3 (Utilities|Array|Length _mediainfoarray_2))
  (bind _returnvalue_4 (Utilities|String|ToString(Integer) _returnvalue_2))
  (bind _returnvalue_5 (Utilities|String|Append "USER: " _returnvalue " - " _playername))
  (bind _output (Utilities|Array|Get(acopy) _mediainfoarray _mediaindex))
  (bind _returnvalue_6 (Utilities|Text|ToText(String) _returnvalue_5))
  (bind _returnvalue_7 (Utilities|String|ToString(Integer) _returnvalue_3))
  (bind _returnvalue_8 (Utilities|String|EnumtoString (.mediaformat _output)))
  (bind _returnvalue_9 (Class|KismetStringLibrary|ToUpper _returnvalue_8))
  (bind _returnvalue_10 (Utilities|String|Append "TRACK: " _returnvalue_4 " / " _returnvalue_7))
  (bind _returnvalue_11 (Utilities|Text|ToText(String) _returnvalue_10))
  (bind _returnvalue_12 (Utilities|String|Append "FORMAT: " _returnvalue_9))
  (bind _returnvalue_13 (Utilities|Text|ToText(String) _returnvalue_12))
  (Utilities|FlowControl|Sequence
    (:then_0
      (bind _asbp_umg_text_box_1 (Utilities|Casting|CastToBP_UMG_TextBox_1 (Variables|/Script/Engine.ChildActorComponent|GetChildActor (Variables|Default|GetUMG_Text_PlayerName))))
      (Default|UpdateText _asbp_umg_text_box_1 _returnvalue_6)
      (Rendering|Components|TextRender|SetText (Variables|Default|GetTextRender_User) _returnvalue_6))
    (:then_1
      (bind _asbp_umg_text_box_1_2 (Utilities|Casting|CastToBP_UMG_TextBox_1 (Variables|/Script/Engine.ChildActorComponent|GetChildActor (Variables|Default|GetUMG_Text_Track))))
      (Default|UpdateText _asbp_umg_text_box_1_2 _returnvalue_11)
      (Rendering|Components|TextRender|SetText (Variables|Default|GetTextRender_Track) _returnvalue_11))
    (:then_2
      (if (Utilities|Array|IsValidIndex _mediainfoarray _mediaindex)
        (bind _asbp_umg_text_box_1_3 (Utilities|Casting|CastToBP_UMG_TextBox_1 (Variables|/Script/Engine.ChildActorComponent|GetChildActor (Variables|Default|GetUMG_Text_Format))))
        (Default|UpdateText _asbp_umg_text_box_1_3 _returnvalue_13)
        (Rendering|Components|TextRender|SetText (Variables|Default|GetTextRender_Format) _returnvalue_13)))))

(fn UpdatePlayerIndex
  (params (Next? :type Boolean))
  (if Next?
    ;[1 1 1] Check the PlayerIndex and advance or loop to beginning
    (if (== (Utilities|Array|Length (Variables|Default|GetPlayer%20Info%20Array)) (+ (Variables|Default|GetPlayerIndex) 1))
      (Variables|Default|SetPlayerIndex 0)
      (else
        (Math|Integer|IncrementInt (Variables|Default|GetPlayerIndex)
          (:%20%20
            _))))
    (else
      ;[1 1 1] Check the PlayerIndex and reverse or loop to beginning
      (if (< (- (Variables|Default|GetPlayerIndex) 1) 0)
        (Variables|Default|SetPlayerIndex (- (Utilities|Array|Length (Variables|Default|GetPlayer%20Info%20Array)) 1))
        (else
          (Math|Integer|DecrementInt (Variables|Default|GetPlayerIndex)
            (:%20%20
              _))))))
  (bind _output_get (Variables|Default|SetCurrentMediaInfo (Utilities|Array|Get(acopy) (.MediaInfoArray (Utilities|Struct|BreakSTRUCT_PlayerInfo (Utilities|Array|Get(acopy) (Variables|Default|GetPlayer%20Info%20Array) (Variables|Default|GetPlayerIndex)))))))
  (return (Variables|Default|GetPlayerIndex) _output_get))

(fn UpdateMediaIndex
  (params (Next? :type Boolean))
  (bind _currentplayerinfo (Variables|Default|GetCurrentPlayerInfo))
  (bind _currentplayerinfo_2 (Variables|Default|GetCurrentPlayerInfo))
  (bind _mediainfoarray (Utilities|Struct|BreakSTRUCT_PlayerInfo _currentplayerinfo))
  (bind _mediainfoarray_2 (Utilities|Struct|BreakSTRUCT_PlayerInfo _currentplayerinfo_2))
  (bind _returnvalue (Utilities|Array|Length _mediainfoarray))
  (bind _returnvalue_2 (Utilities|Array|Length _mediainfoarray_2))
  (if Next?
    ;[1 1 1] Check the PlayerMediaIndex and advance or loop to beginning
    (if (> _returnvalue 0)
      (if (== _returnvalue (+ (Variables|Default|GetMediaIndex) 1))
        (Variables|Default|SetMediaIndex 0)
        (else
          (Math|Integer|IncrementInt (Variables|Default|GetMediaIndex)
            (:%20%20
              _))))
      (bind _output_get (Variables|Default|SetCurrentMediaInfo (Utilities|Array|Get(acopy) (.MediaInfoArray (Utilities|Struct|BreakSTRUCT_PlayerInfo (Variables|Default|GetCurrentPlayerInfo))) (Variables|Default|GetMediaIndex)) :!label _label))
      (return (Variables|Default|GetMediaIndex) _output_get))
    (else
      ;[1 1 1] Check the PlayerMediaIndex and reverse or loop to beginning
      (if (> _returnvalue_2 0)
        (if (< (- (Variables|Default|GetMediaIndex) 1) 0)
          (Variables|Default|SetMediaIndex (- _returnvalue_2 1))
          (goto _label)
          (else
            (Math|Integer|DecrementInt (Variables|Default|GetMediaIndex)
              (:%20%20
                (goto _label)))))))))

(fn UpdateTextInfo
  (params (Enumerator :type ENUM_MediaState%20Enum :default "NewEnumerator0"))
  (bind _mediaplayer (Variables|Default|GetMediaPlayer))
  (bind _servermediatime (Variables|Default|GetServerMediaTime))
  (bind _returnvalue (Class|KismetTextLibrary|AsTimespanTimespan _servermediatime))
  (bind _returnvalue_2 (Class|MediaPlayer|GetTime _mediaplayer))
  (bind _returnvalue_3 (Class|KismetTextLibrary|AsTimespanTimespan _returnvalue_2))
  (bind _returnvalue_4 (Utilities|String|ToString(Text) _returnvalue))
  (bind _returnvalue_5 (Utilities|String|ToString(Text) _returnvalue_3))
  (bind _returnvalue_6 (Utilities|String|Append _returnvalue_4 " / " _returnvalue_5))
  (bind _returnvalue_7 (Utilities|Text|ToText(String) _returnvalue_6))
  (Utilities|FlowControl|Sequence
    (:then_0
      (bind _asbp_umg_text_box_1 (Utilities|Casting|CastToBP_UMG_TextBox_1 (Variables|/Script/Engine.ChildActorComponent|GetChildActor (Variables|Default|GetUMG_Text_MediaTime))))
      (Default|UpdateText _asbp_umg_text_box_1 _returnvalue_7)
      (Rendering|Components|TextRender|SetText (Variables|Default|GetTextRender_MediaTime) _returnvalue_7))
    (:then_1
      ;[1 1 1] DebugText
      (if (Variables|Default|GetShowDebugText?)
        (Rendering|Components|TextRender|SetText (Variables|Default|GetTextRender_Debug_MediaTime) _returnvalue_7)
        (Rendering|Components|TextRender|SetText (Variables|Default|GetTextRender_MediaState) (Utilities|Text|ToText(String) (Utilities|String|Append "MediaState: " (Utilities|String|EnumtoString Enumerator))))
        (Rendering|Components|TextRender|SetText (Variables|Default|GetTextRender_URL) (Utilities|Text|ToText(String) (.url (Variables|Default|GetCurrentMediaInfo))))))))
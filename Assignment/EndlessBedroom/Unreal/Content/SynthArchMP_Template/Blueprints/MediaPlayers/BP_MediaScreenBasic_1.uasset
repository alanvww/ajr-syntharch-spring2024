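; Multiplayer media screen actor that plays a movie or shows a downloaded image on a mesh through dynamic materials, with optional autoplay.
; BP_MediaButton presses drive play, pause and restart, relayed by Server-to-Multicast events for movies, while images load locally.
; A Tick-driven one-second Delay multicasts server playback time, and clients seek when they drift about three seconds or more.
; Failed opens fall back to a looping missing-movie clip.
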(event Custom|Local_PlayMedia_URL
  (bind _mediaplayer (Variables|Default|GetMediaPlayer))
  ;[1 1 1] Play
  (switch Utilities|FlowControl|Switch|SwitchonENUM_MediaState (Variables|Default|GetMediaState)
    (:NewEnumerator5
      (Media|MediaPlayer|Play _mediaplayer :!class /Script/MediaAssets.MediaPlayer))
    (:NewEnumerator1
      (Media|MediaPlayer|OpenSource _mediaplayer (Variables|Default|GetMediaSource)))
    (:NewEnumerator3
      (Class|MediaPlayer|OpenUrl _mediaplayer (Variables|Default|GetMediaURL))))
  (Variables|Default|SetMediaState "NewEnumerator0"))

(event Custom|ShowImage
  (bind _screenimagedmi (Variables|Default|GetScreenImageDMI))
  (bind _texture (|DownloadImage (Variables|Default|GetMediaURL))
    (:OnSuccess
      (Rendering|Material|SetTextureParameterValue _screenimagedmi "Base Texture" _texture)
      (Rendering|Material|SetMaterial (Variables|Default|GetScreenMesh) 0 _screenimagedmi))))

(event Custom|Server_PauseMedia
  (params (MediaState :type ENUM_MediaState%20Enum :default "NewEnumerator0"))
  ;[1 1 1] Pause
  (CallFunction|MulticastPauseMedia MediaState))

(event Custom|Multicast_PauseMedia
  (params (MediaState :type ENUM_MediaState%20Enum :default "NewEnumerator0"))
  ;[1 1 1] Pause
  (Variables|Default|SetMediaState MediaState)
  (Sequencer|Player|Pause (Variables|Default|GetMediaPlayer))
  (Variables|Default|SetMediaState "NewEnumerator5"))

(event Custom|Multicast_RefreshMedia
  (params (MediaState :type ENUM_MediaState%20Enum :default "NewEnumerator0"))
  ;[1 1 1] Refresh
  (Variables|Default|SetMediaState MediaState)
  (Class|MediaPlayer|OpenUrl (Variables|Default|GetMediaPlayer) (Variables|Default|GetMediaURL))
  (Variables|Default|SetMediaState "NewEnumerator0"))

(event Custom|Server_RefreshMedia
  (params (MediaState :type ENUM_MediaState%20Enum :default "NewEnumerator0"))
  ;[1 1 1] Refresh
  (CallFunction|MulticastRefreshMedia MediaState))

(event Custom|OnMediaOpened_Event
  (params (OpenedUrl :type String))
  (bind _mediaplayer (Variables|Default|GetMediaPlayer))
  ;[1 1 1] OnMedia Event Binding
  ;;[1 1 1] OnMediaOpen
  (Components|Timeline|SetLooping _mediaplayer (Variables|Default|GetLooping?))
  (Media|MediaPlayer|Play _mediaplayer :!class /Script/MediaAssets.MediaPlayer)
  (Media|MediaPlayer|Seek _mediaplayer (Math|Timespan|MakeTimespan 0)))

(event Custom|Init_OnMedia_Events
  ;[1 1 1] OnMedia Event Binding
  (Utilities|FlowControl|Sequence
    (:then_0
      ;;[1 1 1] OnMediaOpen
      (EventDispatchers|AssignOnMediaOpened (Variables|Default|GetMediaPlayer) (delegate Custom|OnMediaOpened_Event)))
    (:then_1
      ;;[1 1 1] OnMediaOpen_Failed
      (Media|MediaPlayer|BindEventtoOnMediaOpenFailed (Variables|Default|GetMediaPlayer) (delegate Custom|OnMediaOpened_Failed)))
    (:then_2
      ;;[1 1 1] OnEndReached
      (EventDispatchers|AssignOnEndReached (Variables|Default|GetMediaPlayer) (delegate Custom|OnEndReached_Event)))))

(event Custom|OnEndReached_Event
  ;[1 1 1] OnMedia Event Binding
  ;;[1 1 1] OnEndReached
  (Variables|Default|SetMediaState "NewEnumerator1"))

(event Custom|OnMediaOpened_Failed
  (params (FailedUrl :type String))
  (bind _mediaplayer (Variables|Default|GetMediaPlayer))
  ;[1 1 1] OnMedia Event Binding
  ;;[1 1 1] OnMediaOpen_Failed
  (Media|MediaPlayer|OpenSource _mediaplayer "/Game/SynthArchMP_Template/Media/FMS_MissingMovie_PlayIcon.FMS_MissingMovie_PlayIcon")
  (Components|Timeline|SetLooping _mediaplayer true)
  (Media|MediaPlayer|Play _mediaplayer :!class /Script/MediaAssets.MediaPlayer))

(event Custom|Local_StopMedia
  ;[1 1 1] Stop
  (Media|MediaPlayer|OpenSource (Variables|Default|GetMediaPlayer) "/Game/SynthArchMP_Template/Media/FMS_BlankMovie_PlayIcon.FMS_BlankMovie_PlayIcon")
  (Variables|Default|SetMediaState "NewEnumerator1"))

(event Custom|Server_SyncMedia
  (params (ServerMediaTime :type Timespan%20Structure) (MediaState :type ENUM_MediaState%20Enum :default "NewEnumerator0"))
  ;[1 1 1] Sync Media
  (CallFunction|MulticastSyncMedia ServerMediaTime MediaState))

(event Custom|Multicast_SyncMedia
  (params (ServerMediaTime :type Timespan%20Structure) (MediaState :type ENUM_MediaState%20Enum :default "NewEnumerator0"))
  ;[1 1 1] Sync Media
  (Variables|Default|SetServerMediaTime ServerMediaTime)
  (Utilities|FlowControl|Sequence
    (:then_0
      (CallFunction|CheckClientSync))
    (:then_1
      (Rendering|Components|TextRender|SetText (Variables|Default|GetTextRender_MediaTime) (Utilities|Text|ToText(String) (Utilities|String|Append (Utilities|String|ToString(Text) (Class|KismetTextLibrary|AsTimespanTimespan (Variables|Default|GetServerMediaTime))) " / " (Utilities|String|ToString(Text) (Class|KismetTextLibrary|AsTimespanTimespan (Class|MediaPlayer|GetTime (Variables|Default|GetMediaPlayer))))))))))

(event Custom|Server_PlayMedia_URL
  (params (MediaState :type ENUM_MediaState%20Enum :default "NewEnumerator0"))
  ;[1 1 1] Play
  (CallFunction|MulticastPlayMediaURL MediaState))

(event Custom|Multicast_PlayMedia_URL
  (params (MediaState :type ENUM_MediaState%20Enum :default "NewEnumerator0"))
  (bind _mediaplayer (Variables|Default|GetMediaPlayer))
  ;[1 1 1] Play
  (Variables|Default|SetMediaState MediaState)
  (switch Utilities|FlowControl|Switch|SwitchonENUM_MediaState (Variables|Default|GetMediaState)
    (:NewEnumerator5
      (Media|MediaPlayer|Play _mediaplayer :!class /Script/MediaAssets.MediaPlayer))
    (:NewEnumerator1
      (Media|MediaPlayer|OpenSource _mediaplayer (Variables|Default|GetMediaSource)))
    (:NewEnumerator3
      (Class|MediaPlayer|OpenUrl _mediaplayer (Variables|Default|GetMediaURL))))
  (Variables|Default|SetMediaState "NewEnumerator0"))

(event Custom|SyncMedia
  ;[1 1 1] Sync Media
  (Utilities|FlowControl|Delay 1.0)
  (Networking|SwitchHasAuthority
    (:Authority
      (if (Networking|IsServer)
        (bind _output_get (Variables|Default|SetServerMediaTime (Class|MediaPlayer|GetTime (Variables|Default|GetMediaPlayer))))
        (CallFunction|ServerSyncMedia _output_get (Variables|Default|GetMediaState))))))

(event EventBeginPlay
  (bind _mediasound (Variables|Default|GetMediaSound))
  ;[1 1 1] BeginPlay
  (Utilities|FlowControl|Sequence
    (:then_0
      (Media|MediaSoundComponent|SetMediaPlayer _mediasound (Variables|Default|GetMediaPlayer))
      (Audio|Components|Audio|SetVolumeMultiplier _mediasound (Variables|Default|GetVolume%20Multiplier) :!class /Script/AudioMixer.SynthComponent)
      (CallFunction|InitonMediaEvents))
    (:then_1
      (if (Variables|Default|GetAutoPlay?)
        (switch Utilities|FlowControl|Switch|SwitchonENUM_MediaFormat (Variables|Default|GetMediaFormat)
          (:NewEnumerator0
            (bind _returnvalue (Rendering|Material|CreateDynamicMaterialInstance (Variables|Default|GetScreenMesh) 0 "/Game/SynthArchMP_Template/Media/MI_Media_Movie_1_1.MI_Media_Movie_1_1" "None" :!class /Script/Engine.PrimitiveComponent))
            (bind _output_get (Variables|Default|SetScreenMovieDMI _returnvalue))
            (Rendering|Material|SetTextureParameterValue _output_get "Media Texture" (Variables|Default|GetMediaTexture))
            (Rendering|Material|SetMaterial (Variables|Default|GetScreenMesh) 0 _output_get)
            (Variables|Default|SetMediaState "NewEnumerator1")
            (CallFunction|LocalPlayMediaURL))
          (:NewEnumerator1
            (bind _returnvalue_2 (Rendering|Material|CreateDynamicMaterialInstance (Variables|Default|GetScreenMesh) 0 "/Game/SynthArchMP_Template/Media/MI_Media_Image_1.MI_Media_Image_1" "None" :!class /Script/Engine.PrimitiveComponent))
            (bind _output_get_2 (Variables|Default|SetScreenImageDMI _returnvalue_2))
            (Rendering|Material|SetTextureParameterValue _output_get_2 "Base Texture" "/Game/SynthArchMP_Template/Textures/NoMediaIcon_1.NoMediaIcon_1")
            (Rendering|Material|SetMaterial (Variables|Default|GetScreenMesh) 0 _output_get_2)
            (CallFunction|ShowImage)
            (Variables|Default|SetMediaState "NewEnumerator1")))
        (else
          (switch Utilities|FlowControl|Switch|SwitchonENUM_MediaFormat (Variables|Default|GetMediaFormat)
            (:NewEnumerator0
              (bind _returnvalue_3 (Rendering|Material|CreateDynamicMaterialInstance (Variables|Default|GetScreenMesh) 0 "/Game/SynthArchMP_Template/Media/MI_Media_Movie_1_1.MI_Media_Movie_1_1" "None" :!class /Script/Engine.PrimitiveComponent))
              (bind _output_get_3 (Variables|Default|SetScreenMovieDMI _returnvalue_3))
              (Rendering|Material|SetTextureParameterValue _output_get_3 "Media Texture" (Variables|Default|GetMediaTexture))
              (Rendering|Material|SetMaterial (Variables|Default|GetScreenMesh) 0 _output_get_3)
              (CallFunction|LocalStopMedia)
              (Variables|Default|SetMediaState "NewEnumerator1"))
            (:NewEnumerator1
              (bind _returnvalue_4 (Rendering|Material|CreateDynamicMaterialInstance (Variables|Default|GetScreenMesh) 0 "/Game/SynthArchMP_Template/Media/MI_Media_Image_1.MI_Media_Image_1" "None" :!class /Script/Engine.PrimitiveComponent))
              (bind _output_get_4 (Variables|Default|SetScreenImageDMI _returnvalue_4))
              (Rendering|Material|SetTextureParameterValue _output_get_4 "Base Texture" "/Game/SynthArchMP_Template/Textures/NoMediaIcon_1.NoMediaIcon_1")
              (Rendering|Material|SetMaterial (Variables|Default|GetScreenMesh) 0 _output_get_4)
              (Variables|Default|SetMediaState "NewEnumerator1"))))))
    (:then_2
      (if (not (Variables|Default|GetShowPlaybackControls?))
        (CallFunction|HidePlaybackControls)))))

(event EventPushMediaButton
  (params (ButtonFunction :type ENUM_MediaButtonFunction%20Enum :default "NewEnumerator15") (OtherActor :type Actor%20Object%20Reference) (FunctionTag :type Name :default "None"))
  (bind _mediastate (Variables|Default|GetMediaState))
  ;[1 1 1] Receive input from BP_MediaButton child BPs
  (switch Utilities|FlowControl|Switch|SwitchonENUM_MediaButtonFunction ButtonFunction
    (:NewEnumerator4
      (switch Utilities|FlowControl|Switch|SwitchonENUM_MediaFormat (Variables|Default|GetMediaFormat)
        (:NewEnumerator0
          (CallFunction|ServerPlayMediaURL _mediastate))
        (:NewEnumerator1
          (CallFunction|ShowImage))))
    (:NewEnumerator5
      (CallFunction|ServerPauseMedia _mediastate))
    (:NewEnumerator14
      (CallFunction|ServerRefreshMedia _mediastate))))

(event EventTick
  (params (DeltaSeconds :type Float%20%28single-precision%29))
  ;[0.3051 1 0.5352] Tick
  (CallFunction|SyncMedia))

(fn ConstructionScript)

(fn OnRepServerMediaTime)

(fn CheckClientSync
  (bind _servermediatime (Variables|Default|GetServerMediaTime))
  (bind _mediaplayer (Variables|Default|GetMediaPlayer))
  (bind _returnvalue (Class|MediaPlayer|GetTime _mediaplayer))
  (Networking|SwitchHasAuthority
    (:Remote
      (if (== (Math|Timespan|GetMinutes _servermediatime) (Math|Timespan|GetMinutes _returnvalue))
        (if (not (< (Math|Integer|Absolute(Integer) (- (Math|Timespan|GetSeconds _servermediatime) (Math|Timespan|GetSeconds _returnvalue))) 3))
          (Media|MediaPlayer|Seek (Variables|Default|GetMediaPlayer) (Variables|Default|GetServerMediaTime) :!label _label))
        (else
          (goto _label))))))

(fn HidePlaybackControls
  (bind _buttons_root (Variables|Default|GetButtons_Root))
  (Development|SetHiddeninGame _buttons_root true true)
  (for _array_element (Components|GetChildrenComponents _buttons_root false)
    (bind _aschild_actor_component (Utilities|Casting|CastToChildActorComponent _array_element))
    (bind _asbp_media_button (Utilities|Casting|CastToBP_MediaButton (Variables|/Script/Engine.ChildActorComponent|GetChildActor _aschild_actor_component)))
    (Variables|/Game/SynthArchMP_Template/Blueprints/Buttons/BP_MediaButton.BP_MediaButton_C|SetButtonEnabled? _asbp_media_button false)))
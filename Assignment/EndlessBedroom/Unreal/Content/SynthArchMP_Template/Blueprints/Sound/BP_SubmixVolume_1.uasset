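; BP_SubmixVolume_1 is a box trigger volume that changes a submix's effects and output volume when the local player's capsule enters.
; Entry overrides the effect chain and runs an eased timeline from the game instance's stored volume to this box's, then saves it there.
; Exit waits briefly and restores the default preset, not the volume, only if no other such box overlaps the player.
; SpawnOverlap triggers the entry logic directly.
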(event OnComponentBeginOverlap(BoxCollision)
  (params (OverlappedComponent :type Primitive%20Component%20Object%20Reference) (OtherActor :type Actor%20Object%20Reference) (OtherComp :type Primitive%20Component%20Object%20Reference) (OtherBodyIndex :type Integer) (bFromSweep :type Boolean) (SweepResult :type Hit%20Result%20Structure%20%28by%20ref%29))
  (bind _returnvalue (Game|GetPlayerCharacter 0))
  ;[1 1 1] Begin Overlap
  (Utilities|IsValid _returnvalue
    (:Is%20Valid
      (if (and (== OtherActor _returnvalue) (== OtherComp (Variables|/Script/Engine.Character|GetCapsuleComponent _returnvalue)))
        (Class|AudioMixerBlueprintLibrary|SetSubmixEffectChainOverride (Variables|Default|GetSubmixRef) (Utilities|Array|MakeArray (Variables|Default|GetSubmixEffect)) 2.0)
        (CallFunction|FadeLevels)))))

(event OnComponentEndOverlap(BoxCollision)
  (params (OverlappedComponent :type Primitive%20Component%20Object%20Reference) (OtherActor :type Actor%20Object%20Reference) (OtherComp :type Primitive%20Component%20Object%20Reference) (OtherBodyIndex :type Integer))
  (bind _returnvalue (Game|GetPlayerCharacter 0))
  ;[1 1 1] End Overlap
  (Utilities|IsValid _returnvalue
    (:Is%20Valid
      (if (and (== OtherActor _returnvalue) (== OtherComp (Variables|/Script/Engine.Character|GetCapsuleComponent _returnvalue)))
        (Utilities|FlowControl|Delay 0.2)
        (if (not (> (Utilities|Array|Length (Collision|GetOverlappingActors OtherActor "BP_SubmixVolume_1_C" :!class /Script/Engine.Actor)) 0))
          (Class|AudioMixerBlueprintLibrary|SetSubmixEffectChainOverride (Variables|Default|GetSubmixRef) (Utilities|Array|MakeArray "/Game/SynthArchMP_Template/Sound/ImpulseResponse/Default_SubmixPreset.Default_SubmixPreset") 2.0))))))

(event Custom|FadeLevels
  ;[1 1 1] Fade Levels
  (Variables|Default|SetFadeA (Variables|/Game/SynthArchMP_Template/Blueprints/Core/GameInstance_SynthArchMP.GameInstance_SynthArchMP_C|GetSubmixOutputVolume (Variables|Default|GetGameInstanceRef)))
  (Variables|Default|SetFadeB (Variables|Default|GetOutputVolume))
  (Components|Timeline|SetPlayRate (Variables|Default|GetTimeline_Fade) (/ 1.0 (Variables|Default|GetFadeDuration)))
  (bind _time (Timeline|Timeline_Fade PlayFromStart)
    (:Update
      (Class|SoundSubmix|SetSubmixOutputVolume (Variables|Default|GetSubmixRef) (Math|Interpolation|Ease "EaseInOut" _time (Variables|Default|GetFadeA) (Variables|Default|GetFadeB) 2.0)))
    (:Finished
      (Variables|/Game/SynthArchMP_Template/Blueprints/Core/GameInstance_SynthArchMP.GameInstance_SynthArchMP_C|SetSubmixOutputVolume (Variables|Default|GetGameInstanceRef) (Variables|Default|GetOutputVolume)))))

(event Custom|SpawnOverlap
  ;[1 1 1] Begin Overlap
  (Class|AudioMixerBlueprintLibrary|SetSubmixEffectChainOverride (Variables|Default|GetSubmixRef) (Utilities|Array|MakeArray (Variables|Default|GetSubmixEffect)) 2.0)
  (CallFunction|FadeLevels))

(event EventBeginPlay
  ;[1 1 1] BeginPlay
  (bind _asgame_instance_synth_arch_mp (Utilities|Casting|CastToGameInstance_SynthArchMP (Game|GetGameInstance)))
  (Variables|Default|SetGameInstanceRef _asgame_instance_synth_arch_mp))

(fn ConstructionScript
  (Transformation|SetWorldRotation (Variables|Default|GetTextRender) "0, 0, 0" false false) ; Hack to make the TextRender orient correctly
  (Components|Box|SetBoxExtent (Variables|Default|GetBoxCollision) (Variables|Default|GetBoxExtent) true))
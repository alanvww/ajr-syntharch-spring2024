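; Rotating avatar display actor that shows one static mesh avatar at a time and lets other code cycle through them.
; The construction script gathers AvatarRoot's static mesh children into AvatarArray, previewing only the current index unless DisplayAll is set.
; BeginPlay caches the SynthArchMP game instance and picks a random avatar; NextAvatar and PrevAvatar step with wraparound, updating AvatarMesh.
; Tick yaws AvatarRoot by a per-frame step, unscaled by delta time.
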(event Custom|NextAvatar
  (bind _avatararray (Variables|Default|GetAvatarArray))
  (bind _avatararray_2 (Variables|Default|GetAvatarArray))
  (bind _output (Utilities|Array|Get(acopy) _avatararray))
  (Rendering|SetVisibility (Utilities|Array|Get(acopy) _avatararray_2 (Variables|Default|GetAvatarIndex)) false false)
  (if (> (+ (Variables|Default|GetAvatarIndex) 2) (Utilities|Array|Length _avatararray_2))
    (Variables|Default|SetAvatarIndex 0)
    (Rendering|SetVisibility _output true false)
    (Variables|Default|SetAvatarMesh _output)
    (else
      (bind _result (Math|Integer|IncrementInt (Variables|Default|GetAvatarIndex))
        (:%20%20
          (Rendering|SetVisibility (Utilities|Array|Get(acopy) (Variables|Default|GetAvatarArray) _result) true false)
          (Variables|Default|SetAvatarMesh (Utilities|Array|Get(acopy) (Variables|Default|GetAvatarArray) _result)))))))

(event Custom|PrevAvatar
  (bind _avatararray (Variables|Default|GetAvatarArray))
  (bind _returnvalue (Utilities|Array|LastIndex _avatararray))
  (bind _output (Utilities|Array|Get(acopy) _avatararray _returnvalue))
  (Rendering|SetVisibility (Utilities|Array|Get(acopy) (Variables|Default|GetAvatarArray) (Variables|Default|GetAvatarIndex)) false false)
  (if (> (Variables|Default|GetAvatarIndex) 0)
    (bind _result (Math|Integer|DecrementInt (Variables|Default|GetAvatarIndex))
      (:%20%20
        (Rendering|SetVisibility (Utilities|Array|Get(acopy) (Variables|Default|GetAvatarArray) _result) true false)
        (Variables|Default|SetAvatarMesh (Utilities|Array|Get(acopy) (Variables|Default|GetAvatarArray) _result))))
    (else
      (Variables|Default|SetAvatarIndex _returnvalue)
      (Rendering|SetVisibility _output true false)
      (Variables|Default|SetAvatarMesh _output))))

(event EventBeginPlay
  (bind _avatararray (Variables|Default|GetAvatarArray))
  (bind _asgame_instance_synth_arch_mp (Utilities|Casting|CastToGameInstance_SynthArchMP (Game|GetGameInstance)))
  (Variables|Default|SetGameInstanceRef _asgame_instance_synth_arch_mp)
  (Variables|Default|SetAvatarIndex (Math|Random|RandomInteger (Utilities|Array|Length _avatararray)))
  (for (_array_element _array_index) _avatararray
    (if (== _array_index (Variables|Default|GetAvatarIndex))
      (Variables|Default|SetAvatarMesh _array_element)
      (Rendering|SetVisibility _array_element true false)
      (else
        (Rendering|SetVisibility _array_element false false)))))

(event Collision|EventActorBeginOverlap
  (params (OtherActor :type Actor%20Object%20Reference)))

(event EventTick
  (params (DeltaSeconds :type Float%20%28single-precision%29))
  (Transformation|AddLocalRotation (Variables|Default|GetAvatarRoot) (Math|Rotator|MakeRotator 0.0 0.0 (Variables|Default|GetDeltaRotationZ)) false false))

(fn ConstructionScript
  (Utilities|Array|Clear (Variables|Default|GetAvatarArray))
  (for _array_element (Components|GetChildrenComponents (Variables|Default|GetAvatarRoot) false)
    (bind _asstatic_mesh_component (Utilities|Casting|CastToStaticMeshComponent _array_element))
    (Utilities|Array|Add (Variables|Default|GetAvatarArray) _asstatic_mesh_component))
  (if (not (Variables|Default|GetDisplayAll?))
    (for (_array_element_2 _array_index) (Variables|Default|GetAvatarArray)
      (Rendering|SetVisibility _array_element_2 (select (== _array_index (Variables|Default|GetAvatarIndex)) true false) false))))
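; Trigger volume that teleports the local player back to a player start when their capsule enters its box.
; After the game instance signals level load finished, it caches all enabled BP_PlayerStartCustom_1 actors.
; On overlap it uses the assigned PlayerStart or the closest cached one, adding a random XY offset.
; The move goes through ServerTeleportActor on the first-person character, falling back to the VR character, preserving rotation.
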(event OnComponentBeginOverlap(BoxCollision)
  (params (OverlappedComponent :type Primitive%20Component%20Object%20Reference) (OtherActor :type Actor%20Object%20Reference) (OtherComp :type Primitive%20Component%20Object%20Reference) (OtherBodyIndex :type Integer) (bFromSweep :type Boolean) (SweepResult :type Hit%20Result%20Structure%20%28by%20ref%29))
  (bind _returnvalue (Game|GetPlayerCharacter 0))
  (bind _playerrestartlocationramge (Variables|Default|GetPlayerRestartLocationRamge))
  (bind _gameinstanceref (Variables|Default|GetGameInstanceRef))
  (bind _playerstart (Variables|Default|GetPlayerStart))
  (bind _returnvalue_2 (* _playerrestartlocationramge -1.0))
  (bind _fp_characterref (Variables|/Game/SynthArchMP_Template/Blueprints/Core/GameInstance_SynthArchMP.GameInstance_SynthArchMP_C|GetFP_CharacterRef _gameinstanceref))
  (bind _vr_characterref (Variables|/Game/SynthArchMP_Template/Blueprints/Core/GameInstance_SynthArchMP.GameInstance_SynthArchMP_C|GetVR_CharacterRef _gameinstanceref))
  (Utilities|IsValid _returnvalue
    (:Is%20Valid
      (if (and (== OtherActor _returnvalue) (== OtherComp (Variables|/Script/Engine.Character|GetCapsuleComponent _returnvalue)))
        (Variables|Default|SetOtherActorRef OtherActor)
        (Utilities|IsValid _playerstart
          (:Is%20Valid
            (Variables|Default|SetClosestPlayerStart _playerstart))
          (:Is%20Not%20Valid
            ;[1 1 1] If no PlayerStart is assigned, find the closest PlayerStartCustom
            (Variables|Default|SetClosestPlayerStart 0)
            (Variables|Default|SetClosestPlayerStartDistance 1e+06)
            (for _array_element (Variables|Default|GetPlayerStartArray)
              (if (< (Transformation|GetDistanceTo _array_element (Variables|Default|GetOtherActorRef)) (Variables|Default|GetClosestPlayerStartDistance))
                (Variables|Default|SetClosestPlayerStartDistance (Transformation|GetDistanceTo _array_element (Variables|Default|GetOtherActorRef)))
                (Variables|Default|SetClosestPlayerStart _array_element)))))
        (Utilities|IsValid _fp_characterref
          (:Is%20Valid
            (Default|ServerTeleportActor _fp_characterref (Math|Vector|MakeVector (+ (.X (Math|Vector|BreakVector (Transformation|GetActorLocation (Variables|Default|GetClosestPlayerStart)))) (Math|Random|RandomFloatinRange _returnvalue_2 _playerrestartlocationramge)) (+ (.Y (Math|Vector|BreakVector (Transformation|GetActorLocation (Variables|Default|GetClosestPlayerStart)))) (Math|Random|RandomFloatinRange _returnvalue_2 _playerrestartlocationramge)) (.Z (Math|Vector|BreakVector (Transformation|GetActorLocation (Variables|Default|GetClosestPlayerStart))))) (Transformation|GetActorRotation (Variables|Default|GetOtherActorRef))))
          (:Is%20Not%20Valid
            (Utilities|IsValid _vr_characterref
              (:Is%20Valid
                (Default|ServerTeleportActor _vr_characterref (Math|Vector|MakeVector (+ (.X (Math|Vector|BreakVector (Transformation|GetActorLocation (Variables|Default|GetClosestPlayerStart)))) (Math|Random|RandomFloatinRange _returnvalue_2 _playerrestartlocationramge)) (+ (.Y (Math|Vector|BreakVector (Transformation|GetActorLocation (Variables|Default|GetClosestPlayerStart)))) (Math|Random|RandomFloatinRange _returnvalue_2 _playerrestartlocationramge)) (.Z (Math|Vector|BreakVector (Transformation|GetActorLocation (Variables|Default|GetClosestPlayerStart))))) (Transformation|GetActorRotation (Variables|Default|GetOtherActorRef)))))))))))

(event Custom|InitializeActor
  (Utilities|FlowControl|Sequence
    (:then_0
      (bind _outactors (Actor|GetAllActorsOfClass "/Game/SynthArchMP_Template/Blueprints/BP_PlayerStartCustom_1.BP_PlayerStartCustom_1_C"))
      (for _array_element _outactors
        (if (== (Variables|/Game/SynthArchMP_Template/Blueprints/BP_PlayerStartCustom_1.BP_PlayerStartCustom_1_C|GetEnabled? _array_element) true)
          (Utilities|Array|Add (Variables|Default|GetPlayerStartArray) _array_element))))))

(event EventBeginPlay
  (bind _asgame_instance_synth_arch_mp (Utilities|Casting|CastToGameInstance_SynthArchMP (Game|GetGameInstance)))
  (bind _output_get (Variables|Default|SetGameInstanceRef _asgame_instance_synth_arch_mp))
  (EventDispatchers|BindEventtoEDLevelLoadFinished _output_get (delegate Custom|InitializeActor)))

(event Collision|EventActorBeginOverlap
  (params (OtherActor :type Actor%20Object%20Reference)))

(event EventTick
  (params (DeltaSeconds :type Float%20%28single-precision%29)))

(fn ConstructionScript
  (Components|Box|SetBoxExtent (Variables|Default|GetBoxCollision) (Variables|Default|GetBoxExtent) true)
  (Transformation|SetWorldRotation (Variables|Default|GetTextRender) "0, 0, 0" false false) ; Hack to make the TextRender orient correctly
)
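; Spotlight fixture Blueprint that pairs a spot light with a glowing emissive mesh and supports timed fades of both.
; The construction script creates a dynamic material instance on the fixture mesh and sets its emission strength.
; FadeIntensity runs a timeline, rate-scaled to the requested duration, easing light intensity and emissive color toward their targets.
; The color fade drives all three channels from red alone, producing grayscale results.
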(event Custom|FadeIntensity
  (params (IntensityTarget :type Float%20%28double-precision%29) (FadeDuration :type Float%20%28double-precision%29) (EmissiveColorTarget :type Linear%20Color%20Structure))
  (Variables|Default|SetIntensityStart (Variables|/Script/Engine.LightComponentBase|GetIntensity (Variables|Default|GetSpotLight)))
  (Variables|Default|SetIntensityEnd IntensityTarget)
  (bind _returnvalue (Rendering|Material|GetVectorParameterValue (Variables|Default|GetDMI_EmissiveWhite) "Emissive Color" :!class /Script/Engine.MaterialInstanceDynamic))
  (Variables|Default|SetEmissiveColorCurrent _returnvalue)
  (Variables|Default|SetEmissiveColorTarget EmissiveColorTarget)
  (Components|Timeline|SetPlayRate (Variables|Default|GetTimeline_FadeIntensity) (/ 1.0 FadeDuration))
  (bind _time (Timeline|Timeline_FadeIntensity PlayFromStart)
    (:Update
      (Rendering|Components|Light|SetIntensity (Variables|Default|GetSpotLight) (Math|Interpolation|Ease "EaseInOut" _time (Variables|Default|GetIntensityStart) (Variables|Default|GetIntensityEnd) 2.0))
      (Rendering|Material|SetVectorParameterValue (Variables|Default|GetDMI_EmissiveWhite) "Emissive Color" (Utilities|Struct|MakeLinearColor (Math|Interpolation|Ease "EaseInOut" _time (.R (Utilities|Struct|BreakLinearColor (Variables|Default|GetEmissiveColorCurrent))) (.R (Utilities|Struct|BreakLinearColor (Variables|Default|GetEmissiveColorTarget))) 2.0) (Math|Interpolation|Ease "EaseInOut" _time (.R (Utilities|Struct|BreakLinearColor (Variables|Default|GetEmissiveColorCurrent))) (.R (Utilities|Struct|BreakLinearColor (Variables|Default|GetEmissiveColorTarget))) 2.0) (Math|Interpolation|Ease "EaseInOut" _time (.R (Utilities|Struct|BreakLinearColor (Variables|Default|GetEmissiveColorCurrent))) (.R (Utilities|Struct|BreakLinearColor (Variables|Default|GetEmissiveColorTarget))) 2.0) 1.0) :!class /Script/Engine.MaterialInstanceDynamic))))

(fn ConstructionScript
  (bind _returnvalue (Rendering|Material|CreateDynamicMaterialInstance (Variables|Default|GetFixtureMesh) 1 "/Game/SynthArchMP_Template/Materials/Emissive/MI_EmissiveWhite.MI_EmissiveWhite" "None" :!class /Script/Engine.PrimitiveComponent))
  (Variables|Default|SetDMI_EmissiveWhite _returnvalue)
  (Rendering|Material|SetScalarParameterValue (Variables|Default|GetDMI_EmissiveWhite) "Emission" (Variables|Default|GetMaterialEmission) :!class /Script/Engine.MaterialInstanceDynamic))
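; Trigger box volume meant to toggle a referenced planar reflection's visibility with player presence, though its BeginPlay and overlap events are empty.
; The disconnected logic shows the reflection for the player's capsule or a spawn inside the box, retrying until the player exists.
; Its hide branch first checks for overlapping volumes sharing that reflection.
; The construction script zeroes the text label's world rotation.
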(event OnComponentBeginOverlap(BoxCollision)
  (params (OverlappedComponent :type Primitive%20Component%20Object%20Reference) (OtherActor :type Actor%20Object%20Reference) (OtherComp :type Primitive%20Component%20Object%20Reference) (OtherBodyIndex :type Integer) (bFromSweep :type Boolean) (SweepResult :type Hit%20Result%20Structure%20%28by%20ref%29)))

(event OnComponentEndOverlap(BoxCollision)
  (params (OverlappedComponent :type Primitive%20Component%20Object%20Reference) (OtherActor :type Actor%20Object%20Reference) (OtherComp :type Primitive%20Component%20Object%20Reference) (OtherBodyIndex :type Integer)))

(event EventBeginPlay)

(fn ConstructionScript
  (Transformation|SetWorldRotation (Variables|Default|GetTextRender) "0, 0, 0" false false))

(fn CheckOverlappingTriggerActors
  (params (Target :type Actor%20Object%20Reference))
  (bind _array_element (Utilities|Array|ForEachLoopwithBreak (Collision|GetOverlappingActors Target "BP_PlanarReflectionTriggerVolume_1_C" :!class /Script/Engine.Actor) :!label _label)
    (:LoopBody
      (Development|PrintString (Utilities|GetDisplayName _array_element) true true "(R=0.000000,G=0.660000,B=1.000000,A=1.000000)" 1e+01)
      (bind _asbp_planar_reflection_trigger_volume_1 (Utilities|Casting|CastToBP_PlanarReflectionTriggerVolume_1 _array_element))
      (if (== (Variables|BP_PlanarReflectionTriggerVolume_1_C|GetPlanarReflectionRef _asbp_planar_reflection_trigger_volume_1) (Variables|Default|GetPlanarReflectionRef))
        (LocalVariables|SetOverlapping? true)
        (goto _label Break)))
    (:Completed
      (return (LocalVariables|GetOverlapping?)))))
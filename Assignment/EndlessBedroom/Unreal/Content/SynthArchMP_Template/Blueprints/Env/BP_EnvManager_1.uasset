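; BP_EnvManager_1 is an environment manager that fades lighting and fog over a given duration.
; FadeSettings drives two eased timelines, with play rates scaled to that duration.
; The sky light intensity fade runs only when DFAO is off in the game instance's player settings.
; The fog timeline fades volumetric fog extinction scale and also writes those same values to directional light intensity.
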(event Custom|FadeSettings
  (params (FadeDuration :type Float%20%28double-precision%29) (FadeSkyLight? :type Boolean) (SkyLightIntensity :type Float%20%28double-precision%29) (FadeFog? :type Boolean) (FogExtinctionScale :type Float%20%28double-precision%29))
  (Variables|Default|SetFade%20Duration FadeDuration)
  (Utilities|FlowControl|Sequence
    (:then_0
      ;[1 1 1] Sky Light
      (if FadeSkyLight?
        (if (not (Utilities|Struct|BreakSTRUCT_PlayerSettings_FP (Variables|/Game/SynthArchMP_Template/Blueprints/Core/GameInstance_SynthArchMP.GameInstance_SynthArchMP_C|GetPlayerSettingsFP (Variables|Default|GetGameInstanceRef))))
          (Variables|Default|SetSkyLightIntensityA (Variables|/Script/Engine.LightComponentBase|GetIntensity (Variables|/Script/Engine.SkyLight|GetLightComponent (Variables|Default|GetSkyLightRef))))
          (Variables|Default|SetSkyLightIntensityB SkyLightIntensity)
          (Components|Timeline|SetPlayRate (Variables|Default|GetTimeline_SkyLight) (/ 1.0 (Variables|Default|GetFade%20Duration)))
          (bind _time (Timeline|Timeline_SkyLight PlayFromStart)
            (:Update
              (Rendering|Components|Light|SetIntensity (Variables|/Script/Engine.SkyLight|GetLightComponent (Variables|Default|GetSkyLightRef)) (Math|Interpolation|Ease "EaseInOut" _time (Variables|Default|GetSkyLightIntensityA) (Variables|Default|GetSkyLightIntensityB) 2.0)))))))
    (:then_1
      ;[1 1 1] Fog
      (if FadeFog?
        (Variables|Default|SetFogExtinctionScaleB FogExtinctionScale)
        (Variables|Default|SetFogExtinctionScaleA (Variables|/Script/Engine.ExponentialHeightFogComponent|GetVolumetricFogExtinctionScale (Variables|/Script/Engine.ExponentialHeightFog|GetComponent (Variables|Default|GetExponentialHeightFogRef))))
        (Components|Timeline|SetPlayRate (Variables|Default|GetTimeline_Fog) (/ 1.0 (Variables|Default|GetFade%20Duration)))
        (bind _time_2 (Timeline|Timeline_Fog PlayFromStart)
          (:Update
            (Class|ExponentialHeightFogComponent|SetVolumetricFogExtinctionScale (Variables|/Script/Engine.ExponentialHeightFog|GetComponent (Variables|Default|GetExponentialHeightFogRef)) (Math|Interpolation|Ease "EaseInOut" _time_2 (Variables|Default|GetFogExtinctionScaleA) (Variables|Default|GetFogExtinctionScaleB) 2.0))
            (Rendering|Components|Light|SetIntensity (Variables|/Script/Engine.Light|GetLightComponent (Variables|Default|GetDirectionalLightRef)) (Math|Interpolation|Ease "EaseInOut" _time_2 (Variables|Default|GetFogExtinctionScaleA) (Variables|Default|GetFogExtinctionScaleB) 2.0))))))))

(event EventBeginPlay
  (bind _asgame_instance_synth_arch_mp (Utilities|Casting|CastToGameInstance_SynthArchMP (Game|GetGameInstance)))
  (Variables|Default|SetGameInstanceRef _asgame_instance_synth_arch_mp))

(event Collision|EventActorBeginOverlap
  (params (OtherActor :type Actor%20Object%20Reference)))

(event EventTick
  (params (DeltaSeconds :type Float%20%28single-precision%29)))

(fn ConstructionScript)
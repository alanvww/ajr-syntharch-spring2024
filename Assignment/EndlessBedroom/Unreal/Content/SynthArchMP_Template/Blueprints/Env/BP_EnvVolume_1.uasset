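; BP_EnvVolume_1 is a box trigger volume that changes environment lighting and fog when the local player enters it.
; When enabled, an overlap by player 0's capsule calls FadeSettings on the environment manager with the volume's fade duration, skylight and fog values.
; A SpawnOverlap event fires the same fade without the player check.
; The construction script sizes the box from BoxExtent and resets the text label's world rotation.
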(event OnComponentBeginOverlap(BoxCollision)
  (params (OverlappedComponent :type Primitive%20Component%20Object%20Reference) (OtherActor :type Actor%20Object%20Reference) (OtherComp :type Primitive%20Component%20Object%20Reference) (OtherBodyIndex :type Integer) (bFromSweep :type Boolean) (SweepResult :type Hit%20Result%20Structure%20%28by%20ref%29))
  (bind _returnvalue (Game|GetPlayerCharacter 0))
  ;[1 1 1] Begin Overlap
  (if (Variables|Default|GetEnabled?)
    (Utilities|IsValid _returnvalue
      (:Is%20Valid
        (if (and (== OtherActor _returnvalue) (== OtherComp (Variables|/Script/Engine.Character|GetCapsuleComponent _returnvalue)))
          (Default|FadeSettings (Variables|Default|GetEnvManagerRef) (Variables|Default|GetFade%20Duration) (Variables|Default|GetFade%20Sky%20Light?) (Variables|Default|GetSky%20Light%20Intensity) (Variables|Default|GetFadeFog?) (Variables|Default|GetFog%20Extinction%20Scale)))))))

(event Custom|SpawnOverlap
  ;[1 1 1] Begin Overlap
  (if (Variables|Default|GetEnabled?)
    (Default|FadeSettings (Variables|Default|GetEnvManagerRef) (Variables|Default|GetFade%20Duration) (Variables|Default|GetFade%20Sky%20Light?) (Variables|Default|GetSky%20Light%20Intensity) (Variables|Default|GetFadeFog?) (Variables|Default|GetFog%20Extinction%20Scale))))

(event EventBeginPlay
  (bind _asgame_instance_synth_arch_mp (Utilities|Casting|CastToGameInstance_SynthArchMP (Game|GetGameInstance)))
  (Variables|Default|SetGameInstanceRef _asgame_instance_synth_arch_mp))

(event Collision|EventActorBeginOverlap
  (params (OtherActor :type Actor%20Object%20Reference)))

(event EventTick
  (params (DeltaSeconds :type Float%20%28single-precision%29)))

(fn ConstructionScript
  (Transformation|SetWorldRotation (Variables|Default|GetTextRender) "0, 0, 0" false false) ; Hack to make the TextRender orient correctly
  (Components|Box|SetBoxExtent (Variables|Default|GetBoxCollision) (Variables|Default|GetBoxExtent) true))
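; BP_MediaButton is a networked push button that sends its media function and tag to its parent actor.
; A push locks the button for a trigger delay and routes through the local SynthArchMP PlayerController to the server.
; The multicast notifies the parent on authority only, while playing a sound and timeline press animation.
; The construction script applies configurable mesh, transform, material and visibility; the VR overlap trigger is unconnected.
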(event OnComponentBeginOverlap(ButtonStaticMesh)
  (params (OverlappedComponent :type Primitive%20Component%20Object%20Reference) (OtherActor :type Actor%20Object%20Reference) (OtherComp :type Primitive%20Component%20Object%20Reference) (OtherBodyIndex :type Integer) (bFromSweep :type Boolean) (SweepResult :type Hit%20Result%20Structure%20%28by%20ref%29))
  ;[1 1 1] Trigger ButtonPush with VR overlap
)

(event Custom|Server_ButtonPush
  (params (PushingActor :type Actor%20Object%20Reference))
  ;[1 1 1] ButtonPush animation
  ;;[1 0.243 0.6763] run this through PlayerController?
  (CallFunction|MulticastButtonPush PushingActor))

(event Custom|Multicast_ButtonPush
  (params (PushingActor :type Actor%20Object%20Reference))
  ;[1 1 1] ButtonPush animation
  (Networking|SwitchHasAuthority
    (:Authority
      (Class|BPIButtonActor|PushMediaButton(Message) (Actor|GetParentActor) (Variables|Default|GetButtonFunction) PushingActor (Variables|Default|GetFunctionTag)))
    (:Remote
      _))
  (Audio|PlaySoundatLocation "/Game/SynthArchMP_Template/Sound/FootstepsSounds/WaveFiles/Footsteps_Mono/Female/Concrete/Concrete_Heels_6.Concrete_Heels_6" (Transformation|GetActorLocation) "0, 0, 0" 1.0 1.0 0.0 "/Game/SynthArchMP_Template/Sound/Attenuation/FootstepsFP_SA.FootstepsFP_SA" 0 0 0)
  (bind _time (Timeline|Timeline_ButtonPush PlayFromStart)
    (:Update
      (Transformation|SetRelativeLocation (Variables|Default|GetTransform_Root) (Math|Vector|MakeVector (* _time (Variables|Default|GetButtonLocationEnd)) 0.0 0.0) false false))))

(event Custom|ButtonReset
  ;[1 1 1] Button Reset Delay
  (Variables|Default|SetButtonEnabled? false)
  (Utilities|FlowControl|Delay (Variables|Default|GetTriggerDelay))
  (Variables|Default|SetButtonEnabled? true))

(event EventBeginPlay
  ;[1 1 1] BeginPlay
  (Components|Timeline|SetPlayRate (Variables|Default|GetTimeline_ButtonPush) (/ 1.0 (Variables|Default|GetButtonPushDuration))))

(event EventPushButton
  (params (OtherActor :type Actor%20Object%20Reference) (FunctionTag :type Name :default "None"))
  ;[1 1 1] Event Push Button:
  ; Sent by FP Character from a linetrace
  (if (Variables|Default|GetButtonEnabled?)
    (CallFunction|ButtonReset)
    (bind _asplayer_controller_synth_arch_mp (Utilities|Casting|CastToPlayerController_SynthArchMP (Game|GetPlayerController 0)))
    (Default|ServerMediaButtonPush _asplayer_controller_synth_arch_mp self OtherActor)))

(fn ConstructionScript
  (bind _buttonstaticmesh (Variables|Default|GetButtonStaticMesh))
  (Components|StaticMesh|SetStaticMesh _buttonstaticmesh (Variables|Default|GetButtonMesh))
  (Transformation|SetRelativeTransform _buttonstaticmesh (Variables|Default|GetButtonMeshTransform) false false)
  (Rendering|Material|SetMaterial _buttonstaticmesh 0 (Variables|Default|GetButtonMaterial))
  (Development|SetHiddeninGame (Variables|Default|GetButtonStaticMesh) (Variables|Default|GetHiddenInGame?) false))
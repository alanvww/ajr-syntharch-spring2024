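; Procedural placement actor that builds a 3D grid of repeated meshes or child actors by floor, row and item in its Construction Script.
; Nested loops compose each transform from step offsets, seeded stream randomness and optional alternating 180-degree flips.
; RepeatType outputs Static Mesh components, per-mesh ISM/HISM instances or child actors, with meshes picked randomly or in sequence.
; An optional HISM fix nudges X/Y scale to avoid a rotation rounding bug.
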(event EventBeginPlay)

(event Collision|EventActorBeginOverlap
  (params (OtherActor :type Actor%20Object%20Reference)))

(event EventTick
  (params (DeltaSeconds :type Float%20%28single-precision%29)))

(fn ConstructionScript
  (bind _stream (Variables|Default|GetStream))
  (bind _stream_2 (Variables|Default|GetStream))
  (bind _stream_3 (Variables|Default|GetStream))
  (bind _baserotation (Variables|Rotation|GetBaseRotation))
  (bind _itemrotationmultiplier (Variables|Rotation|GetItemRotationMultiplier))
  (bind _repeatmesharray (Variables|Default|GetRepeatMeshArray))
  (bind _stream_4 (Variables|Default|GetStream))
  (bind _itemrotationrandommin (Variables|Rotation|GetItemRotationRandomMin))
  (bind _materialinstancearray (Variables|Default|GetMaterialInstanceArray))
  (bind _itemrotationrandommax (Variables|Rotation|GetItemRotationRandomMax))
  (bind _itemscalemultiplier (Variables|Scale|GetItemScaleMultiplier))
  (bind _itemrotation (Variables|Rotation|GetItemRotation))
  (bind _hism_ref_array (Variables|Default|GetHISM_Ref_Array))
  (bind _ism_ref_array (Variables|Default|GetISM_Ref_Array))
  (bind _itemscale_randommin (Variables|Scale|GetItemScale_RandomMin))
  (bind _itemscale_randommax (Variables|Scale|GetItemScale_RandomMax))
  (bind _itemlocation (Variables|Location|GetItemLocation))
  (bind _itemlocationrandommin (Variables|Location|GetItemLocationRandomMin))
  (bind _itemscale (Variables|Scale|GetItemScale))
  (bind _itemlocationrandommax (Variables|Location|GetItemLocationRandomMax))
  (bind _floorlocation (Variables|Location|GetFloorLocation))
  (bind _rowlocation (Variables|Location|GetRowLocation))
  (bind _rowlocationrandommin (Variables|Location|GetRowLocationRandomMin))
  (bind _rowlocationrandommax (Variables|Location|GetRowLocationRandomMax))
  (bind _stream_5 (Variables|Default|GetStream))
  (bind _floorlocationrandommin (Variables|Location|GetFloorLocationRandomMin))
  (bind _floorlocationrandommax (Variables|Location|GetFloorLocationRandomMax))
  (bind _stream_6 (Variables|Default|GetStream))
  (bind _stream_7 (Variables|Default|GetStream))
  (bind _returnvalue (Utilities|Array|Length _repeatmesharray))
  (bind _returnvalue_2 (Utilities|Array|Length _ism_ref_array))
  (bind _returnvalue_3 (Math|Random|RandomFloatinRangefromStream _itemscale_randommin _itemscale_randommax _stream_7))
  (bind (_x _y _z) (Math|Vector|BreakVector _itemscale))
  (bind _returnvalue_4 (- _returnvalue 1))
  (bind _returnvalue_5 (- _returnvalue_2 1))
  (bind _returnvalue_6 (Math|Random|RandomIntegerinRangefromStream 0 _returnvalue_5 _stream_2))
  (bind _returnvalue_7 (Math|Random|RandomIntegerinRangefromStream 0 _returnvalue_4 _stream_4))
  (switch Utilities|FlowControl|Switch|SwitchonEnum_ProceduralType (Variables|Default|GetRepeatType)
    (:NewEnumerator3
      _)
    (:NewEnumerator0
      ;[1 1 1] Generate Instance Component
      (Utilities|Array|Clear (Variables|Default|GetISM_Ref_Array))
      (for _index (range 0 (- (Utilities|Array|Length (Variables|Default|GetRepeatMeshArray)) 1))
        (bind _returnvalue_8 (AddComponent|AddInstancedStaticMeshComponent false))
        (Utilities|Array|Add (Variables|Default|GetISM_Ref_Array) _returnvalue_8)
        (Components|StaticMesh|SetStaticMesh _returnvalue_8 (Utilities|Array|Get(acopy) (Variables|Default|GetRepeatMeshArray) _index))
        (Rendering|Material|SetMaterial _returnvalue_8 0 (Utilities|Array|Get(acopy) (Variables|Default|GetMaterialInstanceArray) _index))
        (Class|PrimitiveComponent|SetPhysMaterialOverride _returnvalue_8 (Utilities|Array|Get(acopy) (Variables|Default|GetPhysicalMaterialArray) _index))
        (Rendering|SetCastShadow _returnvalue_8 (Variables|Default|GetCastShadows?))
        (Collision|SetCollisionResponsetoChannel _returnvalue_8 "ECC_GameTraceChannel1" (select (Variables|Default|GetOccludeSound?) "ECR_Block" "ECR_Ignore"))
        (Collision|SetCollisionEnabled _returnvalue_8 (select (Variables|Default|GetCollisionEnabled?) "QueryAndPhysics" "NoCollision"))
        (Transformation|SetMobility _returnvalue_8 (Variables|Lighting|GetMobility))
        (Rendering|Components|SetLightingChannels _returnvalue_8 (Variables|Lighting|GetLightingChannel0?) (Variables|Lighting|GetLightingChannel1?) (Variables|Lighting|GetLightingChannel2?))))
    (:NewEnumerator2
      ;[1 1 1] Generate Hierarchical Instance Component
      (Utilities|Array|Clear (Variables|Default|GetHISM_Ref_Array))
      (for _index_2 (range 0 (- (Utilities|Array|Length (Variables|Default|GetRepeatMeshArray)) 1))
        (bind _returnvalue_9 (AddComponent|AddHierarchicalInstancedStaticMeshComponent false))
        (Utilities|Array|Add (Variables|Default|GetHISM_Ref_Array) _returnvalue_9)
        (Components|StaticMesh|SetStaticMesh _returnvalue_9 (Utilities|Array|Get(acopy) (Variables|Default|GetRepeatMeshArray) _index_2))
        (Rendering|Material|SetMaterial _returnvalue_9 0 (Utilities|Array|Get(acopy) (Variables|Default|GetMaterialInstanceArray) _index_2))
        (Class|PrimitiveComponent|SetPhysMaterialOverride _returnvalue_9 (Utilities|Array|Get(acopy) (Variables|Default|GetPhysicalMaterialArray) _index_2))
        (Rendering|SetCastShadow _returnvalue_9 (Variables|Default|GetCastShadows?))
        (Collision|SetCollisionResponsetoChannel _returnvalue_9 "ECC_GameTraceChannel1" (select (Variables|Default|GetOccludeSound?) "ECR_Block" "ECR_Ignore"))
        (Collision|SetCollisionEnabled _returnvalue_9 (select (Variables|Default|GetCollisionEnabled?) "QueryAndPhysics" "NoCollision"))
        (Transformation|SetMobility _returnvalue_9 (Variables|Lighting|GetMobility))
        (Rendering|Components|SetLightingChannels _returnvalue_9 (Variables|Lighting|GetLightingChannel0?) (Variables|Lighting|GetLightingChannel1?) (Variables|Lighting|GetLightingChannel2?))))
    (:NewEnumerator1
      _))
  (Utilities|Array|Clear (Variables|Default|GetTotalNumberOfItems))
  ;[0.3083 0.573 1] Make Floors
  (for _index_3 (range 0 (- (Variables|Default|GetNumberOfFloors) 1))
    (Variables|Default|SetFloorIndex _index_3)
    ;;[1 1 1] Set Floor random values
    (Variables|Location|SetFloorX_Random (Math|Random|RandomFloatinRangefromStream (.x _floorlocationrandommin) (.x _floorlocationrandommax) _stream_6))
    (Variables|Location|SetFloorY_Random (Math|Random|RandomFloatinRangefromStream (.y _floorlocationrandommin) (.y _floorlocationrandommax) _stream_6))
    (Variables|Location|SetFloorZ_Random (Math|Random|RandomFloatinRangefromStream (.z _floorlocationrandommin) (.z _floorlocationrandommax) _stream_6))
    ;[0.6198 1 0.6633] Make Rows
    (for _index_4 (range 0 (- (Variables|Default|GetNumberOfRows) 1))
      (Variables|Default|SetRowIndex _index_4)
      ;;[1 1 1] Set Row random values
      (Variables|Location|SetRowX_Random (Math|Random|RandomFloatinRangefromStream (.x _rowlocationrandommin) (.x _rowlocationrandommax) _stream_5))
      (Variables|Location|SetRowY_Random (Math|Random|RandomFloatinRangefromStream (.y _rowlocationrandommin) (.y _rowlocationrandommax) _stream_5))
      (Variables|Location|SetRowZ_Random (Math|Random|RandomFloatinRangefromStream (.z _rowlocationrandommin) (.z _rowlocationrandommax) _stream_5))
      ;;[1 1 1] Row Rotation FlipFlop
      (if (Variables|Rotation|GetRowRotX_FlipFlop?)
        (Utilities|FlowControl|FlipFlop
          (:A
            (Variables|Rotation|SetRowRotX_FlipFlop 0.0))
          (:B
            (Variables|Rotation|SetRowRotX_FlipFlop 1.8e+02))))
      (if (Variables|Rotation|GetRowRotY_FlipFlop?)
        (Utilities|FlowControl|FlipFlop
          (:A
            (Variables|Rotation|SetRowRotY_FlipFlop 0.0))
          (:B
            (Variables|Rotation|SetRowRotY_FlipFlop 1.8e+02))))
      (if (Variables|Rotation|GetRowRotZ_FlipFlop?)
        (Utilities|FlowControl|FlipFlop
          (:A
            (Variables|Rotation|SetRowRotZ_FlipFlop 0.0))
          (:B
            (Variables|Rotation|SetRowRotZ_FlipFlop 1.8e+02))))
      ;[1 0.4479 0.4479] Make Items
      (for _index_5 (range 0 (- (Variables|Default|GetNumberOfItems) 1))
        (Variables|Default|SetItemIndex _index_5)
        ;;[1 1 1] Item Rotation FlipFlop
        (if (Variables|Rotation|GetRotX_FlipFlop?)
          (Utilities|FlowControl|FlipFlop
            (:A
              (Variables|Rotation|SetItemRotX_FlipFlop 0.0))
            (:B
              (Variables|Rotation|SetItemRotX_FlipFlop 1.8e+02))))
        (if (Variables|Rotation|GetRotY_FlipFlop?)
          (Utilities|FlowControl|FlipFlop
            (:A
              (Variables|Rotation|SetItemRotY_FlipFlop 0.0))
            (:B
              (Variables|Rotation|SetItemRotY_FlipFlop 1.8e+02))))
        (if (Variables|Rotation|GetRotZ_FlipFlop?)
          (Utilities|FlowControl|FlipFlop
            (:A
              (Variables|Rotation|SetItemRotZ_FlipFlop 0.0))
            (:B
              (Variables|Rotation|SetItemRotZ_FlipFlop 1.8e+02))))
        (Variables|Default|SetItemTransform (Math|Transform|MakeTransform (+ (Variables|Location|GetBaseLocation) (Math|Vector|MakeVector (+ (+ (* (.x _itemlocation) (Math|Conversions|ToFloat(Integer) (Variables|Default|GetItemIndex))) (Math|Random|RandomFloatinRangefromStream (.x _itemlocationrandommin) (.x _itemlocationrandommax) _stream)) (+ (+ (* (.x _rowlocation) (Math|Conversions|ToFloat(Integer) (Variables|Default|GetRowIndex))) (Variables|Location|GetRowX_Random)) (+ (* (.x _floorlocation) (Math|Conversions|ToFloat(Integer) (Variables|Default|GetFloorIndex))) (Variables|Location|GetFloorX_Random)))) (+ (+ (* (.y _itemlocation) (Math|Conversions|ToFloat(Integer) (Variables|Default|GetItemIndex))) (Math|Random|RandomFloatinRangefromStream (.y _itemlocationrandommin) (.y _itemlocationrandommax) _stream)) (+ (+ (* (.y _rowlocation) (Math|Conversions|ToFloat(Integer) (Variables|Default|GetRowIndex))) (Variables|Location|GetRowY_Random)) (+ (* (.y _floorlocation) (Math|Conversions|ToFloat(Integer) (Variables|Default|GetFloorIndex))) (Variables|Location|GetFloorY_Random)))) (+ (+ (* (.z _itemlocation) (Math|Conversions|ToFloat(Integer) (Variables|Default|GetItemIndex))) (Math|Random|RandomFloatinRangefromStream (.z _itemlocationrandommin) (.z _itemlocationrandommax) _stream)) (+ (+ (* (.z _rowlocation) (Math|Conversions|ToFloat(Integer) (Variables|Default|GetRowIndex))) (Variables|Location|GetRowZ_Random)) (+ (* (.z _floorlocation) (Math|Conversions|ToFloat(Integer) (Variables|Default|GetFloorIndex))) (Variables|Location|GetFloorZ_Random)))))) (Math|Rotator|MakeRotator (+ (.roll _baserotation) (+ (+ (+ (.roll _itemrotation) (* (.roll _itemrotationmultiplier) (Math|Conversions|ToFloat(Integer) (Variables|Default|GetItemIndex)))) (Math|Random|RandomFloatinRangefromStream (.roll _itemrotationrandommin) (.roll _itemrotationrandommax) _stream_3)) (+ (Variables|Rotation|GetItemRotX_FlipFlop) (Variables|Rotation|GetRowRotX_FlipFlop)))) (+ (.pitch _baserotation) (+ (+ (+ (.pitch _itemrotation) (* (Math|Conversions|ToFloat(Integer) (Variables|Default|GetItemIndex)) (.pitch _itemrotationmultiplier))) (Math|Random|RandomFloatinRangefromStream (.pitch _itemrotationrandommin) (.pitch _itemrotationrandommax) _stream_3)) (+ (Variables|Rotation|GetItemRotY_FlipFlop) (Variables|Rotation|GetRowRotY_FlipFlop)))) (+ (.yaw _baserotation) (+ (+ (+ (.yaw _itemrotation) (* (Math|Conversions|ToFloat(Integer) (Variables|Default|GetItemIndex)) (.yaw _itemrotationmultiplier))) (Math|Random|RandomFloatinRangefromStream (.yaw _itemrotationrandommin) (.yaw _itemrotationrandommax) _stream_3)) (+ (Variables|Rotation|GetItemRotZ_FlipFlop) (Variables|Rotation|GetRowRotZ_FlipFlop))))) (Math|Vector|MakeVector (* (+ _x (* (.x _itemscalemultiplier) (Math|Conversions|ToFloat(Integer) (Variables|Default|GetItemIndex)))) _returnvalue_3) (* (+ _y (* (.y _itemscalemultiplier) (Math|Conversions|ToFloat(Integer) (Variables|Default|GetItemIndex)))) _returnvalue_3) (* (+ _z (* (.z _itemscalemultiplier) (Math|Conversions|ToFloat(Integer) (Variables|Default|GetItemIndex)))) _returnvalue_3))))
        (Utilities|Array|Add (Variables|Default|GetTotalNumberOfItems) (Variables|Default|GetItemIndex))
        (switch Utilities|FlowControl|Switch|SwitchonEnum_ProceduralType (Variables|Default|GetRepeatType)
          (:NewEnumerator3
            ;[1 1 1] Mesh Instance Construction
            (if (Variables|Default|GetRandomizeMeshes?)
              ;;[1 1 1] Randomize Meshes
              (Variables|Default|SetRepeatMesh (Utilities|Array|Get(acopy) _repeatmesharray _returnvalue_7))
              (Variables|Default|SetPhysicalMaterial (Utilities|Array|Get(acopy) (Variables|Default|GetPhysicalMaterialArray) _returnvalue_7))
              (else
                ;;[1 1 1] Sequence Meshes
                (if (== (Variables|Default|GetItemIndex) 0) ; Reset if first Item in Row
                  (Variables|Default|SetRepeatMeshArrayIndex 0))
                (Variables|Default|SetRepeatMesh (Utilities|Array|Get(acopy) (Variables|Default|GetRepeatMeshArray) (Variables|Default|GetRepeatMeshArrayIndex)))
                (Variables|Default|SetPhysicalMaterial (Utilities|Array|Get(acopy) (Variables|Default|GetPhysicalMaterialArray) (Variables|Default|GetRepeatMeshArrayIndex)))
                (if (> (+ (Variables|Default|GetRepeatMeshArrayIndex) 1) (- (Utilities|Array|Length (Variables|Default|GetRepeatMeshArray)) 1)) ; Reset after last Item in Repeat Mesh Array
                  (Variables|Default|SetRepeatMeshArrayIndex 0)
                  (else
                    (Math|Integer|IncrementInt (Variables|Default|GetRepeatMeshArrayIndex)
                      (:%20%20
                        _))))))
            ;[1 1 1] Material Instance Construction
            (if (Variables|Default|GetRandomizeMaterials?)
              ;;[1 1 1] Randomize Materials
              (Variables|Default|SetRepeatMeshMaterialInstance (Utilities|Array|Get(acopy) _materialinstancearray (Math|Random|RandomIntegerinRangefromStream 0 (- (Utilities|Array|Length _materialinstancearray) 1) (Variables|Default|GetStream))))
              (else
                ;;[1 1 1] Sequence Materials
                (if (== (Variables|Default|GetItemIndex) 0) ; Reset if first Item in Row
                  (Variables|Default|SetMaterialInstanceArrayIndex 0))
                (Variables|Default|SetRepeatMeshMaterialInstance (Utilities|Array|Get(acopy) (Variables|Default|GetMaterialInstanceArray) (Variables|Default|GetMaterialInstanceArrayIndex)))
                (if (> (+ (Variables|Default|GetMaterialInstanceArrayIndex) 1) (- (Utilities|Array|Length (Variables|Default|GetMaterialInstanceArray)) 1))
                  (Variables|Default|SetMaterialInstanceArrayIndex 0)
                  (else
                    (Math|Integer|IncrementInt (Variables|Default|GetMaterialInstanceArrayIndex)
                      (:%20%20
                        _))))))
            ;[1 1 1] Static Mesh Properties
            (bind _returnvalue_10 (AddComponent|AddStaticMeshComponent false (Variables|Default|GetItemTransform)))
            (Components|StaticMesh|SetStaticMesh _returnvalue_10 (Variables|Default|GetRepeatMesh))
            (Rendering|Material|SetMaterial _returnvalue_10 0 (Variables|Default|GetRepeatMeshMaterialInstance))
            (Class|PrimitiveComponent|SetPhysMaterialOverride _returnvalue_10 (Variables|Default|GetPhysicalMaterial))
            (Rendering|SetCastShadow _returnvalue_10 (Variables|Default|GetCastShadows?))
            (Collision|SetCollisionResponsetoChannel _returnvalue_10 "ECC_GameTraceChannel1" (select (Variables|Default|GetOccludeSound?) "ECR_Block" "ECR_Ignore"))
            (Collision|SetCollisionEnabled _returnvalue_10 (select (Variables|Default|GetCollisionEnabled?) "QueryAndPhysics" "NoCollision"))
            (Transformation|SetMobility _returnvalue_10 (Variables|Lighting|GetMobility))
            (Rendering|Components|SetLightingChannels _returnvalue_10 (Variables|Lighting|GetLightingChannel0?) (Variables|Lighting|GetLightingChannel1?) (Variables|Lighting|GetLightingChannel2?)))
          (:NewEnumerator0
            ;[1 1 1] ISM - Mesh Instance Construction
            (if (Variables|Default|GetRandomizeMeshes?)
              ;;[1 1 1] Randomize Meshes
              (Variables|Default|SetISM_Ref (Utilities|Array|Get(acopy) _ism_ref_array _returnvalue_6))
              (Development|PrintString (Utilities|String|Append (Utilities|String|ToString(Integer) (Utilities|Array|Length (Variables|Default|GetTotalNumberOfItems))) "    " (Utilities|String|ToString(Integer) _returnvalue_6)))
              (else
                ;;[1 1 1] Sequence Meshes
                (if (== (Variables|Default|GetItemIndex) 0) ; Reset if first Item in Row
                  (Variables|Default|SetRepeatMeshArrayIndex 0))
                (Variables|Default|SetISM_Ref (Utilities|Array|Get(acopy) (Variables|Default|GetISM_Ref_Array) (Variables|Default|GetRepeatMeshArrayIndex)))
                (if (> (+ (Variables|Default|GetRepeatMeshArrayIndex) 1) (- (Utilities|Array|Length (Variables|Default|GetISM_Ref_Array)) 1)) ; Reset after last Item in Repeat Mesh Array
                  (Variables|Default|SetRepeatMeshArrayIndex 0)
                  (else
                    (Math|Integer|IncrementInt (Variables|Default|GetRepeatMeshArrayIndex)
                      (:%20%20
                        _))))))
            (Components|InstancedStaticMesh|AddInstance (Variables|Default|GetISM_Ref) (Variables|Default|GetItemTransform) false))
          (:NewEnumerator2
            ;[1 1 1] HISM - Mesh Instance Construction
            (if (Variables|Default|GetRandomizeMeshes?)
              ;;[1 1 1] Randomize Mesh Ordering
              (Variables|Default|SetHISM_Ref (Utilities|Array|Get(acopy) _hism_ref_array (Math|Random|RandomIntegerinRangefromStream 0 (- (Utilities|Array|Length _hism_ref_array) 1) (Variables|Default|GetStream))))
              (else
                ;;[1 1 1] Sequence Mesh Ordering
                (if (== (Variables|Default|GetItemIndex) 0) ; Reset if first Item in Row
                  (Variables|Default|SetRepeatMeshArrayIndex 0))
                (Variables|Default|SetHISM_Ref (Utilities|Array|Get(acopy) (Variables|Default|GetHISM_Ref_Array) (Variables|Default|GetRepeatMeshArrayIndex)))
                (if (> (+ (Variables|Default|GetRepeatMeshArrayIndex) 1) (- (Utilities|Array|Length (Variables|Default|GetHISM_Ref_Array)) 1)) ; Reset after last Item in Repeat Mesh Array
                  (Variables|Default|SetRepeatMeshArrayIndex 0)
                  (else
                    (Math|Integer|IncrementInt (Variables|Default|GetRepeatMeshArrayIndex)
                      (:%20%20
                        _))))))
            (Components|InstancedStaticMesh|AddInstance (Variables|Default|GetHISM_Ref) (select (Variables|Scale|GetHISM_ScaleFix?) (Math|Transform|MakeTransform (.location (Variables|Default|GetItemTransform)) (.rotation (Variables|Default|GetItemTransform)) (Math|Vector|MakeVector (+ (.x (.scale (Variables|Default|GetItemTransform))) 0.0001) (+ (.y (.scale (Variables|Default|GetItemTransform))) 0.0001) (.z (.scale (Variables|Default|GetItemTransform))))) (Variables|Default|GetItemTransform)) false))
          (:NewEnumerator1
            ;[1 1 1] Actor
            (bind _returnvalue_11 (AddComponent|AddChildActorComponent false (Math|Transform|MakeTransform "0, 0, 0")))
            (ChildActorComponent|SetChildActorClass _returnvalue_11 (Variables|Default|GetMyActorClass))
            (Transformation|SetRelativeTransform _returnvalue_11 (Variables|Default|GetItemTransform) false false)))))))

(fn FlipFlopRotationRandom
  (bind _stream (Variables|Default|GetStream))
  (if (Variables|Rotation|GetRotX_FlipFlopRandom?)
    (switch int (Class|KismetMathLibrary|RandomIntegerfromStream 2 _stream)
      (:0
        _)
      (:1
        _))
    (Variables|Rotation|SetItemRotX_FlipFlop 0.0))
  (if (Variables|Rotation|GetRotY_FlipFlopRandom?)
    (switch int (Class|KismetMathLibrary|RandomIntegerfromStream 2 _stream)
      (:0
        (Variables|Rotation|SetItemRotY_FlipFlop 0.0))
      (:1
        (Variables|Rotation|SetItemRotY_FlipFlop 1.8e+02))))
  (if (Variables|Rotation|GetRotZ_FlipFlopRandom?)
    (switch int (Class|KismetMathLibrary|RandomIntegerfromStream 2 _stream)
      (:0
        (Variables|Rotation|SetItemRotZ_FlipFlop 0.0))
      (:1
        (Variables|Rotation|SetItemRotZ_FlipFlop 1.8e+02)))))

(fn FlipFlopRotation
  (if (Variables|Rotation|GetRotX_FlipFlop?)
    (Utilities|FlowControl|FlipFlop
      (:A
        (Variables|Rotation|SetItemRotX_FlipFlop 0.0))
      (:B
        (Variables|Rotation|SetItemRotX_FlipFlop 1.8e+02))))
  (if (Variables|Rotation|GetRotY_FlipFlop?)
    (Utilities|FlowControl|FlipFlop
      (:A
        (Variables|Rotation|SetItemRotY_FlipFlop 0.0))
      (:B
        (Variables|Rotation|SetItemRotY_FlipFlop 1.8e+02))))
  (if (Variables|Rotation|GetRotZ_FlipFlop?)
    (Utilities|FlowControl|FlipFlop
      (:A
        (Variables|Rotation|SetItemRotZ_FlipFlop 0.0))
      (:B
        (Variables|Rotation|SetItemRotZ_FlipFlop 1.8e+02))))
  (return))
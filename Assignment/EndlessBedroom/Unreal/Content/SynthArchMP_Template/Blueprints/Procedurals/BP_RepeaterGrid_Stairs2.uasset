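; Procedural grid repeater, apparently for stairs, that builds rows of repeated items in the construction script.
; Each transform combines item and row offsets, seeded random jitter and optional 180-degree flip-flop rotations.
; RepeatType selects static mesh, ISM, HISM or child actor output, with meshes randomized or sequenced per row.
; Only the HISM path adds per-step collision boxes sized from mesh bounds, plus an optional scale nudge working around a rotation rounding bug.
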(event EventBeginPlay)

(event Collision|EventActorBeginOverlap
  (params (OtherActor :type Actor%20Object%20Reference)))

(event EventTick
  (params (DeltaSeconds :type Float%20%28single-precision%29)))

(fn ConstructionScript
  (bind _stream (Variables|Default|GetStream))
  (bind _stream_2 (Variables|Default|GetStream))
  (bind _stream_3 (Variables|Default|GetStream))
  (bind _baserotation (Variables|Rotation|GetBaseRotation))
  (bind _repeatmesharray (Variables|Default|GetRepeatMeshArray))
  (bind _materialinstancearray (Variables|Default|GetMaterialInstanceArray))
  (bind _hism_ref_array (Variables|Default|GetHISM_Ref_Array))
  (bind _ism_ref_array (Variables|Default|GetISM_Ref_Array))
  (bind _stream_4 (Variables|Default|GetStream))
  (bind _returnvalue (Utilities|Array|Length _ism_ref_array))
  (bind _returnvalue_2 (- _returnvalue 1))
  (bind _returnvalue_3 (Math|Random|RandomIntegerinRangefromStream 0 _returnvalue_2 _stream_2))
  (switch Utilities|FlowControl|Switch|SwitchonEnum_RepeaterType (Variables|Default|GetRepeatType)
    (:NewEnumerator3
      _)
    (:NewEnumerator0
      ;[1 1 1] Generate Instance Component
      (Utilities|Array|Clear (Variables|Default|GetISM_Ref_Array))
      (for _index (range 0 (- (Utilities|Array|Length (Variables|Default|GetRepeatMeshArray)) 1))
        (bind _returnvalue_4 (AddComponent|AddInstancedStaticMeshComponent false))
        (Utilities|Array|Add (Variables|Default|GetISM_Ref_Array) _returnvalue_4)
        (Components|StaticMesh|SetStaticMesh _returnvalue_4 (Utilities|Array|Get(acopy) (Variables|Default|GetRepeatMeshArray) _index))
        (Rendering|Material|SetMaterial _returnvalue_4 0 (Utilities|Array|Get(acopy) (Variables|Default|GetMaterialInstanceArray) _index))
        (Rendering|SetCastShadow _returnvalue_4 (Variables|Default|GetCastShadows?))
        (Collision|SetCollisionEnabled _returnvalue_4 (select (Variables|Default|GetCollisionEnabled?) "QueryAndPhysics" "NoCollision"))))
    (:NewEnumerator2
      ;[1 1 1] Generate Hierarchical Instance Component
      (Utilities|Array|Clear (Variables|Default|GetHISM_Ref_Array))
      (for _index_2 (range 0 (- (Utilities|Array|Length (Variables|Default|GetRepeatMeshArray)) 1))
        (bind _returnvalue_5 (AddComponent|AddHierarchicalInstancedStaticMeshComponent false))
        (Utilities|Array|Add (Variables|Default|GetHISM_Ref_Array) _returnvalue_5)
        (Components|StaticMesh|SetStaticMesh _returnvalue_5 (Utilities|Array|Get(acopy) (Variables|Default|GetRepeatMeshArray) _index_2))
        (Rendering|Material|SetMaterial _returnvalue_5 0 (Utilities|Array|Get(acopy) (Variables|Default|GetMaterialInstanceArray) _index_2))
        (Rendering|SetCastShadow _returnvalue_5 (Variables|Default|GetCastShadows?))
        (Collision|SetCollisionEnabled _returnvalue_5 (select (Variables|Default|GetCollisionEnabled?) "QueryAndPhysics" "NoCollision"))
        (Transformation|SetMobility _returnvalue_5 (Variables|Default|GetMobility))
        (Rendering|Components|SetLightingChannels _returnvalue_5 (Variables|Default|GetLightingChannel0?) (Variables|Default|GetLightingChannel1?) (Variables|Default|GetLightingChannel2?))))
    (:NewEnumerator1
      _))
  (Utilities|Array|Clear (Variables|Default|GetNumberOfItems))
  ;[1 1 1] Make Rows and first Item in each
  (for _index_3 (range 0 (- (Variables|Default|GetNumberOfRows) 1))
    (Variables|Default|SetRowIndex _index_3)
    ;[1 1 1] Set Row random values
    (Variables|Location|SetRowX_Random (Math|Random|RandomFloatinRangefromStream (Variables|Location|GetRowX_RandomMin) (Variables|Location|GetRowX_RandomMax) _stream_4))
    (Variables|Location|SetRowY_Random (Math|Random|RandomFloatinRangefromStream (Variables|Location|GetRowY_RandomMin) (Variables|Location|GetRowY_RandomMax) _stream_4))
    (Variables|Location|SetRowZ_Random (Math|Random|RandomFloatinRangefromStream (Variables|Location|GetRowZ_RandomMin) (Variables|Location|GetRowZ_RandomMax) _stream_4))
    ;[1 1 1] Row Rotation FlipFlop
    (if (Variables|Rotation|GetRowRotX_FlipFlop?)
      (Utilities|FlowControl|FlipFlop
        (:A
          (Variables|Rotation|SetRowRotX_FlipFlop 0.0))
        (:B
          (Variables|Rotation|SetRowRotX_FlipFlop 1.8e+02))))
    (if (Variables|Rotation|GetRowRotY_FlipFlop?)
      (Utilities|FlowControl|FlipFlop
        (:A
          (Variables|Rotation|SetRowRotY_FlipFlop 0.0))
        (:B
          (Variables|Rotation|SetRowRotY_FlipFlop 1.8e+02))))
    (if (Variables|Rotation|GetRowRotZ_FlipFlop?)
      (Utilities|FlowControl|FlipFlop
        (:A
          (Variables|Rotation|SetRowRotZ_FlipFlop 0.0))
        (:B
          (Variables|Rotation|SetRowRotZ_FlipFlop 1.8e+02))))
    ;[1 1 1] Make Items in each Row
    (for _index_4 (range 0 (- (Variables|Default|GetNumberOfItemsPerRow) 1))
      (Variables|Default|SetItemIndex _index_4)
      ;[1 1 1] Item Rotation FlipFlop
      (if (Variables|Rotation|GetRotX_FlipFlop?)
        (Utilities|FlowControl|FlipFlop
          (:A
            (Variables|Rotation|SetItemRotX_FlipFlop 0.0))
          (:B
            (Variables|Rotation|SetItemRotX_FlipFlop 1.8e+02))))
      (if (Variables|Rotation|GetRotY_FlipFlop?)
        (Utilities|FlowControl|FlipFlop
          (:A
            (Variables|Rotation|SetItemRotY_FlipFlop 0.0))
          (:B
            (Variables|Rotation|SetItemRotY_FlipFlop 1.8e+02))))
      (if (Variables|Rotation|GetRotZ_FlipFlop?)
        (Utilities|FlowControl|FlipFlop
          (:A
            (Variables|Rotation|SetItemRotZ_FlipFlop 0.0))
          (:B
            (Variables|Rotation|SetItemRotZ_FlipFlop 1.8e+02))))
      (Variables|Default|SetItemTransform (Math|Transform|MakeTransform (+ (Variables|Location|GetBaseLocation) (Math|Vector|MakeVector (+ (+ (* (Variables|Location|GetItemX) (Math|Conversions|ToFloat(Integer) (Variables|Default|GetItemIndex))) (Math|Random|RandomFloatinRangefromStream (Variables|Location|GetItemX_RandomMin) (Variables|Location|GetItemX_RandomMax) _stream)) (+ (* (Variables|Location|GetRowX) (Math|Conversions|ToFloat(Integer) (Variables|Default|GetRowIndex))) (Variables|Location|GetRowX_Random))) (+ (+ (* (Variables|Location|GetItemY) (Math|Conversions|ToFloat(Integer) (Variables|Default|GetItemIndex))) (Math|Random|RandomFloatinRangefromStream (Variables|Location|GetItemY_RandomMin) (Variables|Location|GetItemY_RandomMax) _stream)) (+ (* (Variables|Location|GetRowY) (Math|Conversions|ToFloat(Integer) (Variables|Default|GetRowIndex))) (Variables|Location|GetRowY_Random))) (+ (+ (* (Variables|Location|GetItemZ) (Math|Conversions|ToFloat(Integer) (Variables|Default|GetItemIndex))) (Math|Random|RandomFloatinRangefromStream (Variables|Location|GetItemZ_RandomMin) (Variables|Location|GetItemZ_RandomMax) _stream)) (+ (* (Variables|Location|GetRowZ) (Math|Conversions|ToFloat(Integer) (Variables|Default|GetRowIndex))) (Variables|Location|GetRowZ_Random))))) (Math|Rotator|MakeRotator (+ (.roll _baserotation) (+ (+ (+ (Variables|Rotation|GetItemRotX) (* (Variables|Rotation|GetItemRotX_Multiplier) (Math|Conversions|ToFloat(Integer) (Variables|Default|GetItemIndex)))) (Math|Random|RandomFloatinRangefromStream (Variables|Rotation|GetItemRotX_RandomMax) (Variables|Rotation|GetItemRotX_RandomMin) _stream_3)) (+ (Variables|Rotation|GetItemRotX_FlipFlop) (Variables|Rotation|GetRowRotX_FlipFlop)))) (+ (.pitch _baserotation) (+ (+ (+ (Variables|Rotation|GetItemRotY) (* (Math|Conversions|ToFloat(Integer) (Variables|Default|GetItemIndex)) (Variables|Rotation|GetItemRotY_Multiplier))) (Math|Random|RandomFloatinRangefromStream (Variables|Rotation|GetItemRotY_RandomMin) (Variables|Rotation|GetItemRotY_RandomMax) _stream_3)) (+ (Variables|Rotation|GetItemRotY_FlipFlop) (Variables|Rotation|GetRowRotY_FlipFlop)))) (+ (.yaw _baserotation) (+ (+ (+ (Variables|Rotation|GetItemRotZ) (* (Math|Conversions|ToFloat(Integer) (Variables|Default|GetItemIndex)) (Variables|Rotation|GetItemRotZ_Multiplier))) (Math|Random|RandomFloatinRangefromStream (Variables|Rotation|GetItemRotZ_RandomMin) (Variables|Rotation|GetItemRotZ_RandomMax) _stream_3)) (+ (Variables|Rotation|GetItemRotZ_FlipFlop) (Variables|Rotation|GetRowRotZ_FlipFlop))))) (Variables|Scale|GetItemScale)))
      (Utilities|Array|Add (Variables|Default|GetNumberOfItems) 0)
      (switch Utilities|FlowControl|Switch|SwitchonEnum_RepeaterType (Variables|Default|GetRepeatType)
        (:NewEnumerator3
          ;[1 1 1] Mesh Instance Construction
          (if (Variables|Default|GetRandomizeMeshes?)
            ;;[1 1 1] Randomize Meshes
            (Variables|Default|SetRepeatMesh (Utilities|Array|Get(acopy) _repeatmesharray (Math|Random|RandomIntegerinRangefromStream 0 (- (Utilities|Array|Length _repeatmesharray) 1) (Variables|Default|GetStream))))
            (else
              ;;[1 1 1] Sequence Meshes
              (if (== (Variables|Default|GetItemIndex) 0) ; Reset if first Item in Row
                (Variables|Default|SetRepeatMeshArrayIndex 0))
              (Variables|Default|SetRepeatMesh (Utilities|Array|Get(acopy) (Variables|Default|GetRepeatMeshArray) (Variables|Default|GetRepeatMeshArrayIndex)))
              (if (> (+ (Variables|Default|GetRepeatMeshArrayIndex) 1) (- (Utilities|Array|Length (Variables|Default|GetRepeatMeshArray)) 1)) ; Reset after last Item in Repeat Mesh Array
                (Variables|Default|SetRepeatMeshArrayIndex 0)
                (else
                  (Math|Integer|IncrementInt (Variables|Default|GetRepeatMeshArrayIndex)
                    (:%20%20
                      _))))))
          ;[1 1 1] Material Instance Construction
          (if (Variables|Default|GetRandomizeMaterials?)
            ;;[1 1 1] Randomize Materials
            (Variables|Default|SetRepeatMeshMaterialInstance (Utilities|Array|Get(acopy) _materialinstancearray (Math|Random|RandomIntegerinRangefromStream 0 (- (Utilities|Array|Length _materialinstancearray) 1) (Variables|Default|GetStream))))
            (else
              ;;[1 1 1] Sequence Materials
              (if (== (Variables|Default|GetItemIndex) 0) ; Reset if first Item in Row
                (Variables|Default|SetMaterialInstanceArrayIndex 0))
              (Variables|Default|SetRepeatMeshMaterialInstance (Utilities|Array|Get(acopy) (Variables|Default|GetMaterialInstanceArray) (Variables|Default|GetMaterialInstanceArrayIndex)))
              (if (> (+ (Variables|Default|GetMaterialInstanceArrayIndex) 1) (- (Utilities|Array|Length (Variables|Default|GetMaterialInstanceArray)) 1))
                (Variables|Default|SetMaterialInstanceArrayIndex 0)
                (else
                  (Math|Integer|IncrementInt (Variables|Default|GetMaterialInstanceArrayIndex)
                    (:%20%20
                      _))))))
          ;[1 1 1] Static Mesh Properties
          (bind _returnvalue_6 (AddComponent|AddStaticMeshComponent false (Variables|Default|GetItemTransform)))
          (Components|StaticMesh|SetStaticMesh _returnvalue_6 (Variables|Default|GetRepeatMesh))
          (Rendering|Material|SetMaterial _returnvalue_6 0 (Variables|Default|GetRepeatMeshMaterialInstance))
          (Rendering|SetCastShadow _returnvalue_6 (Variables|Default|GetCastShadows?))
          (Collision|SetCollisionEnabled _returnvalue_6 (select (Variables|Default|GetCollisionEnabled?) "QueryAndPhysics" "NoCollision"))
          (Development|PrintString (Utilities|String|Append "INDEX:  " (Utilities|String|ToString(Integer) (Utilities|Array|Length (Variables|Default|GetRepeatMeshArray))) "  TRANSFORM:  " (Utilities|String|ToString(Rotator) (.rotation (Transformation|GetWorldTransform _returnvalue_6))))))
        (:NewEnumerator0
          ;[1 1 1] ISM - Mesh Instance Construction
          (if (Variables|Default|GetRandomizeMeshes?)
            ;;[1 1 1] Randomize Meshes
            (Variables|Default|SetISM_Ref (Utilities|Array|Get(acopy) _ism_ref_array _returnvalue_3))
            (Development|PrintString (Utilities|String|Append (Utilities|String|ToString(Integer) (Utilities|Array|Length (Variables|Default|GetNumberOfItems))) "    " (Utilities|String|ToString(Integer) _returnvalue_3)))
            (else
              ;;[1 1 1] Sequence Meshes
              (if (== (Variables|Default|GetItemIndex) 0) ; Reset if first Item in Row
                (Variables|Default|SetRepeatMeshArrayIndex 0))
              (Variables|Default|SetISM_Ref (Utilities|Array|Get(acopy) (Variables|Default|GetISM_Ref_Array) (Variables|Default|GetRepeatMeshArrayIndex)))
              (if (> (+ (Variables|Default|GetRepeatMeshArrayIndex) 1) (- (Utilities|Array|Length (Variables|Default|GetISM_Ref_Array)) 1)) ; Reset after last Item in Repeat Mesh Array
                (Variables|Default|SetRepeatMeshArrayIndex 0)
                (else
                  (Math|Integer|IncrementInt (Variables|Default|GetRepeatMeshArrayIndex)
                    (:%20%20
                      _))))))
          (Components|InstancedStaticMesh|AddInstance (Variables|Default|GetISM_Ref) (Variables|Default|GetItemTransform) false))
        (:NewEnumerator2
          ;[1 1 1] HISM - Mesh Instance Construction
          (if (Variables|Default|GetRandomizeMeshes?)
            ;;[1 1 1] Randomize Mesh Ordering
            (Variables|Default|SetHISM_Ref (Utilities|Array|Get(acopy) _hism_ref_array (Math|Random|RandomIntegerinRangefromStream 0 (- (Utilities|Array|Length _hism_ref_array) 1) (Variables|Default|GetStream))))
            (else
              ;;[1 1 1] Sequence Mesh Ordering
              (if (== (Variables|Default|GetItemIndex) 0) ; Reset if first Item in Row
                (Variables|Default|SetRepeatMeshArrayIndex 0))
              (Variables|Default|SetHISM_Ref (Utilities|Array|Get(acopy) (Variables|Default|GetHISM_Ref_Array) (Variables|Default|GetRepeatMeshArrayIndex)))
              (if (> (+ (Variables|Default|GetRepeatMeshArrayIndex) 1) (- (Utilities|Array|Length (Variables|Default|GetHISM_Ref_Array)) 1)) ; Reset after last Item in Repeat Mesh Array
                (Variables|Default|SetRepeatMeshArrayIndex 0)
                (else
                  (Math|Integer|IncrementInt (Variables|Default|GetRepeatMeshArrayIndex)
                    (:%20%20
                      _))))))
          (Components|InstancedStaticMesh|AddInstance (Variables|Default|GetHISM_Ref) (select (Variables|Scale|GetHISM_ScaleFix?) (Math|Transform|MakeTransform (.location (Variables|Default|GetItemTransform)) (.rotation (Variables|Default|GetItemTransform)) (Math|Vector|MakeVector (+ (.x (.scale (Variables|Default|GetItemTransform))) 0.0001) (+ (.y (.scale (Variables|Default|GetItemTransform))) 0.0001) (.z (.scale (Variables|Default|GetItemTransform))))) (Variables|Default|GetItemTransform)) false)
          ;[1 1 1] Make Step Collision
          (bind _returnvalue_7 (AddComponent|AddBoxComponent false (Math|Transform|MakeTransform (+ (.Location (Math|Transform|BreakTransform (Variables|Default|GetItemTransform))) (Variables|Collision|GetStepCollisionLocationOffset)) (Variables|Collision|GetStepCollisionRotation) (Variables|Collision|GetStepCollisionScale))))
          (Components|Box|SetBoxExtent _returnvalue_7 (.BoxExtent (Math|BoxSphereBounds|BreakBoxSphereBounds (StaticMesh|GetBounds (Variables|/Script/Engine.StaticMeshComponent|GetStaticMesh (Variables|Default|GetHISM_Ref))))) true)
          (Collision|SetCollisionEnabled _returnvalue_7 (select (Variables|Collision|GetEnableStepCollision?) "QueryAndPhysics" "NoCollision"))
          (Rendering|SetVisibility _returnvalue_7 (Variables|Collision|GetStepCollisionVisible?) false))
        (:NewEnumerator1
          ;[1 1 1] Actor
          (bind _returnvalue_8 (AddComponent|AddChildActorComponent false (Math|Transform|MakeTransform "0, 0, 0")))
          (ChildActorComponent|SetChildActorClass _returnvalue_8 (Variables|Default|GetMyActorClass))
          (Transformation|SetRelativeTransform _returnvalue_8 (Variables|Default|GetItemTransform) false false))))))

(fn FlipFlopRotationRandom
  (bind _stream (Variables|Default|GetStream))
  (if (Variables|Rotation|GetRotX_FlipFlopRandom?)
    (switch int (Class|KismetMathLibrary|RandomIntegerfromStream 2 _stream)
      (:0
        _)
      (:1
        _))
    (Variables|Rotation|SetItemRotX_FlipFlop 0.0))
  (if (Variables|Rotation|GetRotY_FlipFlopRandom?)
    (switch int (Class|KismetMathLibrary|RandomIntegerfromStream 2 _stream)
      (:0
        (Variables|Rotation|SetItemRotY_FlipFlop 0.0))
      (:1
        (Variables|Rotation|SetItemRotY_FlipFlop 1.8e+02))))
  (if (Variables|Rotation|GetRotZ_FlipFlopRandom?)
    (switch int (Class|KismetMathLibrary|RandomIntegerfromStream 2 _stream)
      (:0
        (Variables|Rotation|SetItemRotZ_FlipFlop 0.0))
      (:1
        (Variables|Rotation|SetItemRotZ_FlipFlop 1.8e+02)))))

(fn FlipFlopRotation
  (if (Variables|Rotation|GetRotX_FlipFlop?)
    (Utilities|FlowControl|FlipFlop
      (:A
        (Variables|Rotation|SetItemRotX_FlipFlop 0.0))
      (:B
        (Variables|Rotation|SetItemRotX_FlipFlop 1.8e+02))))
  (if (Variables|Rotation|GetRotY_FlipFlop?)
    (Utilities|FlowControl|FlipFlop
      (:A
        (Variables|Rotation|SetItemRotY_FlipFlop 0.0))
      (:B
        (Variables|Rotation|SetItemRotY_FlipFlop 1.8e+02))))
  (if (Variables|Rotation|GetRotZ_FlipFlop?)
    (Utilities|FlowControl|FlipFlop
      (:A
        (Variables|Rotation|SetItemRotZ_FlipFlop 0.0))
      (:B
        (Variables|Rotation|SetItemRotZ_FlipFlop 1.8e+02))))
  (return))
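; First-person character prototype with custom surface gravity, using Flying movement and capsule-relative move input plus controller look.
; Each tick, GravityLineTrace traces from the capsule toward its up vector times -1000, not offset by capsule location.
; On a hit, it applies movement along the negated normal (positive for near-X-aligned normals) and interpolates capsule roll and pitch to the surface.
; Debug traces and prints remain; RotateOnSlope, a world-down variant, is unused.
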(event EventBeginPlay
  (Pawn|Components|CharacterMovement|SetMovementMode (Variables|Character|GetCharacterMovement) "MOVE_Flying" 0))

(event Collision|EventActorBeginOverlap
  (params (OtherActor :type Actor%20Object%20Reference)))

(event EventTick
  (params (DeltaSeconds :type Float%20%28single-precision%29))
  (CallFunction|GravityLineTrace))

(event Input|AxisEvents|InputAxisMoveForward
  (params (AxisValue :type Float%20%28single-precision%29))
  (Pawn|Input|AddMovementInput (Math|Vector|GetForwardVector (Variables|Collision|GetCapsuleComponent)) AxisValue false))

(event Input|AxisEvents|InputAxisLookPitch
  (params (AxisValue :type Float%20%28single-precision%29))
  (Pawn|Input|AddControllerPitchInput AxisValue))

(event Input|AxisEvents|InputAxisLookYaw
  (params (AxisValue :type Float%20%28single-precision%29))
  (Pawn|Input|AddControllerYawInput AxisValue))

(event Input|AxisEvents|InputAxisMoveStrafe
  (params (AxisValue :type Float%20%28single-precision%29))
  (Pawn|Input|AddMovementInput (Math|Vector|GetRightVector (Variables|Collision|GetCapsuleComponent)) AxisValue false))

(fn ConstructionScript)

(fn GravityLineTrace
  (bind _capsulecomponent (Variables|Collision|GetCapsuleComponent))
  (bind _capsulecomponent_2 (Variables|Collision|GetCapsuleComponent))
  (bind _returnvalue (Transformation|GetWorldRotation _capsulecomponent_2))
  (bind (_outhit _returnvalue_2) (Collision|LineTraceForObjects (Transformation|GetWorldLocation _capsulecomponent) (* (Math|Vector|GetUpVector _capsulecomponent) -1e+03) (Utilities|Array|MakeArray "ObjectTypeQuery1" "ObjectTypeQuery2") false 0 "ForDuration"))
  (if _returnvalue_2
    (Development|PrintString (Utilities|String|ToString(Vector) (.ImpactNormal (Collision|BreakHitResult _outhit))) true true "(R=0.000000,G=0.114498,B=1.000000,A=1.000000)" 1.0)
    (Pawn|Input|AddMovementInput (* (.ImpactNormal (Collision|BreakHitResult _outhit)) (select (< (Math|Float|Absolute(Float) (.X (Math|Vector|BreakVector (.ImpactNormal (Collision|BreakHitResult _outhit))))) 0.99) -1.0 1.0)) 1.0 false)
    (Transformation|SetWorldRotation _capsulecomponent_2 (Math|Interpolation|RInterpTo _returnvalue (Math|Rotator|MakeRotator (.Roll (Math|Rotator|BreakRotator (Math|Rotator|MakeRotfromXZ (Math|Vector|GetForwardVector _capsulecomponent_2) (.ImpactNormal (Collision|BreakHitResult _outhit))))) (.Pitch (Math|Rotator|BreakRotator (Class|KismetMathLibrary|MakeRotfromYZ (Math|Vector|GetRightVector _capsulecomponent_2) (.ImpactNormal (Collision|BreakHitResult _outhit))))) (.Yaw (Math|Rotator|BreakRotator _returnvalue))) (Utilities|Time|GetWorldDeltaSeconds) 5e+01) false false)
    (Development|PrintString (Utilities|String|ToString(Rotator) (Math|Interpolation|RInterpTo _returnvalue (Math|Rotator|MakeRotator (.Roll (Math|Rotator|BreakRotator (Math|Rotator|MakeRotfromXZ (Math|Vector|GetForwardVector _capsulecomponent_2) (.ImpactNormal (Collision|BreakHitResult _outhit))))) (.Pitch (Math|Rotator|BreakRotator (Class|KismetMathLibrary|MakeRotfromYZ (Math|Vector|GetRightVector _capsulecomponent_2) (.ImpactNormal (Collision|BreakHitResult _outhit))))) (.Yaw (Math|Rotator|BreakRotator _returnvalue))) (Utilities|Time|GetWorldDeltaSeconds) 5e+01)) true true "(R=0.000000,G=0.660000,B=1.000000,A=1.000000)" 1.0)))

(fn RotateonSlope
  (bind _returnvalue (Transformation|GetActorLocation))
  (bind _capsulecomponent (Variables|Collision|GetCapsuleComponent))
  (bind (_x _y _z) (Math|Vector|BreakVector _returnvalue))
  (bind _returnvalue_2 (Transformation|GetWorldRotation _capsulecomponent))
  (bind (_outhit _returnvalue_3) (Collision|LineTraceByChannel _returnvalue (Math|Vector|MakeVector _x _y (- _z 1e+03)) "TraceTypeQuery1" false 0 "ForDuration"))
  (if _returnvalue_3
    (Transformation|SetWorldRotation _capsulecomponent (Math|Interpolation|RInterpTo _returnvalue_2 (Math|Rotator|MakeRotator (.Roll (Math|Rotator|BreakRotator (Math|Rotator|MakeRotfromXZ (Math|Vector|GetForwardVector _capsulecomponent) (.ImpactNormal (Collision|BreakHitResult _outhit))))) (.Pitch (Math|Rotator|BreakRotator (Class|KismetMathLibrary|MakeRotfromYZ (Math|Vector|GetRightVector _capsulecomponent) (.ImpactNormal (Collision|BreakHitResult _outhit))))) (.Yaw (Math|Rotator|BreakRotator _returnvalue_2))) (Utilities|Time|GetWorldDeltaSeconds) 5e+01) false false)
    (Pawn|Input|AddMovementInput (* (.ImpactNormal (Collision|BreakHitResult _outhit)) -1.0) 1.0 false)))
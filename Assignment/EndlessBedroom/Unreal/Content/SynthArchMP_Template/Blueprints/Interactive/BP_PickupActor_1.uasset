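; BP_PickupActor_1 is a physics-driven pickup actor that can be grabbed and dropped in both VR and first-person play.
; BeginPlay configures physics and pawn collision; optional custom gravity replaces engine gravity with a per-tick Z force plus a startup spin impulse, optionally randomized.
; Pickup disables simulation and attaches the mesh, with optional location snapping for first-person only.
; Drop detaches the actor and restores physics and collision settings.
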(event EventBeginPlay
  (bind _staticmesh (Variables|Default|GetStaticMesh))
  (bind _angularimpulsex (Variables|Default|GetAngularImpulseX))
  (bind _angularimpulsey (Variables|Default|GetAngularImpulseY))
  (bind _angularimpulsez (Variables|Default|GetAngularImpulseZ))
  (bind _returnvalue (Math|Vector|MakeVector _angularimpulsex _angularimpulsey _angularimpulsez))
  ;[1 1 1] BeginPlay
  (Physics|SetSimulatePhysics _staticmesh (Variables|Default|GetSimulatePhysics?))
  (Collision|SetCollisionResponsetoChannel _staticmesh "ECC_Pawn" (Variables|Default|GetCollisionResponse))
  (Physics|SetEnableGravity _staticmesh (not (Variables|Default|GetCustomGravity?)))
  ;;[1 1 1] Add angular impulse(rotation) if using custom gravity.
  (if (Variables|Default|GetCustomGravity?)
    (Class|PrimitiveComponent|AddAngularImpulseinRadians _staticmesh (select (Variables|Default|GetRandomImpulseDirection?) (* (Math|Random|RandomUnitVector) _returnvalue) _returnvalue) "None" false)))

(event EventTick
  (params (DeltaSeconds :type Float%20%28single-precision%29))
  (bind _staticmesh (Variables|Default|GetStaticMesh))
  ;[1 1 1] Tick
  ;;[1 1 1] Custom gravity by adding force in the Z axis
  (if (and (Physics|IsSimulatingPhysics (Variables|Default|GetStaticMesh) "None") (Variables|Default|GetCustomGravity?))
    (Physics|AddForce _staticmesh (Math|Vector|MakeVector 0.0 0.0 (Variables|Default|GetCustomGravity)) "None" true)
    (Class|PrimitiveComponent|SetAngularDamping _staticmesh 0.0)))

(event EventPickup
  (params (MotionControllerRef :type Scene%20Component%20Object%20Reference) (AttachTo :type Scene%20Component%20Object%20Reference) (PawnRef :type Actor%20Object%20Reference) (SnapToTarget? :type Boolean))
  (bind _staticmesh (Variables|Default|GetStaticMesh))
  (bind _staticmesh_2 (Variables|Default|GetStaticMesh))
  ;[1 1 1] Pickup
  (Utilities|IsValid MotionControllerRef
    (:Is%20Valid
      ;;[1 1 1] VR Pickup
      (Physics|SetSimulatePhysics _staticmesh_2 false)
      (Transformation|AttachComponentToComponent _staticmesh_2 AttachTo "None" "KeepWorld" "KeepWorld" "KeepWorld" false))
    (:Is%20Not%20Valid
      ;;[1 1 1] FP Pickup
      (Physics|SetSimulatePhysics _staticmesh false)
      (Transformation|AttachComponentToComponent _staticmesh AttachTo "None" (select SnapToTarget? "SnapToTarget" "KeepWorld") "KeepWorld" "KeepWorld" false))))

(event EventDrop
  (bind _staticmesh (Variables|Default|GetStaticMesh))
  ;[1 1 1] Drop
  (Development|PrintString "Drop")
  ;;[1 1 1] Call Detach and reset Physics and Collision
  (Transformation|DetachFromActor "KeepWorld" "KeepWorld" "KeepWorld")
  (Physics|SetSimulatePhysics _staticmesh (Variables|Default|GetSimulatePhysics?))
  (Collision|SetCollisionResponsetoChannel _staticmesh "ECC_Pawn" (Variables|Default|GetCollisionResponse)))

(fn ConstructionScript)
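; Player controller for the SynthArch multiplayer template that relays client requests to server-side logic, since clients can only run server events through their controller.
; It forwards spawn requests from the player options widget to the GameMode and media and lift button pushes to multicast events on the target Blueprint actors.
; Player media revisions go to the GameState, which replicates the player info array.
; BeginPlay caches the GameInstance.
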(event Custom|Server_SpawnPlayer
  (params (PlayerInfo :type STRUCT%20Player%20Info%20Structure))
  ;[1 1 1] Blueprint Actor events initiated by Clients that must run on the Server.
  ; [Clients can only run events on the Server via PlayerController]
  ; We get a reference to BP Actor requesting the Server event, then the Server runs the event in the BP Actor.
  ;;[1 1 1] Called by the client's Player Options widget (BPW_PlayerOptions)
  (bind _asgame_mode_synth_arch_mp (Utilities|Casting|CastToGameMode_SynthArchMP (Game|GetGameMode)))
  (Default|SpawnPlayer _asgame_mode_synth_arch_mp self PlayerInfo))

(event Custom|Server_MediaButtonPush
  (params (BP_Target :type BP%20Media%20Button%20Object%20Reference) (PushingActor :type Actor%20Object%20Reference))
  ;[1 1 1] Blueprint Actor events initiated by Clients that must run on the Server.
  ; [Clients can only run events on the Server via PlayerController]
  ; We get a reference to BP Actor requesting the Server event, then the Server runs the event in the BP Actor.
  (Default|MulticastButtonPush BP_Target PushingActor))

(event Custom|Server_LiftButtonPush
  (params (BP_Target :type BP%20Lift%20Button%20Object%20Reference) (PushingActor :type Actor%20Object%20Reference))
  ;[1 1 1] Blueprint Actor events initiated by Clients that must run on the Server.
  ; [Clients can only run events on the Server via PlayerController]
  ; We get a reference to BP Actor requesting the Server event, then the Server runs the event in the BP Actor.
  (Default|MulticastButtonPush BP_Target PushingActor))

(event Custom|RevisePlayerMedia
  (params (PlayerInfo :type STRUCT%20Player%20Info%20Structure) (PlayerStateName :type String))
  ;[1 1 1] Blueprint Actor events initiated by Clients that must run on the Server.
  ; [Clients can only run events on the Server via PlayerController]
  ; We get a reference to BP Actor requesting the Server event, then the Server runs the event in the BP Actor.
  ;;[1 1 1] The PlayerInfoArray is handled and replicated in the Gamestate.
  (bind _asgame_state_synth_arch_mp (Utilities|Casting|CastToGameState_SynthArchMP (Game|GetGameState)))
  (Default|ServerRevisePlayerMedia _asgame_state_synth_arch_mp PlayerInfo PlayerStateName))

(event EventBeginPlay
  ;[1 1 1] BeginPlay
  (bind _asgame_instance_synth_arch_mp (Utilities|Casting|CastToGameInstance_SynthArchMP (Game|GetGameInstance)))
  (Variables|Default|SetGameInstanceRef _asgame_instance_synth_arch_mp))

(event Input|KeyboardEvents|Escape
  (params (Key :type Key%20Structure :default "None"))
  ;[1 1 1] Input Events (shared by the Lobby, FP and VR pawns)
)

(fn ConstructionScript)
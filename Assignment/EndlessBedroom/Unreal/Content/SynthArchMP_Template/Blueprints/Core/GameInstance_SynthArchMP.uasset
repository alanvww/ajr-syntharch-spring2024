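; Game Instance for the SynthArchMP template that persists first-person and VR player settings and holds the player's media playlist.
; Update functions apply graphics through console commands and light components, while a frame-time benchmark picks and saves a scalability level.
; Media scripts become image/video lists by file extension, with revisions sent to the server through the PlayerController.
; Dev game modes get test playlists; InitSettings_FP/VR are empty, their former logic disconnected.
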(event Custom|LevelLoadFinished
  ;[1 1 1] Init
  ;;[1 1 1] LevelLoadFinished
  (Utilities|FlowControl|Sequence
    (:then_0
      (bind _outactors (Actor|GetAllActorsOfClass "/Script/Engine.DirectionalLight"))
      (Variables|Default|SetDirectionalLight (Utilities|Array|Get(acopy) _outactors))
      (bind _outactors_2 (Actor|GetAllActorsOfClass "/Script/Engine.SkyLight"))
      (Variables|Default|SetSkyLight (Utilities|Array|Get(acopy) _outactors_2)))
    (:then_1
      (Variables|Default|SetLevelLoaded? true)
      (Default|CallEDLevelLoadFinished)
      (Development|PrintString "LevelLoadFinished!!!!!" true true "(R=0.037104,G=0.276042,B=0.075449,A=1.000000)"))))

(event Custom|NewPlayerSpawned
  ;[1 1 1] Init
  (Default|CallEDNewPlayerSpawned))

(event Custom|SaveGameAndQuit
  (bind _savegameref (Variables|Default|GetSaveGameRef))
  ;[1 1 1] Init
  ;;[1 1 1] Save Events
  (Variables|/Game/SynthArchMP_Template/Blueprints/Core/SaveGame_SynthArchMP.SaveGame_SynthArchMP_C|SetPlayerSettingsFP _savegameref (Variables|Default|GetPlayerSettingsFP))
  (Variables|/Game/SynthArchMP_Template/Blueprints/Core/SaveGame_SynthArchMP.SaveGame_SynthArchMP_C|SetPlayerSettingsVR _savegameref (Variables|Default|GetPlayerSettingsVR))
  (CallFunction|SaveData _savegameref "PlayerSettings" true)
  (Utilities|FlowControl|Delay 0.2)
  (Game|QuitGame 0 "Quit" false))

(event Custom|SetBenchmarkedScalability
  ;[0.574 1 0.5387 1 36] Performance Settings
  ;;[1 1 1] Benchmark:
  ;;;[1 1 1] Apply new scalability settings based on the results of the benchmark.
  (bind (_scalabilitylevel _fps) (PerformanceSettings|GetCustomScalabilityLevel (Variables|Default|GetFrameTimeArray)))
  (Variables|Default|SetFPS_Benchmark _fps)
  (PerformanceSettings|SetCustomScalabilitySettings _scalabilitylevel true)
  (CallFunction|SavePlayerSettings)
  (Development|PrintString (Utilities|String|Append "Custom Scalability - " (Utilities|String|ToString(Integer) _scalabilitylevel) " 
Average FPS - " (Utilities|String|ToString(Float) _fps)) true true "(R=1.000000,G=0.203278,B=0.542681,A=1.000000)" 1e+01))

(event Custom|InitSettings_FP
  ;[0.574 1 0.5387 1 36] Performance Settings
)

(event Custom|SavePlayerSettings
  (bind _savegameref (Variables|Default|GetSaveGameRef))
  ;[1 1 1] Init
  ;;[1 1 1] Save Events
  (Variables|/Game/SynthArchMP_Template/Blueprints/Core/SaveGame_SynthArchMP.SaveGame_SynthArchMP_C|SetPlayerSettingsFP _savegameref (Variables|Default|GetPlayerSettingsFP))
  (Variables|/Game/SynthArchMP_Template/Blueprints/Core/SaveGame_SynthArchMP.SaveGame_SynthArchMP_C|SetPlayerSettingsVR _savegameref (Variables|Default|GetPlayerSettingsVR))
  (CallFunction|SaveData _savegameref "PlayerSettings" true))

(event Custom|LoadPlayerSettings
  ;[1 1 1] Init
  ;;[1 1 1] Save Events
  (bind (_success_ _savegameref) (CallFunction|LoadData "PlayerSettings"))
  (if _success_
    (Variables|Default|SetPlayerSettingsFP (Variables|/Game/SynthArchMP_Template/Blueprints/Core/SaveGame_SynthArchMP.SaveGame_SynthArchMP_C|GetPlayerSettingsFP _savegameref))
    (Variables|Default|SetPlayerSettingsVR (Variables|/Game/SynthArchMP_Template/Blueprints/Core/SaveGame_SynthArchMP.SaveGame_SynthArchMP_C|GetPlayerSettingsVR _savegameref))
    (Variables|Default|SetPlayerSettingsLoaded? _success_)))

(event Custom|InitDevSettings
  (bind _returnvalue (Game|GetGameMode))
  ;[1 0.4533 0.9912] Dev Settings
  (if (Variables|Default|GetLevelLoaded?) :!label _label
    (Utilities|IsValid _returnvalue :!label _label_2
      (:Is%20Valid
        (Utilities|Casting|CastToGameMode_SynthArchMP_DevVR _returnvalue
          (:then
            _)
          (:CastFailed
            (Utilities|Casting|CastToGameMode_SynthArchMP_DevFP _returnvalue
              (:then
                _)
              (:CastFailed
                (Utilities|Casting|CastToGameMode_SynthArchMP_DevFP_NoLoad _returnvalue
                  (:then
                    _)
                  (:CastFailed
                    (Utilities|Casting|CastToGameMode_SynthArchMP_DevVR_NoLoad _returnvalue)))))))
        ;;[1 1 1] Set default MediaInfo playlist for testing
        (bind _structout (Utilities|Struct|SetmembersinSTRUCT_PlayerInfo (Variables|Default|GetPlayerInfo) (Utilities|Array|MakeArray (Utilities|Struct|MakeSTRUCT_MediaInfo "SynthArch2022_Spring_Class_1.074.jpeg" "http://www.jonathanwilliamturner.com/staging/synthArch/media/lectures/SynthArch2022_Spring_Class_1_images/SynthArch2022_Spring_Class_1.074.jpeg" "NewEnumerator1") (Utilities|Struct|MakeSTRUCT_MediaInfo "taz_tunnel_4_10sec_1.mp4" "http://www.jonathanwilliamturner.com/staging/synthArch/SynthArchMP/media/test_media/taz_tunnel_4_10sec_1.mp4" "NewEnumerator0") (Utilities|Struct|MakeSTRUCT_MediaInfo "ENDLESS GRADIENT [MONTAGE]" "https://player.vimeo.com/external/377406720.hd.mp4?s=aa6cbcb6b9094ae768ab8ab7167c9c6672ef43c1&profile_id=175" "NewEnumerator0") (Utilities|Struct|MakeSTRUCT_MediaInfo "SLIDE 1" "http://www.jonathanwilliamturner.com/staging/synthArch/media/lectures/SynthArch2022_Spring_Class_1_images/SynthArch2022_Spring_Class_1.006.jpeg" "NewEnumerator1") (Utilities|Struct|MakeSTRUCT_MediaInfo "BAD URL ERROR" "http://www.jonathanwilliamturner.com/staging/synthArch/SynthArchMP/media/test_media/taz_tunnel_4_10sec_1_badURL.mp4" "NewEnumerator0") (Utilities|Struct|MakeSTRUCT_MediaInfo "BAD URL ERROR" "http://www.jonathanwilliamturner.com/staging/synthArch/media/lectures/SynthArch2022_Spring_Class_1_images/NoImage.jpeg" "NewEnumerator1"))))
        (bind _asgame_state_synth_arch_mp (Utilities|Casting|CastToGameState_SynthArchMP (Game|GetGameState)))
        (Default|ServerAddPlayerInfo _asgame_state_synth_arch_mp (Variables|Default|GetPlayerInfo)))
      (:Is%20Not%20Valid
        (Utilities|FlowControl|Delay 0.2)
        (goto _label_2)))
    (else
      (Utilities|FlowControl|Delay 0.2)
      (goto _label))))

(event Custom|RunCustomBenchmark
  ;[0.574 1 0.5387 1 36] Performance Settings
  ;;[1 1 1] Benchmark:
  (Utilities|Array|Clear (Variables|Default|GetFrameTimeArray))
  ;;;[1 1 1] Force Scalability=3 settings to stress test performance
  (bind _returnvalue (Settings|GetGameUserSettings))
  (Class|GameUserSettings|SetOverallScalabilityLevel _returnvalue 3)
  (Class|GameUserSettings|ApplySettings _returnvalue false)
  (Utilities|FlowControl|Delay 0.2)
  ;;;[1 1 1] Get a sampling of frame times.
  (bind _returnvalue_2 (Utilities|Time|SetTimerbyEvent (delegate Custom|GetFrameTimeData) 0.1 true)))

(event Custom|SetSettingsFromSaved_FP
  (bind _playersettingsfp (Variables|Default|GetPlayerSettingsFP))
  (bind (_maxfps _screenpercentage _aa_method _postprocessquality _shadowquality _shadowmethod _volumetricfog _ssao _dfao _gamma _inverty_axis) (Utilities|Struct|BreakSTRUCT_PlayerSettings_FP _playersettingsfp))
  ;[0.574 1 0.5387 1 36] Performance Settings
  ;;[1 1 1] Set Settings FP
  ;;;[1 1 1] FP Default Settings
  (Development|ExecuteConsoleCommand "r.VSync 1" 0)
  (Development|ExecuteConsoleCommand "r.TemporalAA.Upsampling 1" 0)
  (PerformanceSettings|UpdateMaxFPS _maxfps true)
  (PerformanceSettings|UpdateScreenPercentage _screenpercentage true)
  (PerformanceSettings|UpdateAntiAliasingMethod _aa_method false true)
  (PerformanceSettings|UpdatePostProcessQuality _postprocessquality false true)
  (PerformanceSettings|UpdateShadowQuality _shadowquality false true)
  (PerformanceSettings|UpdateShadowMethod _shadowmethod false true)
  (PerformanceSettings|UpdateVolumetricFog _volumetricfog false true)
  (PerformanceSettings|UpdateSSAO _ssao false true)
  (PerformanceSettings|UpdateDFAO _dfao false true)
  (PerformanceSettings|UpdateInvertY _inverty_axis))

(event Custom|GetFrameTimeData
  (bind _frametimearray (Variables|Default|GetFrameTimeArray))
  ;[0.574 1 0.5387 1 36] Performance Settings
  ;;[1 1 1] Benchmark:
  ;;;[1 1 1] Get a sampling of frame times.
  (Utilities|Array|Add _frametimearray (Utilities|Time|GetWorldDeltaSeconds))
  (if (>= (Utilities|Array|Length _frametimearray) 10)
    (Utilities|Time|ClearandInvalidateTimerbyHandle (stale Custom|RunCustomBenchmark _returnvalue_2))
    (CallFunction|SetBenchmarkedScalability)))

(event Custom|InitSettings_VR
  ;[0.574 1 0.5387 1 36] Performance Settings
  ;;[1 1 1] Set Settings VP
)

(event EventInit
  ;[1 1 1] Init
  (Utilities|FlowControl|Sequence
    (:then_0
      (bind _returnvalue (SaveGame|CreateSaveGameObject "/Game/SynthArchMP_Template/Blueprints/Core/SaveGame_SynthArchMP.SaveGame_SynthArchMP_C"))
      (Variables|Default|SetSaveGameRef _returnvalue)
      (CallFunction|LoadPlayerSettings))))

(fn ProcessMediaScript
  (params (MediaScript :type String))
  (Utilities|Array|Clear (.MediaInfoArray (Utilities|Struct|BreakSTRUCT_PlayerInfo (Variables|Default|GetPlayerInfo))))
  ;[1 1 1] Create an array, delimiting by carriage returns.
  ; **Sometimes carriage return is NOT recognized by MacOS and needs to be re-entered manually.
  (for _array_element (Utilities|String|ParseIntoArray MediaScript (Variables|Default|GetMyDelimiter) false)
    ;[1 1 1] Sort by file extension, assign the Media Format and build the Media Info Array.
    (if (Utilities|String|Contains (Utilities|String|Trim _array_element) ".mp4" false true)
      (LocalVariables|SetMediaFormat "NewEnumerator0")
      (Utilities|Array|Add (.MediaInfoArray (Utilities|Struct|BreakSTRUCT_PlayerInfo (Variables|Default|GetPlayerInfo))) (Utilities|Struct|MakeSTRUCT_MediaInfo "" (Utilities|String|Trim _array_element) (LocalVariables|GetMediaFormat)) :!label _label)
      (elif (or (or (Utilities|String|Contains (Utilities|String|Trim _array_element) ".jpeg" false true) (Utilities|String|Contains (Utilities|String|Trim _array_element) ".jpg" false true)) (Utilities|String|Contains (Utilities|String|Trim _array_element) ".png" false true))
        (LocalVariables|SetMediaFormat "NewEnumerator1")
        (goto _label)))))

(fn GetCustomScalabilityLevel
  (params (FrameTimeArray :type Array%20of%20Floats%20%28double-precision%29))
  (for _array_element FrameTimeArray
    (LocalVariables|SetSum (+ _array_element (LocalVariables|GetSum))))
  (bind _output_get (LocalVariables|SetAverageFPS (/ 1.0 (/ (LocalVariables|GetSum) (Utilities|Array|Length FrameTimeArray)))))
  (if (>= _output_get 55.0)
    (Variables|Default|SetCustomScalabilityLevel 3)
    (elif (>= _output_get 25.0)
      (Variables|Default|SetCustomScalabilityLevel 2)
      (elif (>= _output_get 15.0)
        (Variables|Default|SetCustomScalabilityLevel 1)
        (else
          (Variables|Default|SetCustomScalabilityLevel 0)))))
  (return (Variables|Default|GetCustomScalabilityLevel) (LocalVariables|GetAverageFPS)))

(fn RevisePlayerMedia
  ;[1 1 1] We have to request the Server to revise the player media by running the request through the PlayerController.
  (bind _asplayer_controller_synth_arch_mp (Utilities|Casting|CastToPlayerController_SynthArchMP (Game|GetPlayerController 0)))
  (Default|RevisePlayerMedia _asplayer_controller_synth_arch_mp (Variables|Default|GetPlayerInfo) (PlayerState|GetPlayerName (Game|GetPlayerState 0))))

(fn SetCustomScalabilitySettings
  (params (ScalabilityLevel :type Integer) (Save? :type Boolean))
  (Development|ExecuteConsoleCommand "r.VSync 1" 0)
  (Development|ExecuteConsoleCommand "r.TemporalAA.Upsampling 1" 0)
  (Development|ExecuteConsoleCommand "vr.bEnableHMD False" 0)
  (Development|ExecuteConsoleCommand "vr.bEnableStereo False" 0)
  (PerformanceSettings|UpdateMaxFPS (Utilities|Select :Index ScalabilityLevel :Option%200 24.0 :Option%201 3e+01 :Option%202 6e+01 :Option%203 6e+01) Save?)
  (PerformanceSettings|UpdateScreenPercentage (Utilities|Select :Index ScalabilityLevel :Option%200 35.0 :Option%201 5e+01 :Option%202 75.0 :Option%203 1e+02) Save?)
  (PerformanceSettings|UpdateAntiAliasingMethod (Utilities|Select :Index 0 :Option%200 2 :Option%201 2 :Option%202 4 :Option%203 4) false Save?)
  (PerformanceSettings|UpdatePostProcessQuality (Utilities|Select :Index ScalabilityLevel :Option%200 1 :Option%201 2 :Option%202 3 :Option%203 3) false Save?)
  (PerformanceSettings|UpdateShadowQuality (Utilities|Select :Index ScalabilityLevel :Option%200 1 :Option%201 2 :Option%202 2 :Option%203 3) false Save?)
  (PerformanceSettings|UpdateShadowMethod (Utilities|Select :Index ScalabilityLevel :Option%200 0 :Option%201 0 :Option%202 0 :Option%203 0) false Save?)
  (PerformanceSettings|UpdateVolumetricFog (Utilities|Select :Index ScalabilityLevel :Option%200 false :Option%201 false :Option%202 true :Option%203 true) false Save?)
  (PerformanceSettings|UpdateSSAO (Utilities|Select :Index ScalabilityLevel :Option%200 true :Option%201 true :Option%202 false :Option%203 false) false Save?)
  (PerformanceSettings|UpdateDFAO (Utilities|Select :Index ScalabilityLevel :Option%200 false :Option%201 false :Option%202 true :Option%203 true) false Save?))

(fn UpdateAntiAliasingMethod
  (params (Value :type Integer) (VR_Enabled? :type Boolean) (Save? :type Boolean))
  (Utilities|FlowControl|Sequence
    (:then_0
      (Development|ExecuteConsoleCommand (Utilities|String|Append "r.AntiAliasingMethod " (Utilities|String|ToString(Integer) Value)) 0))
    (:then_1
      (if Save?
        (if VR_Enabled?
          (Utilities|Struct|SetmembersinSTRUCT_PlayerSettings_VR (Variables|Default|GetPlayerSettingsVR) Value)
          (else
            (Utilities|Struct|SetmembersinSTRUCT_PlayerSettings_FP (Variables|Default|GetPlayerSettingsFP) Value)))))))

(fn UpdateMaxFPS
  (params (Value :type Float%20%28double-precision%29) (Save? :type Boolean))
  (Utilities|FlowControl|Sequence
    (:then_0
      (Development|ExecuteConsoleCommand (Utilities|String|Append "t.MaxFPS " (Utilities|String|ToString(Float) Value)) 0))
    (:then_1
      (if Save?
        (Utilities|Struct|SetmembersinSTRUCT_PlayerSettings_FP (Variables|Default|GetPlayerSettingsFP) Value)))))

(fn UpdateScreenPercentage
  (params (Value :type Float%20%28double-precision%29) (Save? :type Boolean))
  (Utilities|FlowControl|Sequence
    (:then_0
      (Development|ExecuteConsoleCommand (Utilities|String|Append "r.ScreenPercentage " (Utilities|String|ToString(Float) Value)) 0))
    (:then_1
      (if Save?
        (Utilities|Struct|SetmembersinSTRUCT_PlayerSettings_FP (Variables|Default|GetPlayerSettingsFP) Value)))))

(fn UpdateShadowQuality
  (params (Value :type Integer) (VR_Enabled? :type Boolean) (Save? :type Boolean))
  (Utilities|FlowControl|Sequence
    (:then_0
      (Development|ExecuteConsoleCommand (Utilities|String|Append "sg.ShadowQuality " (Utilities|String|ToString(Integer) Value)) 0))
    (:then_2
      (if Save?
        (if VR_Enabled?
          (Utilities|Struct|SetmembersinSTRUCT_PlayerSettings_VR (Variables|Default|GetPlayerSettingsVR) Value)
          (else
            (Utilities|Struct|SetmembersinSTRUCT_PlayerSettings_FP (Variables|Default|GetPlayerSettingsFP) Value)))))))

(fn UpdateShadowMethod
  (params (Value :type Integer) (VR_Enabled? :type Boolean) (Save? :type Boolean))
  (Utilities|FlowControl|Sequence
    (:then_0
      (switch int Value
        (:0
          (Development|ExecuteConsoleCommand (Utilities|String|Append "r.Shadow.Virtual.Enable " "0") 0))
        (:1
          (Development|ExecuteConsoleCommand (Utilities|String|Append "r.Shadow.Virtual.Enable " "1") 0))
        (:2
          ;[1 0.1823 0.1823] Needs work
          (Development|ExecuteConsoleCommand (Utilities|String|Append "r.Shadow.Virtual.Enable " "0") 0))))
    (:then_1
      (if Save?
        (if VR_Enabled?
          (Utilities|Struct|SetmembersinSTRUCT_PlayerSettings_VR (Variables|Default|GetPlayerSettingsVR) Value)
          (else
            (Utilities|Struct|SetmembersinSTRUCT_PlayerSettings_FP (Variables|Default|GetPlayerSettingsFP) Value)))))))

(fn UpdatePostProcessQuality
  (params (Value :type Integer) (VR_Enabled? :type Boolean) (Save? :type Boolean))
  (Utilities|FlowControl|Sequence
    (:then_0
      (Development|ExecuteConsoleCommand (Utilities|String|Append "sg.PostProcessQuality " (Utilities|String|ToString(Integer) Value)) 0))
    (:then_1
      (if Save?
        (if VR_Enabled?
          (Utilities|Struct|SetmembersinSTRUCT_PlayerSettings_VR (Variables|Default|GetPlayerSettingsVR) Value)
          (else
            (Utilities|Struct|SetmembersinSTRUCT_PlayerSettings_FP (Variables|Default|GetPlayerSettingsFP) Value)))))))

(fn UpdateVolumetricFog
  (params (State :type Boolean) (VR_Enabled? :type Boolean) (Save? :type Boolean))
  (Utilities|FlowControl|Sequence
    (:then_0
      (Development|ExecuteConsoleCommand (Utilities|String|Append "r.VolumetricFog " (Utilities|String|ToString(Integer) (select State 1 0))) 0))
    (:then_1
      (if Save?
        (if VR_Enabled?
          (Utilities|Struct|SetmembersinSTRUCT_PlayerSettings_VR (Variables|Default|GetPlayerSettingsVR) State)
          (else
            (Utilities|Struct|SetmembersinSTRUCT_PlayerSettings_FP (Variables|Default|GetPlayerSettingsFP) State)))))))

(fn UpdateSSAO
  (params (State :type Boolean) (VR_Enabled? :type Boolean) (Save? :type Boolean))
  (Utilities|FlowControl|Sequence
    (:then_0
      (Development|ExecuteConsoleCommand (Utilities|String|Append "r.AmbientOcclusionLevels " (select State "1" "0")) 0))
    (:then_1
      (if Save?
        (if VR_Enabled?
          (Utilities|Struct|SetmembersinSTRUCT_PlayerSettings_VR (Variables|Default|GetPlayerSettingsVR) State)
          (else
            (Utilities|Struct|SetmembersinSTRUCT_PlayerSettings_FP (Variables|Default|GetPlayerSettingsFP) State)))))))

(fn UpdateDFAO
  (params (State :type Boolean) (VR_Enabled? :type Boolean) (Save? :type Boolean))
  (bind _skylight (Variables|Default|GetSkyLight))
  (bind _lightcomponent (Variables|/Script/Engine.SkyLight|GetLightComponent _skylight))
  (Utilities|FlowControl|Sequence
    (:then_0
      (Utilities|IsValid _skylight
        (:Is%20Valid
          (Rendering|Components|Light|SetCastShadows _lightcomponent State)
          (Rendering|Components|Light|SetIntensity _lightcomponent (select State 1.0 0.5)))))
    (:then_1
      (if Save?
        (if VR_Enabled?
          (Utilities|Struct|SetmembersinSTRUCT_PlayerSettings_VR (Variables|Default|GetPlayerSettingsVR) State)
          (else
            (Utilities|Struct|SetmembersinSTRUCT_PlayerSettings_FP (Variables|Default|GetPlayerSettingsFP) State)))))))

(fn UpdateInvertY
  (params (State :type Boolean)))

(fn LoadData
  (params (SlotName :type String))
  (bind _returnvalue (SaveGame|DoesSaveGameExist SlotName))
  (if _returnvalue
    (bind _returnvalue_2 (SaveGame|LoadGamefromSlot SlotName))
    (bind _assave_game_synth_arch_mp (Utilities|Casting|CastToSaveGame_SynthArchMP _returnvalue_2)
      (:then
        (return _returnvalue _assave_game_synth_arch_mp))
      (:CastFailed
        _)))
  (return _returnvalue 0))

(fn SaveData
  (params (SaveGameRef :type Save%20Game%20Object%20Reference) (SlotName :type String) (Overwrite? :type Boolean))
  (bind _returnvalue (SaveGame|DoesSaveGameExist SlotName))
  (if _returnvalue
    (if Overwrite?
      (bind _returnvalue_2 (SaveGame|SaveGametoSlot SaveGameRef SlotName :!label _label))
      (return _returnvalue_2))
    (else
      (goto _label))))

(fn UpdateVRPixelDensity
  (params (Value :type Float%20%28double-precision%29))
  (Development|ExecuteConsoleCommand (Utilities|String|Append "vr.PixelDensity " (Utilities|String|ToString(Float) Value)) 0)
  (Utilities|Struct|SetmembersinSTRUCT_PlayerSettings_VR (Variables|Default|GetPlayerSettingsVR) Value))

(fn UpdateTeleportMethod
  (params (TeleportMethod :type ENUM_TeleportMethod%20Enum :default "NewEnumerator0"))
  (Utilities|FlowControl|Sequence
    (:then_1
      (Utilities|Struct|SetmembersinSTRUCT_PlayerSettings_VR (Variables|Default|GetPlayerSettingsVR) TeleportMethod))))

(fn UpdateSlideSpeed
  (params (Value :type Float%20%28double-precision%29))
  (Utilities|FlowControl|Sequence
    (:then_1
      (Utilities|Struct|SetmembersinSTRUCT_PlayerSettings_VR (Variables|Default|GetPlayerSettingsVR) Value))))

(fn UpdateMoveSpeed
  (params (Value :type Float%20%28double-precision%29))
  (Utilities|FlowControl|Sequence
    (:then_1
      (Utilities|Struct|SetmembersinSTRUCT_PlayerSettings_VR (Variables|Default|GetPlayerSettingsVR) Value))))

(fn UpdateMoveDirection
  (params (MovementOrientation :type ENUM_MovementOrientation%20Enum :default "NewEnumerator0"))
  (Utilities|FlowControl|Sequence
    (:then_1
      (Utilities|Struct|SetmembersinSTRUCT_PlayerSettings_VR (Variables|Default|GetPlayerSettingsVR) MovementOrientation))))

(fn UpdateSnapTurn
  (params (State :type Boolean))
  (Utilities|FlowControl|Sequence
    (:then_1
      (Utilities|Struct|SetmembersinSTRUCT_PlayerSettings_VR (Variables|Default|GetPlayerSettingsVR) State))))
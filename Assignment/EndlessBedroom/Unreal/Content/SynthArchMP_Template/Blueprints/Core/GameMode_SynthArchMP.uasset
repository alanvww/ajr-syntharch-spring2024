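; Game mode for the SynthArchMP multiplayer template that handles joining players and their PlayerInfo.
; SpawnPlayer computes a randomized transform around the custom PlayerStart matching the player's tag.
; It stores PlayerInfo locally when media info exists, then always sends it to the GameState for replication to clients.
; Pawn spawn and possess nodes are disconnected, so the VR check and computed transform currently spawn nothing.
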(event Custom|SpawnPlayer
  (params (NewPlayerController :type Player%20Controller%20Object%20Reference) (PlayerInfo :type STRUCT%20Player%20Info%20Structure))
  ;[1 1 1] Spawn Player
  (Variables|Default|SetNew%20Player%20Controller NewPlayerController)
  (bind _output_get (Variables|Default|SetPlayerInfo PlayerInfo))
  (Utilities|FlowControl|Sequence
    (:then_0
      (bind _spawntransform (CallFunction|SetSpawnTransform))
      (if (.VR_Enabled? (Utilities|Struct|BreakSTRUCT_PlayerInfo _output_get))
        _))
    (:then_1
      ;;[1 1 1] Add the joining player's PlayerInfo to the PlayerInfoArray, which is replicated to all Clients on the GameState.
      (if (> (Utilities|Array|Length (.MediaInfoArray (Utilities|Struct|BreakSTRUCT_PlayerInfo (Variables|Default|GetPlayerInfo)))) 0)
        (Utilities|Array|Add (Variables|Default|GetPlayerInfoArray) (Variables|Default|GetPlayerInfo)))
      (bind _asgame_state_synth_arch_mp (Utilities|Casting|CastToGameState_SynthArchMP (Game|GetGameState)))
      (Default|ServerAddPlayerInfo _asgame_state_synth_arch_mp (Variables|Default|GetPlayerInfo)))))

(event Custom|SpawnDefaultPawn)

(event EventBeginPlay
  (bind _asgame_instance_synth_arch_mp (Utilities|Casting|CastToGameInstance_SynthArchMP (Game|GetGameInstance)))
  (Variables|Default|SetGameInstanceRef _asgame_instance_synth_arch_mp))

(fn ConstructionScript)

(fn SetSpawnTransform
  (bind _playerstartrange (LocalVariables|GetPlayerStartRange))
  (bind _returnvalue (* -1 _playerstartrange))
  ;[1 1 1] Determine the PlayerStart location
  (bind _outactors (Actor|GetAllActorsOfClass "/Game/SynthArchMP_Template/Blueprints/BP_PlayerStartCustom_1.BP_PlayerStartCustom_1_C"))
  (bind _array_element (Utilities|Array|ForEachLoopwithBreak _outactors :!label _label)
    (:LoopBody
      (if (Utilities|Name|Equal(Name) (Variables|/Game/SynthArchMP_Template/Blueprints/BP_PlayerStartCustom_1.BP_PlayerStartCustom_1_C|GetPlayerStartTag _array_element) (.PlayerStartTag (Utilities|Struct|BreakSTRUCT_PlayerInfo (Variables|Default|GetPlayerInfo))))
        (goto _label Break)))
    (:Completed
      (return (Math|Transform|MakeTransform (Math|Vector|MakeVector (+ (.x (.Location (Math|Transform|BreakTransform (Transformation|GetActorTransform _array_element)))) (Math|Random|RandomFloatinRange _returnvalue _playerstartrange)) (+ (.y (.Location (Math|Transform|BreakTransform (Transformation|GetActorTransform _array_element)))) (Math|Random|RandomFloatinRange _returnvalue _playerstartrange)) (.z (.Location (Math|Transform|BreakTransform (Transformation|GetActorTransform _array_element))))) (.Rotation (Math|Transform|BreakTransform (Transformation|GetActorTransform _array_element))) (.Scale (Math|Transform|BreakTransform (Transformation|GetActorTransform _array_element))))))))
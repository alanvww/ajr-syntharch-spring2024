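; GameState for the SynthArch multiplayer template that holds a shared PlayerInfoArray of players and their media.
; Server events add player entries or revise a named player's media, then multicast the updated array to clients.
; The multicasts fire PlayerInfoAdded and PlayerMediaRevised dispatchers for bound media players such as BP_MediaScreenAdvanced.
; The array's OnRep also fires PlayerInfoAdded.
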(event Custom|Multicast_RevisePlayerMedia
  (params (PlayerInfoArray :type Array%20of%20STRUCT%20Player%20Info%20Structures) (PlayerStateName :type String))
  ;[1 1 1] Revise Player Media:
  ; Replace the corresponding player's MediaInfoArray and then replicate the PlayerInfoArray. Multicast the event dispatcher "PlayerMediaRevised" which is received by BP_MediaScreenAdvanced (or any MediaPlayers bound to it).
  (Variables|Default|SetPlayerInfoArray PlayerInfoArray)
  (Default|CallPlayerMediaRevised PlayerStateName))

(event Custom|Server_AddPlayerInfo
  (params (PlayerInfoArray :type STRUCT%20Player%20Info%20Structure))
  ;[1 1 1] Add Player Info:
  ; Joining players are added to the PlayerInfoArray. Multicast the event dispatcher "PlayerInfoAdded" which is received by BP_MediaScreenAdvanced (or any MediaPlayers bound to it).
  (Utilities|Array|Add (Variables|Default|GetPlayerInfoArray) PlayerInfoArray)
  (CallFunction|MulticastUpdatePlayerInfoArray (Variables|Default|GetPlayerInfoArray)))

(event Custom|Multicast_UpdatePlayerInfoArray
  (params (PlayerInfoArray :type Array%20of%20STRUCT%20Player%20Info%20Structures))
  ;[1 1 1] Add Player Info:
  ; Joining players are added to the PlayerInfoArray. Multicast the event dispatcher "PlayerInfoAdded" which is received by BP_MediaScreenAdvanced (or any MediaPlayers bound to it).
  (Variables|Default|SetPlayerInfoArray PlayerInfoArray)
  (Default|CallPlayerInfoAdded))

(event Custom|Server_RevisePlayerMedia
  (params (PlayerInfoArray :type STRUCT%20Player%20Info%20Structure%20%28by%20ref%29) (PlayerStateName :type String))
  ;[1 1 1] Revise Player Media:
  ; Replace the corresponding player's MediaInfoArray and then replicate the PlayerInfoArray. Multicast the event dispatcher "PlayerMediaRevised" which is received by BP_MediaScreenAdvanced (or any MediaPlayers bound to it).
  (bind (_array_element _array_index) (Utilities|Array|ForEachLoopwithBreak (Variables|Default|GetPlayerInfoArray))
    (:LoopBody
      (if (Utilities|Enum|Equal(Enum) (.PlayerStateName (Utilities|Struct|BreakSTRUCT_PlayerInfo _array_element)) PlayerStateName)
        (Utilities|Struct|SetmembersinSTRUCT_PlayerInfo (Utilities|Array|Get(acopy) (Variables|Default|GetPlayerInfoArray) _array_index) (.MediaInfoArray (Utilities|Struct|BreakSTRUCT_PlayerInfo PlayerInfoArray)))))
    (:Completed
      (CallFunction|MulticastRevisePlayerMedia (Variables|Default|GetPlayerInfoArray) PlayerStateName))))

(event EventBeginPlay)

(fn ConstructionScript)

(fn OnRepPlayerInfoArray
  (Default|CallPlayerInfoAdded))
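; BP_LevelManager_Bedrooms is a level manager actor, apparently for the Bedrooms level of the SynthArchMP template.
; On BeginPlay it caches the SynthArchMP game instance and checks the game mode.
; Under the DevFP or DevVR game modes it waits a second and calls LevelLoadFinished on the instance, while the main game mode triggers nothing.
; Its construction script zeroes the TextRender's world rotation as an orientation hack.
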(event EventBeginPlay
  (bind _returnvalue (Game|GetGameMode))
  (bind _asgame_instance_synth_arch_mp (Utilities|Casting|CastToGameInstance_SynthArchMP (Game|GetGameInstance)))
  (Variables|Default|SetGameInstanceRef _asgame_instance_synth_arch_mp)
  (Utilities|Casting|CastToGameMode_SynthArchMP _returnvalue
    (:CastFailed
      (Utilities|Casting|CastToGameMode_SynthArchMP_DevFP _returnvalue
        (:then
          _)
        (:CastFailed
          (Utilities|Casting|CastToGameMode_SynthArchMP_DevVR _returnvalue)))
      (Utilities|FlowControl|Delay 1.0)
      (bind _asgame_instance_synth_arch_mp_2 (Utilities|Casting|CastToGameInstance_SynthArchMP (Game|GetGameInstance)))
      (Default|LevelLoadFinished _asgame_instance_synth_arch_mp_2))))

(fn ConstructionScript
  (Transformation|SetWorldRotation (Variables|Default|GetTextRender) "0, 0, 0" false false) ; Hack to make the TextRender orient correctly
)
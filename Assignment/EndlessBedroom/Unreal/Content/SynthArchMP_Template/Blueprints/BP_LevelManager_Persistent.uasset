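; Persistent-level manager for SynthArchMP that handles startup and streams in the Atrium_1 level.
; On BeginPlay it repositions the player pawn and applies default scalability, retrying until pawn and controller are valid.
; The local player sees a loading screen until the StreamLevelsLoaded dispatcher notifies the game instance and swaps in the Player Options menu.
; DevFP and DevVR game modes skip that setup and UI, only loading the level and notifying the game instance.
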(event Custom|LoadStreamLevels
  (params (Dev? :type Boolean))
  ;[1 1 1] Load the levels?
  (Game|LoadStreamLevel(byName) "Atrium_1" true)
  (if Dev?
    (bind _asgame_instance_synth_arch_mp (Utilities|Casting|CastToGameInstance_SynthArchMP (Game|GetGameInstance)))
    (Default|LevelLoadFinished _asgame_instance_synth_arch_mp)
    (else
      (Default|CallStreamLevelsLoaded))))

(event Custom|ShowPlayerOptions
  (bind _returnvalue (Game|GetPlayerController 0))
  ;[1 1 1] Load the levels?
  (bind _asgame_instance_synth_arch_mp (Utilities|Casting|CastToGameInstance_SynthArchMP (Game|GetGameInstance)))
  (Default|LevelLoadFinished _asgame_instance_synth_arch_mp)
  (Widget|RemovefromParent (stale EventBeginPlay _returnvalue_4))
  (Utilities|Casting|CastToPlayerController_SynthArchMP _returnvalue)
  (bind _returnvalue_2 (UserInterface|CreateWidget "/Game/SynthArchMP_Template/Blueprints/Widgets/BPW_PlayerOptions.BPW_PlayerOptions_C" _returnvalue))
  (UserInterface|Viewport|AddtoViewport _returnvalue_2 0))

(event EventBeginPlay
  (bind _returnvalue (Game|GetGameMode))
  (bind _returnvalue_2 (Game|GetPlayerController 0))
  (bind _returnvalue_3 (Game|Player|GetPlayerPawn 0))
  (Utilities|FlowControl|Sequence
    (:then_0
      (bind _asgame_instance_synth_arch_mp (Utilities|Casting|CastToGameInstance_SynthArchMP (Game|GetGameInstance)))
      (Variables|Default|SetGameInstanceRef _asgame_instance_synth_arch_mp)
      (Utilities|Casting|CastToGameMode_SynthArchMP _returnvalue
        (:then
          (Utilities|FlowControl|Sequence :!label _label
            (:then_0
              (Utilities|IsValid _returnvalue_3 :!label _label_2
                (:Is%20Valid
                  (Transformation|SetActorLocationAndRotation _returnvalue_3 "0, 0, 0")
                  ;[1 1 1] Default Console Commands for the Player Options menu
                  (Default|SetCustomScalabilitySettings (Variables|Default|GetGameInstanceRef) 2 false))
                (:Is%20Not%20Valid
                  (Utilities|FlowControl|Delay 0.2)
                  (goto _label_2))))
            (:then_1
              ;[1 1 1] Show loading screen widget and set the input mode for the Player Options screen
              (Utilities|IsValid _returnvalue_2 :!label _label_3
                (:Is%20Valid
                  (if (Pawn|IsLocalController _returnvalue_2)
                    (bind _returnvalue_4 (UserInterface|CreateWidget "/Game/SynthArchMP_Template/Blueprints/Widgets/BPW_LoadingScreen.BPW_LoadingScreen_C" _returnvalue_2))
                    (UserInterface|Viewport|AddtoViewport _returnvalue_4 0)
                    (Input|SetInputModeGameandUI _returnvalue_2 _returnvalue_4 "LockOnCapture" false false)
                    (Variables|/Script/Engine.PlayerController|SetbShowMouseCursor _returnvalue_2 true)
                    ;[1 1 1] Load the levels?
                    (EventDispatchers|BindEventtoStreamLevelsLoaded (delegate Custom|ShowPlayerOptions))
                    (CallFunction|LoadStreamLevels false)))
                (:Is%20Not%20Valid
                  (Utilities|FlowControl|Delay 0.2)
                  (goto _label_3))))))
        (:CastFailed
          (Utilities|Casting|CastToGameMode_SynthArchMP_DevFP _returnvalue
            (:then
              _)
            (:CastFailed
              (Utilities|Casting|CastToGameMode_SynthArchMP_DevVR _returnvalue
                (:then
                  _)
                (:CastFailed
                  (goto _label)))))
          ;[1 1 1] Dev Mode
          (CallFunction|LoadStreamLevels true))))))

(fn ConstructionScript
  (Transformation|SetWorldRotation (Variables|Default|GetTextRender) "0, 0, 0" false false) ; Hack to make the TextRender orient correctly
)
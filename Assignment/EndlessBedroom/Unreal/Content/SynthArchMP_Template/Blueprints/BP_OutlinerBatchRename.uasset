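; BP_OutlinerBatchRename is an editor utility Blueprint that batch-renames the Outliner labels of every actor of a chosen ActorClass.
; Its Rename event shows a suppressible overwrite warning, then relabels each found actor with its class display name, minus the last character, plus a one-based index.
; The warning's result is not checked, so renaming always proceeds; other graph fragments are unconnected leftovers.
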(event Custom|Rename
  (Class|EditorDialogLibrary|ShowSuppressableWarningDialog (Utilities|Text|MakeLiteralText "Batch Outliner Rename") (Utilities|Text|MakeLiteralText "Warning!! This will overwrite all display labels for this class.") "" "" true)
  (bind _outactors (Actor|GetAllActorsOfClass 0 (Variables|Default|GetActor%20Class)))
  (for (_array_element _array_index) _outactors
    (EditorScripting|ActorEditing|SetActorLabel _array_element (Utilities|String|Append (Utilities|String|LeftChop (Utilities|GetClassDisplayName (Utilities|GetClass _array_element)) 1) (Utilities|String|ToString(Integer) (+ _array_index 1))) true)))

(event EventBeginPlay)

(event Collision|EventActorBeginOverlap
  (params (OtherActor :type Actor%20Object%20Reference)))

(event EventTick
  (params (DeltaSeconds :type Float%20%28single-precision%29)))

(fn ConstructionScript)
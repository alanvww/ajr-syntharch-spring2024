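; Multiplayer lift actor that moves between floor heights stored in an array when its Up, Down or Call buttons are pushed.
; Button pushes go to a server event that ignores input mid-move, bounds-checks and steps the floor, with Call Up descending and Call Down ascending.
; A multicast then plays a duration-scaled timeline that eases the lift root's height and modulates the lift sound's volume and pitch.
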(event Custom|Server_MoveLift
  (params (ButtonFunction :type ENUM_LiftButtonFunction%20Enum :default "NewEnumerator16") (FloorNum :type Integer))
  ;[1 1 1] Move Lift
  (if (not (Audio|Components|Audio|IsPlaying (Variables|Default|GetTimeline_MoveLIft)))
    (switch Utilities|FlowControl|Switch|SwitchonENUM_LiftButtonFunction ButtonFunction
      (:NewEnumerator0
        (if (< (+ (Variables|Default|GetFloorNum) 1) (Utilities|Array|Length (Variables|Default|GetLiftZ_Array))) :!label _label
          (bind _result (Math|Integer|IncrementInt (Variables|Default|GetFloorNum))
            (:%20%20
              (CallFunction|MulticastMoveLift _result)))))
      (:NewEnumerator1
        (if (>= (- (Variables|Default|GetFloorNum) 1) 0) :!label _label_2
          (bind _result_2 (Math|Integer|DecrementInt (Variables|Default|GetFloorNum))
            (:%20%20
              (CallFunction|MulticastMoveLift _result_2)))))
      (:NewEnumerator14
        (goto _label_2))
      (:NewEnumerator15
        (goto _label)))))

(event Custom|Multicast_MoveLift
  (params (FloorNum :type Integer))
  (bind _liftsound (Variables|Default|GetLiftSound))
  ;[1 1 1] Move Lift
  (Variables|Default|SetLiftZ_A (.z (Variables|/Script/Engine.SceneComponent|GetRelativeLocation (Variables|Default|GetLift_Root))))
  (Variables|Default|SetLiftZ_B (Utilities|Array|Get(acopy) (Variables|Default|GetLiftZ_Array) FloorNum))
  (Audio|Components|Audio|Play (Variables|Default|GetLiftSound) 0.0)
  (bind (_direction _time _volume _pitch) (Timeline|Timeline_MoveLIft PlayFromStart)
    (:Update
      (Transformation|SetRelativeLocation (Variables|Default|GetLift_Root) (Math|Vector|MakeVector 0.0 0.0 (Math|Interpolation|Ease "EaseInOut" _time (Variables|Default|GetLiftZ_A) (Variables|Default|GetLiftZ_B) 2.0)) false false)
      (Audio|Components|Audio|SetVolumeMultiplier _liftsound _volume :!class /Script/Engine.AudioComponent)
      (Audio|Components|Audio|SetPitchMultiplier _liftsound _pitch))
    (:Finished
      (Audio|Components|Audio|Stop (Variables|Default|GetLiftSound)))))

(event EventBeginPlay
  (Components|Timeline|SetPlayRate (Variables|Default|GetTimeline_MoveLIft) (/ 1.0 (Variables|Default|GetDuration))))

(event EventPushLiftButton
  (params (ButtonFunction :type ENUM_LiftButtonFunction%20Enum :default "NewEnumerator16") (OtherActor :type Actor%20Object%20Reference) (FunctionTag :type Name :default "None"))
  (CallFunction|ServerMoveLift ButtonFunction))

(fn ConstructionScript)